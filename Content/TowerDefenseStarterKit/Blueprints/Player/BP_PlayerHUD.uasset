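; BP_PlayerHUD is the tower defense player HUD blueprint that switches the game into the Loadout Menu or Mission Summary screens.
; Both functions set a HUD state through BP_GameInstance and switch input to UI-only, focused on the active HUD widget.
; Before showing the summary, it records mission success or failure in BP_GameState and has BP_PlayerController run its pre-summary protocols.
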(fn `DisplayLoadoutMenu`
  ;[0 1 1 0.5] Execute all required protocols before displaying the Loadout Menu at level start
  (bind _asbp_game_instance (cast `/Game/TowerDefenseStarterKit/Blueprints/BP_GameInstance` (`GameplayStatics.GetGameInstance`)))
  (`/Game/TowerDefenseStarterKit/Blueprints/BP_GameInstance.UpdateHUDState` _asbp_game_instance "NewEnumerator0")
  (`WidgetBlueprintLibrary.SetInputMode_UIOnlyEx` (`GameplayStatics.GetPlayerController` 0) (`/Game/TowerDefenseStarterKit/Blueprints/FunctionLibraries/BPFL_GetterFunctions.GetActiveHUDWidget` self)))

(fn `DisplayMissionSummary`
  (params (`MissionSuccess?` :type Boolean))
  ;[0 1 1 0.5] Execute all required protocols before displaying the Mission Summary
  (bind _asbp_game_state (cast `/Game/TowerDefenseStarterKit/Blueprints/BP_GameState` (`GameplayStatics.GetGameState`)))
  (`/Game/TowerDefenseStarterKit/Blueprints/BP_GameState.UpdateMissionStatus` _asbp_game_state `MissionSuccess?`)
  (bind _asbp_player_controller (cast `/Game/TowerDefenseStarterKit/Blueprints/Player/BP_PlayerController` (`GameplayStatics.GetPlayerController` 0)))
  (`/Game/TowerDefenseStarterKit/Blueprints/Player/BP_PlayerController.ExecutePreMissionSummaryProtocols` _asbp_player_controller)
  (`/Game/TowerDefenseStarterKit/Blueprints/BP_GameInstance.UpdateHUDState` (cast `/Game/TowerDefenseStarterKit/Blueprints/BP_GameInstance` (`GameplayStatics.GetGameInstance`) :!pure true) "NewEnumerator3")
  (`WidgetBlueprintLibrary.SetInputMode_UIOnlyEx` (`GameplayStatics.GetPlayerController` 0) (`/Game/TowerDefenseStarterKit/Blueprints/FunctionLibraries/BPFL_GetterFunctions.GetActiveHUDWidget` self)))

(fn `UserConstructionScript`)