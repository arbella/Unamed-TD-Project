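; BPC_SmoothZoom is an actor component that smoothly zooms its owner's camera in and out within set limits.
; ZoomIn and ZoomOut step a clamped target zoom from the supplied current value.
; A 60 Hz tick interpolates toward that target, reading and writing zoom through the owner's BPI_CameraZoom interface.
; Owners lacking the interface get a printed warning at BeginPlay, which names the class BPC_StepZoom.
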(event `self.ReceiveBeginPlay`
  ;[0 1 1 0.5] Initiates the component if the owner meets the compatibility requirements
  (if (`KismetSystemLibrary.DoesImplementInterface` (`self.GetOwner`) "/Game/TowerDefenseStarterKit/Blueprints/Player/CameraZoom/BPI_CameraZoom.BPI_CameraZoom_C")
    (bind _camerazoom (message `/Game/TowerDefenseStarterKit/Blueprints/Player/CameraZoom/BPI_CameraZoom.RetrieveCurrentZoom` (`self.GetOwner`)))
    (set `self.NewCameraZoom` _camerazoom)
    (`self.SetComponentTickInterval` (/ 1.0 60.0))
    (`self.SetComponentTickEnabled` true)
    (else
      (`self.DisplayOwnerIncompatibilityWarning`))))

(event `self.ReceiveTick`
  (params (DeltaSeconds :type "Float (single-precision)"))
  ;[0 1 1 0.5] Uses interpolation to smoothly update the camera zoom of the owning actor
  (set `self.DeltaTime` DeltaSeconds)
  (bind _camerazoom (message `/Game/TowerDefenseStarterKit/Blueprints/Player/CameraZoom/BPI_CameraZoom.RetrieveCurrentZoom` (`self.GetOwner`)))
  (if (not (== _camerazoom (`self.NewCameraZoom`)))
    (message `/Game/TowerDefenseStarterKit/Blueprints/Player/CameraZoom/BPI_CameraZoom.UpdateCameraZoom` (`self.GetOwner`) (`KismetMathLibrary.FInterpTo` _camerazoom (`self.NewCameraZoom`) (`self.DeltaTime`) (`self.CameraZoomSpeed`))) ; Requests the owner to set the new camera zoom value
  ))

(fn `DisplayOwnerIncompatibilityWarning`
  ;[0 0 0 0.5] Prints a warning message if the owning actor does not implement the requisite interface
  (`KismetSystemLibrary.PrintString` (`KismetStringLibrary.Concat_StrStr` "WARNING: [Class - BPC_StepZoom] Owning Actor '" (`KismetSystemLibrary.GetDisplayName` (`self.GetOwner`)) "' does not implement required interface BPI_CameraZoom")))

(fn `ZoomIn`
  (params (CurrentCameraZoom :type "Float (double-precision)"))
  ;[0 1 1 0.5] Calculates the new zoom value based on the current camera zoom of the owner
  (set `self.NewCameraZoom` (`KismetMathLibrary.FClamp` (+ CurrentCameraZoom -1000.0) (`self.ZoomInLimit`) (`self.ZoomOutLimit`))))

(fn `ZoomOut`
  (params (CurrentCameraZoom :type "Float (double-precision)"))
  ;[0 1 1 0.5] Calculates the new zoom value based on the current camera zoom of the owner
  (set `self.NewCameraZoom` (`KismetMathLibrary.FClamp` (+ CurrentCameraZoom 1000.0) (`self.ZoomInLimit`) (`self.ZoomOutLimit`))))