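; BPC_StepZoom is an actor component that gives its owner stepped camera zoom between in and out limits.
; On BeginPlay it divides the zoom range into equal increments, or prints a warning if the owner lacks BPI_CameraZoom.
; ZoomIn and ZoomOut read the current zoom through that interface, shift it one increment, clamp it and send it back to the owner.
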(event `self.ReceiveBeginPlay`
  ;[0 1 1 0.5] Initiates the component if the owner meets the compatibility requirements
  (if (`KismetSystemLibrary.DoesImplementInterface` (`self.GetOwner`) "/Game/TowerDefenseStarterKit/Blueprints/Player/CameraZoom/BPI_CameraZoom.BPI_CameraZoom_C")
    (set `self.ScrollZoomIncrement` (/ (- (`self.ZoomOutLimit`) (`self.ZoomInLimit`)) (`KismetMathLibrary.Conv_IntToDouble` (`self.NumberOfZoomSteps`))))
    (else
      (`self.DisplayOwnerIncompatibilityWarning`))))

(fn `DisplayOwnerIncompatibilityWarning`
  ;[0 0 0 0.5] Prints a warning message if the owning actor does not implement the requisite interface
  (`KismetSystemLibrary.PrintString` (`KismetStringLibrary.Concat_StrStr` "WARNING: [Class - BPC_StepZoom] Owning Actor '" (`KismetSystemLibrary.GetDisplayName` (`self.GetOwner`)) "' does not implement required interface BPI_CameraZoom")))

(fn `ZoomIn`
  ;[0 1 1 0.5] Increases the camera zoom by a single step
  (bind _camerazoom (message `/Game/TowerDefenseStarterKit/Blueprints/Player/CameraZoom/BPI_CameraZoom.RetrieveCurrentZoom` (`self.GetOwner`)))
  (message `/Game/TowerDefenseStarterKit/Blueprints/Player/CameraZoom/BPI_CameraZoom.UpdateCameraZoom` (`self.GetOwner`) (`KismetMathLibrary.FClamp` (- _camerazoom (`self.ScrollZoomIncrement`)) (`self.ZoomInLimit`) (`self.ZoomOutLimit`))))

(fn `ZoomOut`
  ;[0 1 1 0.5] Decreases the camera zoom by a single step
  (bind _camerazoom (message `/Game/TowerDefenseStarterKit/Blueprints/Player/CameraZoom/BPI_CameraZoom.RetrieveCurrentZoom` (`self.GetOwner`)))
  (message `/Game/TowerDefenseStarterKit/Blueprints/Player/CameraZoom/BPI_CameraZoom.UpdateCameraZoom` (`self.GetOwner`) (`KismetMathLibrary.FClamp` (+ _camerazoom (`self.ScrollZoomIncrement`)) (`self.ZoomInLimit`) (`self.ZoomOutLimit`))))