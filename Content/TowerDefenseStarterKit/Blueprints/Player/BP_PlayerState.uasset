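; Player state Blueprint for the tower defense kit that tracks the player's score and tower points.
; ModifyPlayerScore adds a delta clamped at zero, while ModifyTowerPoints adds one without clamping and GetTowerPoints returns the current total.
; Both modify functions push the new value to player controller 0 through HUD update messages, an interface approach noted as added in version 2.8.
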(fn `GetTowerPoints`
  (returns (TowerPoints :type Integer))
  ;[1 1 1] Version 2.8
  (return (`self.TowerPoints`)))

(fn `ModifyPlayerScore`
  (params (By :type Integer))
  (returns (NewScore :type Integer))
  (bind _returnvalue (+ (`self.PlayerScore`) By))
  ;[0 1 1 0.5] Updates the player score data & relays the new information over to the player controller for performing any necessary HUD updates
  (if (> _returnvalue 0)
    (set `self.PlayerScore` _returnvalue)
    (else
      (set `self.PlayerScore` 0)))
  ;;[1 1 1] Version  2.8: HUD Updates through new dedicated interface
  (message `/Game/TowerDefenseStarterKit/Blueprints/Player/BPI_GameInfoDisplay.OnPlayerScoreUpdated` (`GameplayStatics.GetPlayerController` 0) (`self.PlayerScore`))
  (return (`self.PlayerScore`)))

(fn `ModifyTowerPoints`
  (params (By :type Integer))
  ;[0 1 1 0.5] Version 2.8: Modifies tower points by the specified amount
  (bind _output_get (set `self.TowerPoints` (+ (`self.TowerPoints`) By)))
  (message `/Game/TowerDefenseStarterKit/Blueprints/Player/BPI_GameInfoDisplay.OnTowerPointsUpdated` (`GameplayStatics.GetPlayerController` 0) _output_get)
  (return))

(fn `UserConstructionScript`)