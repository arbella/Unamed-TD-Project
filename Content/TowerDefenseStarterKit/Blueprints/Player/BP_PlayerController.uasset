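; Player controller for the tower defense game, routing cursor selection, tower build/upgrade/sell/function requests and global ability targeting.
; Looping timers trace under the cursor to highlight grid cells or move the targeting reticule, toggled as modes change.
; Selections and UI button events drive the Tower Manager, PlayerState tower points and Global Abilities Manager, and relay info, score and wave updates to the HUD.
; Pawn input stays disabled until a timer detects a valid viewport size.
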(event `self.ReceiveBeginPlay`
  ;[0 1 1 0.5] Turn on Vsync to prevent potential screen tearing & disable all inputs from player pawn untill startup protocols have been executed
  (`KismetSystemLibrary.ExecuteConsoleCommand` "r.vsync 1" self)
  (`self.DisableInput` (`GameplayStatics.GetPlayerPawn` 0) self))

(event `ExecutePreMissionSummaryProtocols`
  ;[0 1 1 0.5] Hide Tower Constructor UI element before displaying the mission summary; Pauses game only after the Tower Constructor menu has been hidden; Without delay the 'Set Hidden in Game' execution get halted due to pause
  (`/Game/TowerDefenseStarterKit/Blueprints/Towers/BP_TowerManager.StopTowerConstructionSystems` (`/Game/TowerDefenseStarterKit/Blueprints/FunctionLibraries/BPFL_GetterFunctions.GetTowerManager` self))
  (`KismetSystemLibrary.Delay` 0.2)
  (`GameplayStatics.SetGamePaused` true))

(event `NewTargetSelected`
  (params (SelectedActor :type "Actor Object Reference"))
  ;[0 1 1 0.5] Initiates info display for the selected actor
  (`/Engine/EditorBlueprintResources/StandardMacros.IsValid` SelectedActor
    (:`Is Valid`
      (if (`KismetSystemLibrary.DoesImplementInterface` SelectedActor "/Game/TowerDefenseStarterKit/Blueprints/HUDControl/BPI_TargetInfoDisplay.BPI_TargetInfoDisplay_C")
        (bind (_name _description _stats) (message `/Game/TowerDefenseStarterKit/Blueprints/HUDControl/BPI_TargetInfoDisplay.RetrieveTargetInfo` SelectedActor))
        (`self.UpdateHUD_TargetInfo` _name _description _stats)))))

(event `UpdateHUD_TargetInfo`
  (params (Name :type Text) (Description :type Text) (Stats :type "Array of /Game/TowerDefenseStarterKit/Blueprints/HUDControl/Struct_HUDStats Structure"))
  ;[0 1 1 0.5] Requests HUD to display specifed information
  (bind _aswidget_game_hud (cast `/Game/TowerDefenseStarterKit/UI/PlayerHUD/Widget_GameHUD` (`/Game/TowerDefenseStarterKit/Blueprints/FunctionLibraries/BPFL_GetterFunctions.GetActiveHUDWidget` self)))
  (`/Game/TowerDefenseStarterKit/UI/PlayerHUD/Widget_GameHUD.DisplayTargetInfo` _aswidget_game_hud Name Description Stats))

(event `/Game/TowerDefenseStarterKit/Blueprints/Player/BPI_TowerConstructorInteraction.TowerInteractionDisabled`
  (params (Tower :type "/Game/TowerDefenseStarterKit/Blueprints/Towers/BP_Tower_Parent Object Reference"))
  ;[0 1 0.4 0.5] BPI_TowerConstructorInteraction interface functions: Enables the Tower Constructor UI to communicate state changes to the player controller
  (if (== Tower (`self.SelectedActor`))
    (`self.SetDefaultUIState`)))

(event `/Game/TowerDefenseStarterKit/Blueprints/Player/BPI_GlobalAbilityInteraction.OnGlobalAbilityManagerInitialized`
  (params (SelectedAbilities :type "Array of /Game/TowerDefenseStarterKit/Blueprints/GlobalAbilities/EGlobalAbilities Enum (by ref)" :default _) (GlobalAbilityDTMap :type "Map of /Game/TowerDefenseStarterKit/Blueprints/GlobalAbilities/EGlobalAbilities Enum to DataTableRowHandle Structure" :default _))
  ;[0 1 0.4 0.5] BPI_GlobalAbilityInteraction interface functions: Enables communication about global ability selection/activation state changes
  ;;[1 1 1] Global Ability Manager Initialization
  (bind _aswidget_game_hud (cast `/Game/TowerDefenseStarterKit/UI/PlayerHUD/Widget_GameHUD` (`/Game/TowerDefenseStarterKit/Blueprints/FunctionLibraries/BPFL_GetterFunctions.GetActiveHUDWidget` self)))
  (`/Game/TowerDefenseStarterKit/UI/PlayerHUD/Widget_GameHUD.OnActivateGlobalAbilitySelection` _aswidget_game_hud SelectedAbilities GlobalAbilityDTMap))

(event `/Game/TowerDefenseStarterKit/Blueprints/Player/BPI_TowerConstructorInteraction.TowerBuildButtonClicked`
  (params (TowerModel :type "/Game/TowerDefenseStarterKit/Blueprints/Towers/ETowerModels Enum" :default "NewEnumerator2") (ConstructionCost :type Integer))
  ;[0 1 0.4 0.5] BPI_TowerConstructorInteraction interface functions: Enables the Tower Constructor UI to communicate state changes to the player controller
  ;;[1 1 1] Tower Interaction Button Click Responses
  (`/Game/TowerDefenseStarterKit/Blueprints/Towers/BP_TowerManager.SpawnTower` (`/Game/TowerDefenseStarterKit/Blueprints/FunctionLibraries/BPFL_GetterFunctions.GetTowerManager` self) (`self.SelectedGridCellIndex`) (`self.SelectedGridGeneratorIndex`) TowerModel)
  ;;;[1 1 1] Version 2.8: Tower Points now stored in Player State
  (bind _asbp_player_state (cast `/Game/TowerDefenseStarterKit/Blueprints/Player/BP_PlayerState` (`self.PlayerState`))
    (:`then`
      (`/Game/TowerDefenseStarterKit/Blueprints/Player/BP_PlayerState.ModifyTowerPoints` _asbp_player_state (* ConstructionCost -1)))
    (:`CastFailed`
      _))
  (`self.SetDefaultUIState`))

(event `/Game/TowerDefenseStarterKit/Blueprints/Player/BPI_GlobalAbilityInteraction.GlobalAbilityButtonClicked`
  (params (bIsSelected :type Boolean) (AbilityType :type "/Game/TowerDefenseStarterKit/Blueprints/GlobalAbilities/EGlobalAbilities Enum" :default "NewEnumerator2"))
  ;[0 1 0.4 0.5] BPI_GlobalAbilityInteraction interface functions: Enables communication about global ability selection/activation state changes
  ;;[1 1 1] Global Ability Button Interactions
  (if bIsSelected
    (`self.ActivateGlobalAbilityTargeting` AbilityType)
    (bind _aswidget_game_hud (cast `/Game/TowerDefenseStarterKit/UI/PlayerHUD/Widget_GameHUD` (`/Game/TowerDefenseStarterKit/Blueprints/FunctionLibraries/BPFL_GetterFunctions.GetActiveHUDWidget` self)))
    (`/Game/TowerDefenseStarterKit/UI/PlayerHUD/Widget_GameHUD.OnGlobalAbilitySelected` _aswidget_game_hud AbilityType)
    (else
      (`self.DeactivateGlobalAbilityTargeting`))))

(event `/Game/TowerDefenseStarterKit/Blueprints/Player/BPI_TowerConstructorInteraction.TowerUpgradeButtonClicked`
  (params (UpgradedTowerModel :type "/Game/TowerDefenseStarterKit/Blueprints/Towers/ETowerModels Enum" :default "NewEnumerator2") (UpgradeCost :type Integer))
  ;[0 1 0.4 0.5] BPI_TowerConstructorInteraction interface functions: Enables the Tower Constructor UI to communicate state changes to the player controller
  ;;[1 1 1] Tower Interaction Button Click Responses
  (`/Game/TowerDefenseStarterKit/Blueprints/Towers/BP_TowerManager.UpgradeTower` (`/Game/TowerDefenseStarterKit/Blueprints/FunctionLibraries/BPFL_GetterFunctions.GetTowerManager` self) (`self.SelectedActor`) UpgradedTowerModel)
  ;;;[1 1 1] Version 2.8: Tower Points now stored in Player State
  (bind _asbp_player_state (cast `/Game/TowerDefenseStarterKit/Blueprints/Player/BP_PlayerState` (`self.PlayerState`))
    (:`then`
      (`/Game/TowerDefenseStarterKit/Blueprints/Player/BP_PlayerState.ModifyTowerPoints` _asbp_player_state (* UpgradeCost -1)))
    (:`CastFailed`
      _))
  (`self.SetDefaultUIState`))

(event `/Game/TowerDefenseStarterKit/Blueprints/Player/BPI_GlobalAbilityInteraction.GlobalAbilityButtonHovered`
  (params (AbilityType :type "/Game/TowerDefenseStarterKit/Blueprints/GlobalAbilities/EGlobalAbilities Enum" :default "NewEnumerator2"))
  ;[0 1 0.4 0.5] BPI_GlobalAbilityInteraction interface functions: Enables communication about global ability selection/activation state changes
  ;;[1 1 1] Global Ability Button Interactions
  (bind (_functionname _functiondescription _stats) (`/Game/TowerDefenseStarterKit/Blueprints/GlobalAbilities/BP_GlobalAbilitiesManager.GetInfoAboutGlobalAbility` (`self.GlobalAbilitiesManager`) AbilityType))
  (`self.UpdateHUD_TargetInfo` _functionname _functiondescription _stats)
  (set `self.CurrentMouseCursor` "Default") ; Ensures that a mouse cursor is available for interacting with the focused widget
)

(event `/Game/TowerDefenseStarterKit/Blueprints/Player/BPI_TowerConstructorInteraction.TowerFunctionButtonClicked`
  (params (TowerFunction :type "/Game/TowerDefenseStarterKit/Blueprints/Towers/TowerFunctions/ETowerFunctions Enum" :default "NewEnumerator0") (ActivationCost :type Integer))
  ;[0 1 0.4 0.5] BPI_TowerConstructorInteraction interface functions: Enables the Tower Constructor UI to communicate state changes to the player controller
  ;;[1 1 1] Tower Interaction Button Click Responses
  (`/Game/TowerDefenseStarterKit/Blueprints/Towers/BP_TowerManager.ActivateTowerFunctionForTower` (`/Game/TowerDefenseStarterKit/Blueprints/FunctionLibraries/BPFL_GetterFunctions.GetTowerManager` self) (`self.SelectedActor`) TowerFunction)
  ;;;[1 1 1] Version 2.8: Tower Points now stored in Player State
  (bind _asbp_player_state (cast `/Game/TowerDefenseStarterKit/Blueprints/Player/BP_PlayerState` (`self.PlayerState`))
    (:`then`
      (`/Game/TowerDefenseStarterKit/Blueprints/Player/BP_PlayerState.ModifyTowerPoints` _asbp_player_state (* ActivationCost -1)))
    (:`CastFailed`
      _))
  (`self.SetDefaultUIState`))

(event `/Game/TowerDefenseStarterKit/Blueprints/Player/BPI_GlobalAbilityInteraction.GlobalAbilityButtonUnhovered`
  ;[0 1 0.4 0.5] BPI_GlobalAbilityInteraction interface functions: Enables communication about global ability selection/activation state changes
  ;;[1 1 1] Global Ability Button Interactions
  (`self.UpdateHUD_HideTargetStats`) ; Request the player controller to hide the target stats information
  (if (`self.IsGlobalAbilityTargetingActive?`)
    (set `self.CurrentMouseCursor` "None") ; Disable Mouse Cursor if the Global Ability Targeting Reticule is active
  ))

(event `/Game/TowerDefenseStarterKit/Blueprints/Player/BPI_TowerConstructorInteraction.TowerRecycleButtonClicked`
  (params (SellingPrice :type Integer))
  ;[0 1 0.4 0.5] BPI_TowerConstructorInteraction interface functions: Enables the Tower Constructor UI to communicate state changes to the player controller
  ;;[1 1 1] Tower Interaction Button Click Responses
  (bind _asbp_tower_parent (cast `/Game/TowerDefenseStarterKit/Blueprints/Towers/BP_Tower_Parent` (`self.SelectedActor`)))
  (`/Game/TowerDefenseStarterKit/Blueprints/Towers/BP_Tower_Parent.SellTower` _asbp_tower_parent)
  ;;;[1 1 1] Comment
  (bind _asbp_player_state (cast `/Game/TowerDefenseStarterKit/Blueprints/Player/BP_PlayerState` (`self.PlayerState`))
    (:`then`
      (`/Game/TowerDefenseStarterKit/Blueprints/Player/BP_PlayerState.ModifyTowerPoints` _asbp_player_state SellingPrice))
    (:`CastFailed`
      _))
  (`self.SetDefaultUIState`))

(event `/Game/TowerDefenseStarterKit/Blueprints/Player/BPI_GlobalAbilityInteraction.OnGlobalAbilityDeployed`
  (params (AbilityType :type "/Game/TowerDefenseStarterKit/Blueprints/GlobalAbilities/EGlobalAbilities Enum" :default "NewEnumerator2") (RechargeTime :type "Float (single-precision)"))
  ;[0 1 0.4 0.5] BPI_GlobalAbilityInteraction interface functions: Enables communication about global ability selection/activation state changes
  ;;[1 1 1] Global Ability Deployment
  (bind _aswidget_game_hud (cast `/Game/TowerDefenseStarterKit/UI/PlayerHUD/Widget_GameHUD` (`/Game/TowerDefenseStarterKit/Blueprints/FunctionLibraries/BPFL_GetterFunctions.GetActiveHUDWidget` self)))
  (`/Game/TowerDefenseStarterKit/UI/PlayerHUD/Widget_GameHUD.OnBeginGlobalAbilityRecharge` _aswidget_game_hud AbilityType RechargeTime))

(event `/Game/TowerDefenseStarterKit/Blueprints/Player/BPI_TowerConstructorInteraction.TowerBuildButtonHovered`
  (params (TowerModel :type "/Game/TowerDefenseStarterKit/Blueprints/Towers/ETowerModels Enum" :default "NewEnumerator2"))
  ;[0 1 0.4 0.5] BPI_TowerConstructorInteraction interface functions: Enables the Tower Constructor UI to communicate state changes to the player controller
  ;;[1 1 1] Tower Interaction Button Hover Responses
  (bind (_towername _description _stats) (`/Game/TowerDefenseStarterKit/Blueprints/Towers/BP_TowerManager.GetInfoAboutTowerModel` (`/Game/TowerDefenseStarterKit/Blueprints/FunctionLibraries/BPFL_GetterFunctions.GetTowerManager` self) TowerModel))
  (`self.UpdateHUD_TargetInfo` _towername _description _stats)
  (`/Game/TowerDefenseStarterKit/Blueprints/Towers/BP_TowerManager.DisplayRangeForTowerModel` (`/Game/TowerDefenseStarterKit/Blueprints/FunctionLibraries/BPFL_GetterFunctions.GetTowerManager` self) TowerModel))

(event `/Game/TowerDefenseStarterKit/Blueprints/Player/BPI_TowerConstructorInteraction.TowerUpgradeButtonHovered`
  (params (UpgradedTowerModel :type "/Game/TowerDefenseStarterKit/Blueprints/Towers/ETowerModels Enum" :default "NewEnumerator2"))
  ;[0 1 0.4 0.5] BPI_TowerConstructorInteraction interface functions: Enables the Tower Constructor UI to communicate state changes to the player controller
  ;;[1 1 1] Tower Interaction Button Hover Responses
  (bind (_towername _description _stats) (`/Game/TowerDefenseStarterKit/Blueprints/Towers/BP_TowerManager.GetInfoAboutTowerModel` (`/Game/TowerDefenseStarterKit/Blueprints/FunctionLibraries/BPFL_GetterFunctions.GetTowerManager` self) UpgradedTowerModel))
  (`self.UpdateHUD_TargetInfo` _towername _description _stats)
  (`/Game/TowerDefenseStarterKit/Blueprints/Towers/BP_TowerManager.DisplayRangeForTowerModel` (`/Game/TowerDefenseStarterKit/Blueprints/FunctionLibraries/BPFL_GetterFunctions.GetTowerManager` self) UpgradedTowerModel))

(event `/Game/TowerDefenseStarterKit/Blueprints/Player/BPI_GameInfoDisplay.OnTowerPointsUpdated`
  (params (NewValue :type Integer))
  ;[0 1 0.4 0.5] Version 2.8: BPI_GameInfoDisplay Interface Functions - HUD Updates for general game state changes
  (bind _aswidget_game_hud (cast `/Game/TowerDefenseStarterKit/UI/PlayerHUD/Widget_GameHUD` (`/Game/TowerDefenseStarterKit/Blueprints/FunctionLibraries/BPFL_GetterFunctions.GetActiveHUDWidget` self)))
  (`/Game/TowerDefenseStarterKit/UI/PlayerHUD/Widget_GameHUD.UpdateTowerPoints` _aswidget_game_hud NewValue)
  (`/Game/TowerDefenseStarterKit/Blueprints/Towers/BP_TowerManager.RefreshTowerConstructor` (`/Game/TowerDefenseStarterKit/Blueprints/FunctionLibraries/BPFL_GetterFunctions.GetTowerManager` self)) ; Refreshes Tower Constructor state based on updated Tower Points value
)

(event `/Game/TowerDefenseStarterKit/Blueprints/Player/BPI_GameInfoDisplay.OnPlayerScoreUpdated`
  (params (NewValue :type Integer))
  ;[0 1 0.4 0.5] Version 2.8: BPI_GameInfoDisplay Interface Functions - HUD Updates for general game state changes
  (bind _aswidget_game_hud (cast `/Game/TowerDefenseStarterKit/UI/PlayerHUD/Widget_GameHUD` (`/Game/TowerDefenseStarterKit/Blueprints/FunctionLibraries/BPFL_GetterFunctions.GetActiveHUDWidget` self)))
  (`/Game/TowerDefenseStarterKit/UI/PlayerHUD/Widget_GameHUD.UpdatePlayerScoreDisplay` _aswidget_game_hud NewValue))

(event `/Game/TowerDefenseStarterKit/Blueprints/Player/BPI_TowerConstructorInteraction.TowerFunctionButtonHovered`
  (params (TowerFunction :type "/Game/TowerDefenseStarterKit/Blueprints/Towers/TowerFunctions/ETowerFunctions Enum" :default "NewEnumerator0"))
  ;[0 1 0.4 0.5] BPI_TowerConstructorInteraction interface functions: Enables the Tower Constructor UI to communicate state changes to the player controller
  ;;[1 1 1] Tower Interaction Button Hover Responses
  (bind (_functionname _functiondescription _stats) (`/Game/TowerDefenseStarterKit/Blueprints/Towers/BP_TowerManager.GetInfoAboutTowerFunction` (`/Game/TowerDefenseStarterKit/Blueprints/FunctionLibraries/BPFL_GetterFunctions.GetTowerManager` self) TowerFunction))
  (`self.UpdateHUD_TargetInfo` _functionname _functiondescription _stats))

(event `/Game/TowerDefenseStarterKit/Blueprints/Player/BPI_GameInfoDisplay.DisplayTotalWaveCount`
  (params (`EndlessMode?` :type Boolean) (WaveCount :type Integer))
  ;[0 1 0.4 0.5] Version 2.8: BPI_GameInfoDisplay Interface Functions - HUD Updates for general game state changes
  (bind _aswidget_game_hud (cast `/Game/TowerDefenseStarterKit/UI/PlayerHUD/Widget_GameHUD` (`/Game/TowerDefenseStarterKit/Blueprints/FunctionLibraries/BPFL_GetterFunctions.GetActiveHUDWidget` self)))
  (`/Game/TowerDefenseStarterKit/UI/PlayerHUD/Widget_GameHUD.UpdateTotalWaveCount` _aswidget_game_hud `EndlessMode?` WaveCount))

(event `/Game/TowerDefenseStarterKit/Blueprints/Player/BPI_GameInfoDisplay.OnNewWaveStarted`
  (params (NewWaveNumber :type Integer))
  ;[0 1 0.4 0.5] Version 2.8: BPI_GameInfoDisplay Interface Functions - HUD Updates for general game state changes
  (bind _aswidget_game_hud (cast `/Game/TowerDefenseStarterKit/UI/PlayerHUD/Widget_GameHUD` (`/Game/TowerDefenseStarterKit/Blueprints/FunctionLibraries/BPFL_GetterFunctions.GetActiveHUDWidget` self)))
  (`/Game/TowerDefenseStarterKit/UI/PlayerHUD/Widget_GameHUD.UpdateCurrentWaveNumber` _aswidget_game_hud NewWaveNumber))

(event `/Game/TowerDefenseStarterKit/Blueprints/Player/BPI_TowerConstructorInteraction.TowerRecycleButtonHovered`
  (bind _selectedactor (`self.SelectedActor`))
  ;[0 1 0.4 0.5] BPI_TowerConstructorInteraction interface functions: Enables the Tower Constructor UI to communicate state changes to the player controller
  ;;[1 1 1] Tower Interaction Button Hover Responses
  ;;[1 1 1] Tower Interaction Button Unhover Responses
  (`/Engine/EditorBlueprintResources/StandardMacros.IsValid` _selectedactor :!label _label
    (:`Is Valid`
      (bind (_name _description _stats) (message `/Game/TowerDefenseStarterKit/Blueprints/HUDControl/BPI_TargetInfoDisplay.RetrieveTargetInfo` _selectedactor))
      (`self.UpdateHUD_TargetInfo` _name _description _stats)
      (bind _asbp_tower_parent (cast `/Game/TowerDefenseStarterKit/Blueprints/Towers/BP_Tower_Parent` (`self.SelectedActor`)))
      (`/Game/TowerDefenseStarterKit/Blueprints/Towers/BP_TowerManager.DisplayRangeForTowerModel` (`/Game/TowerDefenseStarterKit/Blueprints/FunctionLibraries/BPFL_GetterFunctions.GetTowerManager` self) (`/Game/TowerDefenseStarterKit/Blueprints/Towers/BP_Tower_Parent.TowerModel` _asbp_tower_parent)))))

(event `/Game/TowerDefenseStarterKit/Blueprints/Player/BPI_GameInfoDisplay.DisplayWaveCountdownTimer`
  ;[0 1 0.4 0.5] Version 2.8: BPI_GameInfoDisplay Interface Functions - HUD Updates for general game state changes
  (bind _aswidget_game_hud (cast `/Game/TowerDefenseStarterKit/UI/PlayerHUD/Widget_GameHUD` (`/Game/TowerDefenseStarterKit/Blueprints/FunctionLibraries/BPFL_GetterFunctions.GetActiveHUDWidget` self)))
  (`/Game/TowerDefenseStarterKit/UI/PlayerHUD/Widget_GameHUD.UpdateWaveCountDownTimerVisibility` _aswidget_game_hud "SelfHitTestInvisible"))

(event `/Game/TowerDefenseStarterKit/Blueprints/Player/BPI_GameInfoDisplay.OnWaveCountdownTimerUpdated`
  (params (NewValue :type "Float (single-precision)"))
  ;[0 1 0.4 0.5] Version 2.8: BPI_GameInfoDisplay Interface Functions - HUD Updates for general game state changes
  (bind _aswidget_game_hud (cast `/Game/TowerDefenseStarterKit/UI/PlayerHUD/Widget_GameHUD` (`/Game/TowerDefenseStarterKit/Blueprints/FunctionLibraries/BPFL_GetterFunctions.GetActiveHUDWidget` self)))
  (`/Game/TowerDefenseStarterKit/UI/PlayerHUD/Widget_GameHUD.UpdateWaveCountDownTimer` _aswidget_game_hud NewValue))

(event `/Game/TowerDefenseStarterKit/Blueprints/Player/BPI_GameInfoDisplay.HideWaveCountdownTimer`
  ;[0 1 0.4 0.5] Version 2.8: BPI_GameInfoDisplay Interface Functions - HUD Updates for general game state changes
  (bind _aswidget_game_hud (cast `/Game/TowerDefenseStarterKit/UI/PlayerHUD/Widget_GameHUD` (`/Game/TowerDefenseStarterKit/Blueprints/FunctionLibraries/BPFL_GetterFunctions.GetActiveHUDWidget` self)))
  (`/Game/TowerDefenseStarterKit/UI/PlayerHUD/Widget_GameHUD.UpdateWaveCountDownTimerVisibility` _aswidget_game_hud "Collapsed"))

(event `/Game/TowerDefenseStarterKit/Blueprints/Player/BPI_TowerConstructorInteraction.TowerBuildButtonUnhovered`
  ;[0 1 0.4 0.5] BPI_TowerConstructorInteraction interface functions: Enables the Tower Constructor UI to communicate state changes to the player controller
  ;;[1 1 1] Tower Interaction Button Unhover Responses
  (`self.UpdateHUD_HideTargetStats`) ; Request the Player Controller to hide the target stats display
  (`/Game/TowerDefenseStarterKit/Blueprints/Towers/BP_TowerManager.HideTowerRange` (`/Game/TowerDefenseStarterKit/Blueprints/FunctionLibraries/BPFL_GetterFunctions.GetTowerManager` self)))

(event `/Game/TowerDefenseStarterKit/Blueprints/Player/BPI_TowerConstructorInteraction.TowerUpgradeButtonUnhovered`
  ;[0 1 0.4 0.5] BPI_TowerConstructorInteraction interface functions: Enables the Tower Constructor UI to communicate state changes to the player controller
  ;;[1 1 1] Tower Interaction Button Unhover Responses
  (goto _label))

(event `/Game/TowerDefenseStarterKit/Blueprints/Player/BPI_TowerConstructorInteraction.TowerFunctionButtonUnhovered`
  ;[0 1 0.4 0.5] BPI_TowerConstructorInteraction interface functions: Enables the Tower Constructor UI to communicate state changes to the player controller
  ;;[1 1 1] Tower Interaction Button Unhover Responses
  (goto _label))

(event `/Game/TowerDefenseStarterKit/Blueprints/Player/BPI_TowerConstructorInteraction.TowerRecycleButtonUnhovered`
  ;[0 1 0.4 0.5] BPI_TowerConstructorInteraction interface functions: Enables the Tower Constructor UI to communicate state changes to the player controller
  ;;[1 1 1] Tower Interaction Button Unhover Responses
  (goto _label))

(fn `ActivateGlobalAbilityTargeting`
  (params (GlobalAbility :type "/Game/TowerDefenseStarterKit/Blueprints/GlobalAbilities/EGlobalAbilities Enum" :default "NewEnumerator2"))
  ;[0 1 1 0.5] Disable Grid Cell Detection & Tower Constructor; Activate Global Ability Targeting system
  (`/Game/TowerDefenseStarterKit/Blueprints/Towers/BP_TowerManager.StopTowerConstructionSystems` (`/Game/TowerDefenseStarterKit/Blueprints/FunctionLibraries/BPFL_GetterFunctions.GetTowerManager` self))
  (`self.DisableGridCellDetection`)
  (`/Game/TowerDefenseStarterKit/Blueprints/Misc/BP_GridCellHighlighter.RemoveGridCellHighlights` (`self.GridCellHighlighter`))
  (`/Game/TowerDefenseStarterKit/Blueprints/GlobalAbilities/BP_GlobalAbilitiesManager.OnTargetingActivated` (`self.GlobalAbilitiesManager`) GlobalAbility)
  (if (not (`KismetSystemLibrary.K2_TimerExistsHandle` (`self.UpdateTargetingReticuleTimerHandle`)))
    (bind _returnvalue (`KismetSystemLibrary.K2_SetTimer` null "UpdateGlobalAbilityTargetingReticule" (`self.UpdateActorTransformTimerInterval`) true))
    (set `self.UpdateTargetingReticuleTimerHandle` _returnvalue))
  (return))

(fn `BeginGlobalAbilityDeployment`
  (bind (_hitresult _returnvalue) (`self.GetHitResultUnderCursorByChannel` "TraceTypeQuery3" false))
  (bind (_bblockinghit _binitialoverlap _time _distance _location _impactpoint _normal _impactnormal _physmat _hitactor) (`GameplayStatics.BreakHitResult` _hitresult))
  ;[0 1 1 0.5] Request the Targeting Reticule to deploy the Global Ability based on the hit result
  (if _returnvalue
    (if (`KismetSystemLibrary.DoesImplementInterface` _hitactor (`/Game/TowerDefenseStarterKit/Blueprints/Misc/BP_TargetingReticule.GetGlobalAbilityTargetInterface` (`self.TargetingReticule`)))
      (`/Game/TowerDefenseStarterKit/Blueprints/GlobalAbilities/BP_GlobalAbilitiesManager.OnDeployGlobalAbility` (`self.GlobalAbilitiesManager`) _location)
      (`self.DeactivateGlobalAbilityTargeting`))))

(fn `DeactivateGlobalAbilityTargeting`
  (bind _updatetargetingreticuletimerhandle (`self.UpdateTargetingReticuleTimerHandle`))
  ;[0 1 1 0.5] Deactivate the Global Ability Targeting system & activate Grid Cell Detection
  (if (`KismetSystemLibrary.K2_TimerExistsHandle` _updatetargetingreticuletimerhandle)
    (`KismetSystemLibrary.K2_ClearAndInvalidateTimerHandle` _updatetargetingreticuletimerhandle))
  (`/Game/TowerDefenseStarterKit/Blueprints/Misc/BP_TargetingReticule.HideTargetingReticule` (`self.TargetingReticule`))
  (`/Game/TowerDefenseStarterKit/Blueprints/GlobalAbilities/BP_GlobalAbilitiesManager.OnTargetingDeactivated` (`self.GlobalAbilitiesManager`))
  (`self.EnableGridCellDetection`)
  (set `self.CurrentMouseCursor` "Default")
  (return))

(fn `DetectGridCells`
  (locals (Local_TraceHitLocation :type "Vector Structure") (Local_TraceHitActor :type "Actor Object Reference"))
  (bind (_hitresult _returnvalue) (`self.GetHitResultUnderCursorByChannel` "TraceTypeQuery2" false))
  (bind (_bblockinghit _binitialoverlap _time _distance _location _impactpoint _normal _impactnormal _physmat _hitactor) (`GameplayStatics.BreakHitResult` _hitresult))
  ;[0 1 1 0.5] Used to identify any grid cells at the cursor/touch location
  (if _returnvalue
    (set `local.Local_TraceHitLocation` _location)
    (bind _output_get (set `local.Local_TraceHitActor` _hitactor))
    (if (`KismetSystemLibrary.DoesImplementInterface` _output_get "/Game/TowerDefenseStarterKit/Blueprints/GridSystems/BPI_GridLink.BPI_GridLink_C")
      (bind (_gridcellindex _gridgeneratorindex) (message `/Game/TowerDefenseStarterKit/Blueprints/GridSystems/BPI_GridLink.RetrieveTraceHitGridData` (`local.Local_TraceHitActor`) (`local.Local_TraceHitLocation`)))
      (`/Game/TowerDefenseStarterKit/Blueprints/Misc/BP_GridCellHighlighter.HighlightGridCellAtIndex` (`self.GridCellHighlighter`) _gridcellindex _gridgeneratorindex)
      (else
        (`/Game/TowerDefenseStarterKit/Blueprints/Misc/BP_GridCellHighlighter.RemoveGridCellHighlights` (`self.GridCellHighlighter`) :!label _label)))
    (else
      (goto _label))))

(fn `DisableGridCellDetection`
  (bind _gridcelldetectiontimerhandle (`self.GridCellDetectionTimerHandle`))
  ;[0 1 1 0.5] Request the Grid Cell Detector to deactivate Grid Cell Detection
  (if (`KismetSystemLibrary.K2_TimerExistsHandle` _gridcelldetectiontimerhandle)
    (`KismetSystemLibrary.K2_ClearAndInvalidateTimerHandle` _gridcelldetectiontimerhandle)
    (return)
    (else
      (return))))

(fn `EnableGridCellDetection`
  ;[0 1 1 0.5] Request the Grid Cell Detector to activate Grid Cell Detection
  (if (not (`KismetSystemLibrary.K2_TimerExistsHandle` (`self.GridCellDetectionTimerHandle`)))
    (bind _returnvalue (`KismetSystemLibrary.K2_SetTimer` null "DetectGridCells" (`self.GridCellDetectionTimerInterval`) true))
    (set `self.GridCellDetectionTimerHandle` _returnvalue))
  (return))

(fn `GetGridCellDetectionStatus`
  (returns (`Enabled?` :type Boolean))
  ;[0 1 1 0.5] Returns if Grid Cell Detection is active or not
  (return (`KismetSystemLibrary.K2_TimerExistsHandle` (`self.GridCellDetectionTimerHandle`))))

(fn `GetSelectedActorDetails`
  (returns (SelectedActorType :type "/Game/TowerDefenseStarterKit/Blueprints/Player/ESelectedActorType Enum"))
  (locals (Local_TraceHitLocation :type "Vector Structure") (Local_TraceHitActor :type "Actor Object Reference") (Local_SelectedActorType :type "/Game/TowerDefenseStarterKit/Blueprints/Player/ESelectedActorType Enum" :default "NewEnumerator2"))
  (bind (_hitresult _returnvalue) (`self.GetHitResultUnderCursorByChannel` "TraceTypeQuery2" false))
  (bind (_bblockinghit _binitialoverlap _time _distance _location _impactpoint _normal _impactnormal _physmat _hitactor) (`GameplayStatics.BreakHitResult` _hitresult))
  ;[0 1 1 0.5] Identifies the selected actor based on the hit result under mouse cursor
  (if _returnvalue
    (set `local.Local_TraceHitLocation` _location)
    (bind _output_get (set `local.Local_TraceHitActor` _hitactor))
    (if (`KismetSystemLibrary.DoesImplementInterface` _output_get "/Game/TowerDefenseStarterKit/Blueprints/GridSystems/BPI_GridLink.BPI_GridLink_C")
      (bind (_gridcellindex _gridgeneratorindex) (message `/Game/TowerDefenseStarterKit/Blueprints/GridSystems/BPI_GridLink.RetrieveTraceHitGridData` (`local.Local_TraceHitActor`) (`local.Local_TraceHitLocation`)))
      (set `self.SelectedGridCellIndex` _gridcellindex)
      (set `self.SelectedGridGeneratorIndex` _gridgeneratorindex)
      (bind _gridcelldata (`/Game/TowerDefenseStarterKit/Blueprints/GridSystems/BP_GridManager.GetGridCellData` (`/Game/TowerDefenseStarterKit/Blueprints/FunctionLibraries/BPFL_GetterFunctions.GetGridManager` self) (`self.SelectedGridCellIndex`) (`self.SelectedGridGeneratorIndex`)))
      (switch `/Game/TowerDefenseStarterKit/Blueprints/GridSystems/EGridCellStatus` (`.GridStatus_19_98EF95C8445FE5D7AFA485AD4114B12F` (break `/Game/TowerDefenseStarterKit/Blueprints/GridSystems/Struct_GridCellData` _gridcelldata))
        (:`NewEnumerator0`
          (set `self.SelectedActor` null)
          (set `local.Local_SelectedActorType` "NewEnumerator2"))
        (:`NewEnumerator1`
          (set `self.SelectedActor` (`.TowerActor_20_DAC62711485A5B07DF08158DC082D797` (break `/Game/TowerDefenseStarterKit/Blueprints/GridSystems/Struct_GridCellData` _gridcelldata)))
          (set `local.Local_SelectedActorType` "NewEnumerator1")))
      (elif (`KismetSystemLibrary.DoesImplementInterface` (`local.Local_TraceHitActor`) "/Game/TowerDefenseStarterKit/Blueprints/HUDControl/BPI_TargetInfoDisplay.BPI_TargetInfoDisplay_C")
        (set `self.SelectedActor` (`local.Local_TraceHitActor`))
        (set `local.Local_SelectedActorType` "NewEnumerator3")
        (else
          (set `self.SelectedActor` null :!label _label)
          (set `local.Local_SelectedActorType` "NewEnumerator4"))))
    (else
      (goto _label)))
  (return (`local.Local_SelectedActorType`)))

(fn `InitializePlayerController`
  (params (GlobalAbilitiesManager :type "/Game/TowerDefenseStarterKit/Blueprints/GlobalAbilities/BP_GlobalAbilitiesManager Object Reference"))
  (locals (Local_SpawnTransform :type "Transform Structure"))
  ;[0 1 1 0.5] Initialize Player Controller - Sets Input Mode to accept both game & UI interaction; Spawn Grid Cell Detector & store a reference to it
  (set `self.GlobalAbilitiesManager` GlobalAbilitiesManager)
  (`WidgetBlueprintLibrary.SetInputMode_GameAndUIEx` self (`/Game/TowerDefenseStarterKit/Blueprints/FunctionLibraries/BPFL_GetterFunctions.GetActiveHUDWidget` self) "LockAlways" false)
  (bind _returnvalue (`|SpawnActorFromClass` "/Game/TowerDefenseStarterKit/Blueprints/Misc/BP_GridCellHighlighter.BP_GridCellHighlighter_C" (`KismetMathLibrary.MakeTransform` (0.0 0.0 0.0)) "AlwaysSpawn" "OverrideRootScale" null null))
  (set `self.GridCellHighlighter` _returnvalue)
  (`self.EnableGridCellDetection`)
  (bind _returnvalue_2 (`|SpawnActorFromClass` "/Game/TowerDefenseStarterKit/Blueprints/Misc/BP_TargetingReticule.BP_TargetingReticule_C" (`self.GetTransform` (`GameplayStatics.GetPlayerPawn` 0)) "AlwaysSpawn" "OverrideRootScale" null null))
  (set `self.TargetingReticule` _returnvalue_2)
  (bind _returnvalue_3 (`KismetSystemLibrary.K2_SetTimer` null "WaitForViewportInitialization" 0.04 true)) ; Start timer to check if viewport has been initialized [viewport size is required for edge scrolling]
  (set `self.ViewportCheckTimerHandle` _returnvalue_3)
  (return))

(fn `IsGlobalAbilityTargetingActive?`
  (returns (ReturnValue :type Boolean))
  ;[0 1 1 0.5] Returns if the Global Ability Targeting system is active or not
  (return (`KismetSystemLibrary.K2_TimerExistsHandle` (`self.UpdateTargetingReticuleTimerHandle`))))

(fn `ManageSelectedActorInteraction`
  (bind _towermanager (`/Game/TowerDefenseStarterKit/Blueprints/FunctionLibraries/BPFL_GetterFunctions.GetTowerManager` self))
  ;[0 1 1 0.5] Identifies the selected actor & handles the interactions accordingly
  (if (`self.GetGridCellDetectionStatus`)
    (bind _selectedactortype (`self.GetSelectedActorDetails`))
    (switch `/Game/TowerDefenseStarterKit/Blueprints/Player/ESelectedActorType` _selectedactortype
      (:`NewEnumerator2`
        (`self.DisableGridCellDetection`)
        (`/Game/TowerDefenseStarterKit/Blueprints/Misc/BP_GridCellHighlighter.HighlightGridCellAtIndex` (`self.GridCellHighlighter`) (`self.SelectedGridCellIndex`) (`self.SelectedGridGeneratorIndex`))
        (`/Game/TowerDefenseStarterKit/Blueprints/Towers/BP_TowerManager.InitiateTowerCreationSystem` (`/Game/TowerDefenseStarterKit/Blueprints/FunctionLibraries/BPFL_GetterFunctions.GetTowerManager` self) (`self.SelectedGridCellIndex`) (`self.SelectedGridGeneratorIndex`))
        (`self.UpdateHUD_HideTargetStats`))
      (:`NewEnumerator1`
        (`self.DisableGridCellDetection`)
        (`/Game/TowerDefenseStarterKit/Blueprints/Misc/BP_GridCellHighlighter.HighlightGridCellAtIndex` (`self.GridCellHighlighter`) (`self.SelectedGridCellIndex`) (`self.SelectedGridGeneratorIndex`))
        (`self.NewTargetSelected` (`self.SelectedActor`))
        (bind _asbp_tower_parent (cast `/Game/TowerDefenseStarterKit/Blueprints/Towers/BP_Tower_Parent` (`self.SelectedActor`)))
        (bind _towermodel (`/Game/TowerDefenseStarterKit/Blueprints/Towers/BP_Tower_Parent.TowerModel` _asbp_tower_parent))
        (`/Game/TowerDefenseStarterKit/Blueprints/Towers/BP_TowerManager.InitiateTowerControlSystem` _towermanager _towermodel (`self.SelectedGridCellIndex`) (`self.SelectedGridGeneratorIndex`))
        (`/Game/TowerDefenseStarterKit/Blueprints/Towers/BP_TowerManager.DisplayRangeForTowerModel` _towermanager _towermodel))
      (:`NewEnumerator3`
        (`/Game/TowerDefenseStarterKit/Blueprints/Towers/BP_TowerManager.StopTowerConstructionSystems` (`/Game/TowerDefenseStarterKit/Blueprints/FunctionLibraries/BPFL_GetterFunctions.GetTowerManager` self))
        (`self.EnableGridCellDetection`)
        (`self.NewTargetSelected` (`self.SelectedActor`)))
      (:`NewEnumerator4`
        (`self.SetDefaultUIState`)))
    (else
      (`self.SetDefaultUIState`))))

(fn `SetDefaultUIState`
  ;[0 1 1 0.5] Set the in game UI to it's default state
  (`/Game/TowerDefenseStarterKit/Blueprints/Towers/BP_TowerManager.StopTowerConstructionSystems` (`/Game/TowerDefenseStarterKit/Blueprints/FunctionLibraries/BPFL_GetterFunctions.GetTowerManager` self))
  (`self.EnableGridCellDetection`)
  (`self.UpdateHUD_HideTargetStats`)
  (return))

(fn `UpdateGlobalAbilityTargetingReticule`
  (bind (_hitresult _returnvalue) (`self.GetHitResultUnderCursorByChannel` "TraceTypeQuery3" false))
  (bind (_bblockinghit _binitialoverlap _time _distance _location _impactpoint _normal _impactnormal _physmat _hitactor) (`GameplayStatics.BreakHitResult` _hitresult))
  ;[0 1 1 0.5] Display/hide global ability targeting reticule based on the underlying platform
  (if _returnvalue
    (`/Game/TowerDefenseStarterKit/Blueprints/Misc/BP_TargetingReticule.DisplayTargetingReticule` (`self.TargetingReticule`) _location (`KismetSystemLibrary.DoesImplementInterface` _hitactor (`/Game/TowerDefenseStarterKit/Blueprints/Misc/BP_TargetingReticule.GetGlobalAbilityTargetInterface` (`self.TargetingReticule`))))))

(fn `UpdateHUD_HideTargetStats`
  ;[0 1 1 0.5] Request the Active HUD Widget to hide the target stats UI element
  (bind _aswidget_game_hud (cast `/Game/TowerDefenseStarterKit/UI/PlayerHUD/Widget_GameHUD` (`/Game/TowerDefenseStarterKit/Blueprints/FunctionLibraries/BPFL_GetterFunctions.GetActiveHUDWidget` self)))
  (`/Game/TowerDefenseStarterKit/UI/PlayerHUD/Widget_GameHUD.HideTargetInfo` _aswidget_game_hud))

(fn `UserConstructionScript`)

(fn `WaitForViewportInitialization`
  (bind (_returnvalue_x _returnvalue_y) (`KismetMathLibrary.BreakVector2D` (`WidgetLayoutLibrary.GetViewportSize`)))
  ;[0 1 1 0.5] Check if viewport size returns zero; If not clear the timer & initialize player pawn
  (if (not (== (* _returnvalue_x _returnvalue_y) 0.0))
    (`KismetSystemLibrary.K2_ClearAndInvalidateTimerHandle` (`self.ViewportCheckTimerHandle`))
    (bind _asbp_player_pawn (cast `/Game/TowerDefenseStarterKit/Blueprints/Player/BP_PlayerPawn` (`GameplayStatics.GetPlayerPawn` 0)))
    (`/Game/TowerDefenseStarterKit/Blueprints/Player/BP_PlayerPawn.InitializePlayerPawn` _asbp_player_pawn)
    (`self.EnableInput` _asbp_player_pawn self)))