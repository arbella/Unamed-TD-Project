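; BP_GridManager holds the tower defense level's grid state, recording the position, tower and status of every cell.
; InitializeGridManager, called manually instead of on BeginPlay, gathers and indexes all grid generators, builds GridData from their cell vectors, then has each display its cells.
; UpdateGridData copies a generator's cell array, replaces one entry and writes the nested struct back.
; Getters expose grid data, generators, single cells and cell size, with half-size precomputed at construction.
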(fn `GetGridCellData`
  (params (GridCellIndex :type Integer) (GridGeneratorIndex :type Integer))
  (returns (GridCellData :type "/Game/TowerDefenseStarterKit/Blueprints/GridSystems/Struct_GridCellData Structure"))
  ;[0 1 1 0.5] Version 2.8: Returns grid information associated with the specified cell and generator
  (return (`|GetArrayItem` (`.GridGeneratorData_11_13E757544C1E18F1261E9C9C7CA2FC04` (break `/Game/TowerDefenseStarterKit/Blueprints/GridSystems/Struct_GridData` (`|GetArrayItem` (`self.GridData`) GridGeneratorIndex))) GridCellIndex)))

(fn `GetGridCellSize`
  (returns (GridCellSize :type "Float (double-precision)"))
  (return (`self.GridCellSize`)))

(fn `GetGridData`
  (returns (GridDataArray :type "Array of /Game/TowerDefenseStarterKit/Blueprints/GridSystems/Struct_GridData Structure"))
  ;[0 1 1 0.5] Returns an array containing information about the entire grid system in the level
  (return (`self.GridData`)))

(fn `GetGridGenerators`
  (returns (GridGeneratorArray :type "Array of /Game/TowerDefenseStarterKit/Blueprints/GridSystems/BP_GridGenerator Object Reference"))
  ;[0 1 1 0.5] Returns an array containing references to all grid generators in the level
  (return (`self.GridGenerators`)))

(fn `GetHalfGridCellSize`
  (returns (HalfGridCellSize :type "Float (double-precision)"))
  (return (`self.HalfGridCellSize`)))

(fn `InitializeGridData`
  (locals (Local_GridGeneratorData :type "Array of /Game/TowerDefenseStarterKit/Blueprints/GridSystems/Struct_GridCellData Structure"))
  ;[0 1 1 0.5] Set up the base template for Grid Data Array using the Grid Generators placed throughout the level
  (bind _outactors (`GameplayStatics.GetAllActorsOfClass` (`self.GridGeneratorClass`)))
  (bind _output_get (set `self.GridGenerators` _outactors))
  (for (_array_element _array_index) _output_get
    (`/Game/TowerDefenseStarterKit/Blueprints/GridSystems/BP_GridGenerator.SetGeneratorIndex` _array_element _array_index)
    (for _array_element_2 (`/Game/TowerDefenseStarterKit/Blueprints/GridSystems/BP_GridGenerator.GetGridVectorArray` _array_element)
      (`KismetArrayLibrary.Array_Add` (`local.Local_GridGeneratorData`) (make `/Game/TowerDefenseStarterKit/Blueprints/GridSystems/Struct_GridCellData` _array_element_2)))
    (`KismetArrayLibrary.Array_Add` (`self.GridData`) (make `/Game/TowerDefenseStarterKit/Blueprints/GridSystems/Struct_GridData` (`/Game/TowerDefenseStarterKit/Blueprints/GridSystems/BP_GridGenerator.GetGridGeneratorIndex` _array_element) (`local.Local_GridGeneratorData`) _array_element))
    (`KismetArrayLibrary.Array_Clear` (`local.Local_GridGeneratorData`)))
  (return))

(fn `InitializeGridManager`
  ;[0 1 1 0.5] Used to initialize the Grid Manager manually instead of relying on the Begin Play Event
  (`self.InitializeGridData`)
  (for _array_element (`self.GridGenerators`)
    (`/Game/TowerDefenseStarterKit/Blueprints/GridSystems/BP_GridGenerator.DisplayGridCells` _array_element))
  (return))

(fn `UpdateGridData`
  (params (GridCellIndex :type Integer) (GridGeneratorIndex :type Integer) (Tower :type "/Game/TowerDefenseStarterKit/Blueprints/Towers/BP_Tower_Parent Object Reference") (GridStatus :type "/Game/TowerDefenseStarterKit/Blueprints/GridSystems/EGridCellStatus Enum" :default "NewEnumerator0"))
  (locals (Local_GridGeneratorData :type "Array of /Game/TowerDefenseStarterKit/Blueprints/GridSystems/Struct_GridCellData Structure") (Local_GridCellIndex :type Integer) (Local_GridGeneratorIndex :type Integer))
  (bind ((`GeneratorIndex_9_04C183AE4F7B8E23A5CDB4AA42FF3348` _generatorindex) (`GridGenerator_13_116FE1614615A5B5C63B70B45CFF220B` _gridgenerator)) (break `/Game/TowerDefenseStarterKit/Blueprints/GridSystems/Struct_GridData` (`|GetArrayItem` (`self.GridData`) (`local.Local_GridGeneratorIndex`))))
  ;[0 1 1 0.5] Updates Grid Data Array
  (set `local.Local_GridCellIndex` GridCellIndex)
  (set `local.Local_GridGeneratorIndex` GridGeneratorIndex)
  (set `local.Local_GridGeneratorData` (`.GridGeneratorData_11_13E757544C1E18F1261E9C9C7CA2FC04` (break `/Game/TowerDefenseStarterKit/Blueprints/GridSystems/Struct_GridData` (`|GetArrayItem` (`self.GridData`) (`local.Local_GridGeneratorIndex`)))))
  (`KismetArrayLibrary.Array_Set` (`local.Local_GridGeneratorData`) (`local.Local_GridCellIndex`) (make `/Game/TowerDefenseStarterKit/Blueprints/GridSystems/Struct_GridCellData` (`.GridVector_10_7F7B6B8542ECC301E9FFB082D723054A` (break `/Game/TowerDefenseStarterKit/Blueprints/GridSystems/Struct_GridCellData` (`|GetArrayItem` (`local.Local_GridGeneratorData`) (`local.Local_GridCellIndex`)))) Tower GridStatus))
  (`KismetArrayLibrary.Array_Set` (`self.GridData`) (`local.Local_GridGeneratorIndex`) (make `/Game/TowerDefenseStarterKit/Blueprints/GridSystems/Struct_GridData` _generatorindex (`local.Local_GridGeneratorData`) _gridgenerator))
  (return))

(fn `UserConstructionScript`
  (set `self.HalfGridCellSize` (/ (`self.GridCellSize`) 2.0)) ; Stored as a variable to prevent the need for runtime calculations to get this value
)