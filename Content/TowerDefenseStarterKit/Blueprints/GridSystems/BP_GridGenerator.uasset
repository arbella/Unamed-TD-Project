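; Placeable tower-placement grid for the tower defense kit, sized by user-set X and Y cell counts and the cell size from BP_GridManager.
; Construction scales the platform, builds an array of cell centers along its axes, adds an instanced cell mesh at each, and optionally blocks a global-ability trace channel.
; RetrieveTraceHitGridData (BPI_GridLink) projects a hit location onto the actor's axes to return cell and generator indices.
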(fn `CreateGridArray`
  (bind _gridsize (`self.GridSize`))
  (bind _gridplatform (`self.GridPlatform`))
  (bind _returnvalue (/ _gridsize 2.0))
  (bind _returnvalue_2 (/ (`self.GridSize`) 2.0))
  ;[0 1 1 0.5] Calculates Grid Details based on the grid size, grid count & actor transform
  (set `self.StartingVector` (+ (- (- (`KismetSystemLibrary.GetComponentBounds` (`self.GridPlatform`)) (* (`SceneComponent.GetRightVector` (`self.GridPlatform`)) (* _returnvalue_2 (`KismetMathLibrary.Conv_IntToDouble` (`self.GridCountY`))))) (* (`SceneComponent.GetForwardVector` _gridplatform) (* _returnvalue_2 (`KismetMathLibrary.Conv_IntToDouble` (`self.GridCountX`))))) (`SceneComponent.GetUpVector` _gridplatform)))
  (for _index (range (`self.GridCountX`))
    (for _index_2 (range (`self.GridCountY`))
      (`KismetArrayLibrary.Array_Add` (`self.GridVectorArray`) (+ (`self.StartingVector`) (+ (* (`SceneComponent.GetRightVector` (`self.GridPlatform`)) (+ (* _index_2 _gridsize) _returnvalue)) (* (`SceneComponent.GetForwardVector` (`self.GridPlatform`)) (+ (* _index _gridsize) _returnvalue)))))))
  (return))

(fn `DisplayGridCells`
  ;[0 1 1 0.5] Display Grid Cells
  (`SceneComponent.SetHiddenInGame` (`self.GridCell`) false false)
  (return))

(fn `GetGridGeneratorIndex`
  (returns (GeneratorIndex :type Integer))
  (return (`self.GeneratorIndex`)))

(fn `GetGridVectorArray`
  (returns (GridVectorArray :type "Array of Vector Structure"))
  (return (`self.GridVectorArray`)))

(fn `RetrieveTraceHitGridData`
  (params (TraceHitLocation :type "Vector Structure"))
  (returns (GridCellIndex :type Integer) (GridGeneratorIndex :type Integer))
  (locals (Local_GridCellIndex :type Integer))
  (bind _gridsize (`self.GridSize`))
  (bind _startingvector (`self.StartingVector`))
  ;[0 1 0.4 0.5] 'BPI_GridLink' interface function used to retrieve grid data of the implementing actor
  (set `local.Local_GridCellIndex` (+ (* (`self.GridCountY`) (`KismetMathLibrary.FFloor` (/ (`KismetMathLibrary.VSize` (`KismetMathLibrary.ProjectVectorOnToVector` (- TraceHitLocation _startingvector) (`self.GetActorForwardVector`))) _gridsize))) (`KismetMathLibrary.FFloor` (/ (`KismetMathLibrary.VSize` (`KismetMathLibrary.ProjectVectorOnToVector` (- TraceHitLocation _startingvector) (`self.GetActorRightVector`))) _gridsize))))
  (return (`local.Local_GridCellIndex`) (`self.GeneratorIndex`)))

(fn `SetGeneratorIndex`
  (params (Index :type Integer))
  (set `self.GeneratorIndex` Index)
  (return))

(fn `UserConstructionScript`
  (bind _gridsize (`self.GridSize`))
  (bind _gridsize_2 (`self.GridSize`))
  (bind _gridplatform (`self.GridPlatform`))
  (bind (_min _max) (`StaticMeshComponent.GetLocalBounds` (`self.GridPlatform`)))
  (bind (_min_2 _max_2) (`StaticMeshComponent.GetLocalBounds` (`self.GridCell`)))
  ;[0 1 1 0.5] Scales the Grid Floor based on the user defined grid counts in X & Y directions; Create Grid Instances for visualizing Tower Placement locations during level design
  (bind _outactors (`GameplayStatics.GetAllActorsOfClass` "/Game/TowerDefenseStarterKit/Blueprints/GridSystems/BP_GridManager.BP_GridManager_C"))
  (set `self.GridSize` (`/Game/TowerDefenseStarterKit/Blueprints/GridSystems/BP_GridManager.GetGridCellSize` (`|GetArrayItem` _outactors))) ; Used to scale the Grid Mesh
  (set `self.DefaultGridMeshBounds` (- _max _min))
  (`SceneComponent.SetWorldScale3D` (`self.GridPlatform`) (`KismetMathLibrary.MakeVector` (/ (* (`KismetMathLibrary.Conv_IntToDouble` (`self.GridCountX`)) _gridsize) (.x (`self.DefaultGridMeshBounds`))) (/ (* (`KismetMathLibrary.Conv_IntToDouble` (`self.GridCountY`)) _gridsize) (.y (`self.DefaultGridMeshBounds`))) 1.0)) ; Set grid platform scale based on the grid size
  (`self.CreateGridArray`)
  (`SceneComponent.SetWorldScale3D` (`self.GridCell`) (`KismetMathLibrary.MakeVector` (* (/ _gridsize_2 (.x (- _max_2 _min_2))) 0.9) (* (/ _gridsize_2 (.y (- _max_2 _min_2))) 0.9) 1.0)) ; Set grid cell platform scale based on the grid size
  (for _array_element (`self.GridVectorArray`)
    (`InstancedStaticMeshComponent.AddInstanceWorldSpace` (`self.GridCell`) (`KismetMathLibrary.MakeTransform` (`KismetMathLibrary.MakeVector` (.x _array_element) (.y _array_element) (.z _array_element)) (`self.K2_GetActorRotation`) (`SceneComponent.K2_GetComponentScale` (`self.GridCell`)))))
  (if (`self.BlockGlobalAbilityDeployment?`)
    (`PrimitiveComponent.SetCollisionResponseToChannel` _gridplatform "ECC_GameTraceChannel6" "ECR_Block")
    (else
      (`PrimitiveComponent.SetCollisionResponseToChannel` _gridplatform "ECC_GameTraceChannel6" "ECR_Ignore"))))