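; Friendly Tower Guardian AI unit that hunts wave enemies until its lifespan expires or its health runs out.
; Visual Perception picks targets from the spawn controller's enemy list, favouring ones not combat-locked, then triggers Threat Response to move and attack.
; It claims a combat lock on its target, halting vision checks on success or retrying by looping timer on failure.
; Incoming damage updates a 3D health bar and ignores player-controller-instigated hits such as airstrikes.
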(event `self.ReceiveBeginPlay`
  ;[0 1 1 0.5] Initialize the default parameters & issue move order towards the Exit Point
  (bind _aswidget_3dstats_bar (cast `/Game/TowerDefenseStarterKit/UI/Generic/Widget_3DStatsBar` (`WidgetComponent.GetUserWidgetObject` (`self.3DStatsBar`))))
  (`/Game/TowerDefenseStarterKit/UI/Generic/Widget_3DStatsBar.InitializeHealthBar` _aswidget_3dstats_bar (struct :`G` 1.0 :`B` 1.0 :`A` 1.0) 1.0)
  (`KismetSystemLibrary.Delay` (`self.LifeSpan`))
  (`self.K2_DestroyActor`) ; Destroy actor once it's lifespan has expired
)

(event `/Game/TowerDefenseStarterKit/Blueprints/GenericSystems/BPI_DamageApplicationSystem.ApplyDirectDamage`
  (params (BaseDamage :type "Float (single-precision)") (CritChance :type "Float (single-precision)") (CritDamageMultiplier :type "Float (single-precision)") (DamagedCauser :type "Actor Object Reference") (EventInstigator :type "Controller Object Reference"))
  ;[1 0 0 0.5] Receive Damage/Update Health Bar Widget; Destroy self if health becomes less than or equal to zero
  (if (not (== EventInstigator (`GameplayStatics.GetPlayerController` 0)))
    (`self.UpdateHealth` (* (`/Game/TowerDefenseStarterKit/Blueprints/GenericSystems/BPC_DamageCalculator.CalculateFinalDamage` (`self.DamageCalculator`) BaseDamage CritChance CritDamageMultiplier) -1.0))
    (if (not (> (`self.UnitHealth`) 0.0))
      (`/Engine/EditorBlueprintResources/StandardMacros.DoOnce` false ; Ensures that termination protocols get called only once
        (:`Completed`
          (`self.K2_DestroyActor`))))))

(event `/Game/TowerDefenseStarterKit/Blueprints/AI/BPI_VisualPerception.UpdateVisualPerceptionData`
  (params (TargetActor :type "Actor Object Reference"))
  ;[0 1 0.4 0.5] BPI_VisualPerception interface function - Visual Perception relays the latest information it possesses over to it's owning actor
  (`/Engine/EditorBlueprintResources/StandardMacros.IsValid` TargetActor
    (:`Is Valid`
      (`self.StopCombatLockActivationTimer`)
      (set `self.ActiveTarget` TargetActor)
      (`/Game/TowerDefenseStarterKit/Blueprints/AI/BPC_ThreatResponse.ActivateThreatResponse` (`self.ThreatResponse`)) ; Activates Threat Response if Visual Perception component provides a relevant target
    )))

(event `/Game/TowerDefenseStarterKit/Blueprints/AI/BPI_ThreatResponse.PerformAttackOrderPreconditions`
  ;[0 1 0.4 0.5] BPI_ThreatResponse functions
  (bind _success_ (message `/Game/TowerDefenseStarterKit/Blueprints/AI/BPI_CombatLock.ActivateCombatLock` (`self.ActiveTarget`) self)) ; Attempts to lock on to the new target before activating Threat Response
  (if _success_
    (`/Game/TowerDefenseStarterKit/Blueprints/AI/BPC_VisualPerception.StopVisionCheck` (`self.VisualPerception`)) ; Stop Visual Perception calculations once a target is confirmed for Threat Response evaluation
    (else
      (`self.StartCombatLockActivationTimer`) ; If the combat lock attempt failed, start a timer to continuously keep attempting to lock in as long as the said target is relevant
    ))
  (`self.MoveToActiveTarget`))

(event `/Game/TowerDefenseStarterKit/Blueprints/AI/BPI_ThreatResponse.AttackActiveTarget`
  ;[0 1 0.4 0.5] BPI_ThreatResponse functions
  (message `/Game/TowerDefenseStarterKit/Blueprints/GenericSystems/BPI_DamageApplicationSystem.ApplyDirectDamage` (`self.ActiveTarget`) (`self.AttackDamage`) (`self.CritHitChance`) (`self.CritHitDamageMultiplier`) self (`AIBlueprintHelperLibrary.GetAIController` self))
  (`KismetSystemLibrary.Delay` (`self.AttackAnimationDuration`))
  (`/Game/TowerDefenseStarterKit/Blueprints/AI/BPC_ThreatResponse.AttackOrderExecuted` (`self.ThreatResponse`) true))

(event `/Game/TowerDefenseStarterKit/Blueprints/AI/BPI_ThreatResponse.RevertToDefaultState`
  ;[0 1 0.4 0.5] BPI_ThreatResponse functions
  (`self.StopCombatLockActivationTimer`)
  (set `self.ActiveTarget` null)
  (`/Game/TowerDefenseStarterKit/Blueprints/AI/BPC_VisualPerception.ActivateVisualPerception` (`self.VisualPerception`)))

(event `/Game/TowerDefenseStarterKit/Blueprints/AI/BPI_ThreatResponse.CancelMovement`
  ;[0 1 0.4 0.5] BPI_ThreatResponse functions
  (`Controller.StopMovement` (`AIBlueprintHelperLibrary.GetAIController` self)))

(fn `EvaluateVisualPerceptionTargets`
  (params (MaxPriorityTarget :type "Actor Object Reference") (NewTarget :type "Actor Object Reference") (DistanceToMaxPriorityTarget :type "Float (double-precision)") (DistanceToNewTarget :type "Float (double-precision)"))
  (returns (NewMaxPriorityTarget :type "Actor Object Reference") (DistanceToNewMaxPriorityTarget :type "Float (double-precision)") (`SearchForMoreTargets?` :type Boolean))
  (locals (Local_ExistingMaxPriorityTarget :type "Actor Object Reference") (Local_NewTarget :type "Actor Object Reference") (Local_DistanceToExistingMaxPriorityTarget :type "Float (double-precision)") (Local_DistanceToNewTarget :type "Float (double-precision)"))
  (bind _local_newtarget (`local.Local_NewTarget`))
  ;[0 1 0.4 0.5] BPI_VisualPerception interface function - Evaluates threat priority levels between different targets analyzed by the Visual Perception component
  (set `local.Local_ExistingMaxPriorityTarget` MaxPriorityTarget)
  (set `local.Local_NewTarget` NewTarget)
  (set `local.Local_DistanceToExistingMaxPriorityTarget` DistanceToMaxPriorityTarget)
  (set `local.Local_DistanceToNewTarget` DistanceToNewTarget)
  (`/Engine/EditorBlueprintResources/StandardMacros.IsValid` (`self.ActiveTarget`)
    (:`Is Valid`
      (bind _islockedincombat_ (message `/Game/TowerDefenseStarterKit/Blueprints/AI/BPI_CombatLock.RetrieveCombatLockStatus` _local_newtarget))
      (if _islockedincombat_
        _
        (else
          (return (`local.Local_NewTarget`) (`local.Local_DistanceToNewTarget`) false) ; If the new target can be locked in to combat, then set it as the highest priority potential target & cancel further analysis in the current visual perception cycle
        )))
    (:`Is Not Valid`
      (bind _islockedincombat__2 (message `/Game/TowerDefenseStarterKit/Blueprints/AI/BPI_CombatLock.RetrieveCombatLockStatus` _local_newtarget))
      (if _islockedincombat__2
        (`/Engine/EditorBlueprintResources/StandardMacros.IsValid` (`local.Local_ExistingMaxPriorityTarget`)
          (:`Is Valid`
            _)
          (:`Is Not Valid`
            (return (`local.Local_NewTarget`) (`local.Local_DistanceToNewTarget`) true) ; If no max priority target exists, set the new target as the new max priority target & keep searching for more potential targets
          ))
        (else
          (return (`local.Local_NewTarget`) (`local.Local_DistanceToNewTarget`) false) ; If the new target can be locked in to combat, then set it as the highest priority potential target & cancel further analysis in the current visual perception cycle
        ))))
  (return (`local.Local_ExistingMaxPriorityTarget`) (`local.Local_DistanceToExistingMaxPriorityTarget`) true) ; If the new target cannot be locked in, do not make any changes & keep searching for more potential targets
)

(fn `GetMovementSpeed`
  (returns (ReturnValue :type "Float (double-precision)"))
  ;[0 1 1 0.5] Version 2_8_2: Returns the movement speed
  (return (`KismetMathLibrary.VSize` (`self.GetVelocity`))))

(fn `LockOnToActiveTarget`
  ;[0 1 1 0.5] Attempts to lock on to the active target [Used when the active target is already locked in combat with another entity]
  (`/Engine/EditorBlueprintResources/StandardMacros.IsValid` (`self.ActiveTarget`)
    (:`Is Valid`
      (bind _success_ (message `/Game/TowerDefenseStarterKit/Blueprints/AI/BPI_CombatLock.ActivateCombatLock` (`self.ActiveTarget`) self)) ; Attempts to lock on to the active target
      (if _success_
        (`self.StopCombatLockActivationTimer`) ; Once the target has been locked, stop the combat lock activation timer
      ))))

(fn `MoveToActiveTarget`
  (bind _activetarget (`self.ActiveTarget`))
  ;[0 1 1 0.5] Move towards the Active Target
  (`/Engine/EditorBlueprintResources/StandardMacros.IsValid` _activetarget
    (:`Is Valid`
      (`AIController.MoveToActor` (`AIBlueprintHelperLibrary.GetAIController` self) _activetarget -1.0 true true false null true))
    (:`Is Not Valid`
      _))
  (return))

(fn `RetrieveTargetInfo`
  (returns (Name :type Text) (Description :type Text) (Stats :type "Array of /Game/TowerDefenseStarterKit/Blueprints/HUDControl/Struct_HUDStats Structure"))
  ;[0 1 0.4 0.5] BPI_TargetInfoDisplay interface function
  (return (`self.ObjectName`) (`self.ObjectDescription`) (`|MakeArray` (make `/Game/TowerDefenseStarterKit/Blueprints/HUDControl/Struct_HUDStats` "Damage" (`KismetTextLibrary.Conv_DoubleToText` (`self.AttackDamage`) "HalfToEven")) (make `/Game/TowerDefenseStarterKit/Blueprints/HUDControl/Struct_HUDStats` "Health" (`KismetTextLibrary.Conv_DoubleToText` (`self.UnitHealth`) "HalfToEven")))))

(fn `RetrieveTargetingSystemData`
  (returns (ActiveTarget :type "Actor Object Reference") (AttackRange :type "Float (double-precision)"))
  ;[0 1 0.4 0.5] BPI_ThreatResponse interface function - Returns information necessary for threat response evaluation
  (return (`self.ActiveTarget`) (`self.AttackRange`)))

(fn `RetrieveVisualPerceptionRequisites`
  (returns (VisionRange :type "Float (double-precision)") (VisionAngle :type "Float (double-precision)") (PotentialTargets :type "Array of Actor Object Reference"))
  ;[0 1 0.4 0.5] BPI_VisualPerception interface function - Returns information pertinent to visual perception calculation
  (return (`self.VisionRange`) (`self.VisionAngle`) (`/Game/TowerDefenseStarterKit/Blueprints/WaveSpawningSystems/BP_WaveSpawnController.GetEnemyUnitList` (`/Game/TowerDefenseStarterKit/Blueprints/FunctionLibraries/BPFL_GetterFunctions.GetWaveSpawnController` self))))

(fn `StartCombatLockActivationTimer`
  ;[0 1 1 0.5] Starts the Combat Lock activation timer
  (if (not (`KismetSystemLibrary.K2_TimerExistsHandle` (`self.CombatLockActivationTimerHandle`)))
    (bind _returnvalue (`KismetSystemLibrary.K2_SetTimer` null "LockOnToActiveTarget" 0.1 true))
    (set `self.CombatLockActivationTimerHandle` _returnvalue)))

(fn `StopCombatLockActivationTimer`
  (bind _combatlockactivationtimerhandle (`self.CombatLockActivationTimerHandle`))
  ;[0 1 1 0.5] Stops the Combat Lock activation timer
  (if (`KismetSystemLibrary.K2_TimerExistsHandle` _combatlockactivationtimerhandle)
    (`KismetSystemLibrary.K2_ClearAndInvalidateTimerHandle` _combatlockactivationtimerhandle)))

(fn `UpdateHealth`
  (params (Increment :type "Float (double-precision)"))
  ;[0 1 1 0.5] Updates the health based on the input parameter
  (set `self.UnitHealth` (`KismetMathLibrary.FClamp` (+ Increment (`self.UnitHealth`)) 0.0 (`self.MaxHealth`)))
  (bind _aswidget_3dstats_bar (cast `/Game/TowerDefenseStarterKit/UI/Generic/Widget_3DStatsBar` (`WidgetComponent.GetUserWidgetObject` (`self.3DStatsBar`)))
    (:`then`
      (`/Engine/EditorBlueprintResources/StandardMacros.IsValid` _aswidget_3dstats_bar
        (:`Is Valid`
          (`/Game/TowerDefenseStarterKit/UI/Generic/Widget_3DStatsBar.UpdateHealthBar` _aswidget_3dstats_bar (/ (`self.UnitHealth`) (`self.MaxHealth`))))
        (:`Is Not Valid`
          _))
      (return))
    (:`CastFailed`
      (return))))

(fn `UserConstructionScript`
  (set `self.UnitHealth` (`self.MaxHealth`)))