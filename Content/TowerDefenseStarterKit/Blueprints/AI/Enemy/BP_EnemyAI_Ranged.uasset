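; Ranged enemy AI unit for the tower defense game that spots towers and shoots projectiles at its target.
; Visual Perception picks the nearest tower and activates Threat Response, which pauses vision checks and fires through the Projectile Spawn Controller.
; Towers are attacked once per activation, other targets repeatedly; on reverting to default, vision resumes after a delay unless locked in combat.
; It also supplies name, description and stats to the target info display.
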(event `/Game/TowerDefenseStarterKit/Blueprints/AI/BPI_VisualPerception.UpdateVisualPerceptionData`
  (params (TargetActor :type "Actor Object Reference"))
  ;[0 1 0.4 0.5] BPI_VisualPerception interface function - Visual Perception relays the latest information it possesses over to it's owning actor
  (`/Engine/EditorBlueprintResources/StandardMacros.IsValid` TargetActor
    (:`Is Valid`
      (set `self.ActiveTarget` TargetActor)
      (`/Game/TowerDefenseStarterKit/Blueprints/AI/BPC_ThreatResponse.ActivateThreatResponse` (`self.ThreatResponse`)) ; Activates Threat Response if Visual Perception component provides a relevant target
    )))

(event `/Game/TowerDefenseStarterKit/Blueprints/AI/BPI_ThreatResponse.AttackActiveTarget`
  (bind _unitcore (`self.UnitCore`))
  (bind _threatresponse (`self.ThreatResponse`))
  (bind _returnvalue (+ (`SceneComponent.K2_GetComponentLocation` _unitcore) (* (`SceneComponent.GetForwardVector` _unitcore) 50.0)))
  ;[0 1 0.4 0.5] BPI_ThreatResponse interface functions
  (`/Game/TowerDefenseStarterKit/Blueprints/Projectiles/BP_ProjectileSpawnController.CreateBulletProjectile` (`/Game/TowerDefenseStarterKit/Blueprints/FunctionLibraries/BPFL_GetterFunctions.GetProjectileSpawnController` self) (`self.AttackDamage`) (`self.CritHitChance`) (`self.CritHitDamageMultiplier`) self (`KismetMathLibrary.MakeTransform` _returnvalue (`KismetMathLibrary.FindLookAtRotation` _returnvalue (`self.K2_GetActorLocation` (`self.ActiveTarget`)))))
  (`KismetSystemLibrary.Delay` (`self.AttackAnimationDuration`)) ; Placeholder delay to simulate real attack animation timeflow
  (cast `/Game/TowerDefenseStarterKit/Blueprints/Towers/BP_Tower_Parent` (`self.ActiveTarget`)
    (:`then`
      (`/Game/TowerDefenseStarterKit/Blueprints/AI/BPC_ThreatResponse.AttackOrderExecuted` _threatresponse false) ; Towers are attacked only once during a single activation of Threat Response
    )
    (:`CastFailed`
      (`/Game/TowerDefenseStarterKit/Blueprints/AI/BPC_ThreatResponse.AttackOrderExecuted` _threatresponse true) ; Any target except towers will be attacked repeatedly
    )))

(event `/Game/TowerDefenseStarterKit/Blueprints/AI/BPI_ThreatResponse.RevertToDefaultState`
  ;[0 1 0.4 0.5] BPI_ThreatResponse interface functions
  (`parent.RevertToDefaultState`)
  (`KismetSystemLibrary.Delay` 2.0) ; Proceed forward for specified time before reactivating vision check
  (if (not (`self.LockedInCombat?`))
    (`/Game/TowerDefenseStarterKit/Blueprints/AI/BPC_VisualPerception.ActivateVisualPerception` (`self.VisualPerception`))))

(event `/Game/TowerDefenseStarterKit/Blueprints/AI/BPI_ThreatResponse.PerformAttackOrderPreconditions`
  ;[0 1 0.4 0.5] BPI_ThreatResponse interface functions
  (`/Game/TowerDefenseStarterKit/Blueprints/AI/BPC_VisualPerception.StopVisionCheck` (`self.VisualPerception`)) ; Stop Visual Perception calculations once a target is confirmed for Threat Response evaluation
)

(fn `EvaluateVisualPerceptionTargets`
  (params (MaxPriorityTarget :type "Actor Object Reference") (NewTarget :type "Actor Object Reference") (DistanceToMaxPriorityTarget :type "Float (double-precision)") (DistanceToNewTarget :type "Float (double-precision)"))
  (returns (NewMaxPriorityTarget :type "Actor Object Reference") (DistanceToNewMaxPriorityTarget :type "Float (double-precision)") (`SearchForMoreTargets?` :type Boolean))
  ;[0 1 0.4 0.5] BPI_VisualPerception interface function - Evaluates threat priority levels between different targets analyzed by the Visual Perception component
  (`/Engine/EditorBlueprintResources/StandardMacros.IsValid` MaxPriorityTarget ; Check if a max priority target already exists
    (:`Is Valid`
      (if (< DistanceToNewTarget DistanceToMaxPriorityTarget)
        _
        (else
          (return MaxPriorityTarget DistanceToMaxPriorityTarget true) ; If the distance to new target is greater than the distance to the existing max priority target, then make no changes
        )))
    (:`Is Not Valid`
      _))
  (return NewTarget DistanceToNewTarget true) ; If either no max priority target exists, or the distance to new target is less than the distance to the existing max priority target, then set the new target as the max priority target
)

(fn `RetrieveTargetInfo`
  (returns (Name :type Text) (Description :type Text) (Stats :type "Array of /Game/TowerDefenseStarterKit/Blueprints/HUDControl/Struct_HUDStats Structure"))
  ;[0 1 0.4 0.5] BPI_TargetInfoDisplay interface function
  (return (`self.ObjectName`) (`self.ObjectDescription`) (`|MakeArray` (make `/Game/TowerDefenseStarterKit/Blueprints/HUDControl/Struct_HUDStats` "Max Speed" (`KismetTextLibrary.Conv_DoubleToText` (`self.MaxSpeed`) "HalfToEven")) (make `/Game/TowerDefenseStarterKit/Blueprints/HUDControl/Struct_HUDStats` "Health" (`KismetTextLibrary.Conv_DoubleToText` (`self.UnitHealth`) "HalfToEven")) (make `/Game/TowerDefenseStarterKit/Blueprints/HUDControl/Struct_HUDStats` "Attack" (`KismetTextLibrary.Conv_DoubleToText` (`self.AttackDamage`) "HalfToEven")))))

(fn `RetrieveVisualPerceptionRequisites`
  (returns (VisionRange :type "Float (double-precision)") (VisionAngle :type "Float (double-precision)") (PotentialTargets :type "Array of Actor Object Reference"))
  ;[0 1 0.4 0.5] BPI_VisualPerception interface function - Returns information pertinent to visual perception calculation
  (return (`self.VisionRange`) (`self.VisionAngle`) (`/Game/TowerDefenseStarterKit/Blueprints/Towers/BP_TowerManager.Towers` (`/Game/TowerDefenseStarterKit/Blueprints/FunctionLibraries/BPFL_GetterFunctions.GetTowerManager` self))))

(fn `UserConstructionScript`
  (`parent.UserConstructionScript`))