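; Base tower defense enemy that advances to the exit point by nav mesh or timer-driven spline movement, per NavModel.
; Max health scales with the square root of the wave cycle multiplier at construction.
; A combat lock sets one target and activates ThreatResponse, whose interface events halt movement, deal damage and later resume the march.
; Damage updates a 3D health bar; zero health fires a deletion dispatcher once, and EndPlay spawns an explosion.
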(event `self.ReceiveBeginPlay`
  ;[0 1 1 0.5] Initialize the default parameters & issue move order towards the Exit Point
  (bind _aswidget_3dstats_bar (cast `/Game/TowerDefenseStarterKit/UI/Generic/Widget_3DStatsBar` (`WidgetComponent.GetUserWidgetObject` (`self.3DStatsBar`))))
  (`/Game/TowerDefenseStarterKit/UI/Generic/Widget_3DStatsBar.InitializeHealthBar` _aswidget_3dstats_bar (struct :`R` 1.0 :`G` 0.5 :`A` 1.0) 1.0)
  (`self.MoveToExitPoint`))

(event `/Game/TowerDefenseStarterKit/Blueprints/GenericSystems/BPI_DamageApplicationSystem.ApplyDirectDamage`
  (params (BaseDamage :type "Float (single-precision)") (CritChance :type "Float (single-precision)") (CritDamageMultiplier :type "Float (single-precision)") (DamagedCauser :type "Actor Object Reference") (EventInstigator :type "Controller Object Reference"))
  ;[1 0 0 0.5] Receive Damage/Update Health Bar Widget; Destroy self if health becomes less than or equal to zero; Update Tower Points
  (`self.UpdateHealth` (* (`/Game/TowerDefenseStarterKit/Blueprints/GenericSystems/BPC_DamageCalculator.CalculateFinalDamage` (`self.DamageCalculator`) BaseDamage CritChance CritDamageMultiplier) -1.0))
  (if (not (> (`self.UnitHealth`) 0.0))
    (`/Engine/EditorBlueprintResources/StandardMacros.DoOnce` false ; Ensures that termination protocols get called only once
      (:`Completed`
        (`self.ActivateTerminationProtocols` false)))))

(event `self.ReceiveEndPlay`
  (params (EndPlayReason :type "EEndPlayReason Enum" :default "Destroyed"))
  ;[1 0 0 0.5] Spawn Explosion Particle when destroyed
  (`GameplayStatics.SpawnEmitterAtLocation` "/Game/TowerDefenseStarterKit/Effects/Explosion/P_Explosion_Small.P_Explosion_Small" (`self.K2_GetActorLocation`)))

(event `/Game/TowerDefenseStarterKit/Blueprints/AI/BPI_ThreatResponse.AttackActiveTarget`
  ;[0 1 0.4 0.5] BPI_ThreatResponse interface functions
  (message `/Game/TowerDefenseStarterKit/Blueprints/GenericSystems/BPI_DamageApplicationSystem.ApplyDirectDamage` (`self.ActiveTarget`) (`self.AttackDamage`) (`self.CritHitChance`) (`self.CritHitDamageMultiplier`) self (`AIBlueprintHelperLibrary.GetAIController` self))
  (`KismetSystemLibrary.Delay` (`self.AttackAnimationDuration`)) ; Placeholder delay to simulate real attack animation timeflow
  (`/Game/TowerDefenseStarterKit/Blueprints/AI/BPC_ThreatResponse.AttackOrderExecuted` (`self.ThreatResponse`) true) ; Reports to Threat Response that the attack order has been executed
)

(event `/Game/TowerDefenseStarterKit/Blueprints/AI/BPI_ThreatResponse.CancelMovement`
  (bind _splinemovementtimerhandle (`self.SplineMovementTimerHandle`))
  ;[0 1 0.4 0.5] BPI_ThreatResponse interface functions
  (if (`KismetSystemLibrary.K2_TimerExistsHandle` _splinemovementtimerhandle)
    (`KismetSystemLibrary.K2_ClearAndInvalidateTimerHandle` _splinemovementtimerhandle) ; Stop spline movement
    (set `self.SplineMovementSpeed` 0.0)
    (else
      (`Controller.StopMovement` (`AIBlueprintHelperLibrary.GetAIController` self)) ; Stop nav mesh movement
    )))

(event `/Game/TowerDefenseStarterKit/Blueprints/AI/BPI_ThreatResponse.RevertToDefaultState`
  ;[0 1 0.4 0.5] BPI_ThreatResponse interface functions
  (set `self.LockedInCombat?` false)
  (set `self.ActiveTarget` null)
  (`self.MoveToExitPoint`))

(event `/Game/TowerDefenseStarterKit/Blueprints/AI/BPI_ThreatResponse.PerformAttackOrderPreconditions`
  ;[0 1 0.4 0.5] BPI_ThreatResponse interface functions
  (`/Game/TowerDefenseStarterKit/Blueprints/AI/BPI_ThreatResponse.CancelMovement`))

(fn `ActivateCombatLock`
  (params (LockInstigator :type "Actor Object Reference"))
  (returns (`Success?` :type Boolean))
  ;[0 1 0.4 0.5] BPI_CombatLock interface function - Activates a combat lock with the target, If the target is not already locked into combat with another entity
  (if (`self.LockedInCombat?`)
    (return false) ; Combat lock activation failed
    (else
      (set `self.ActiveTarget` LockInstigator) ; The Combat Lock instigator becomes the highest priority target
      (set `self.LockedInCombat?` true)
      (`/Game/TowerDefenseStarterKit/Blueprints/AI/BPC_ThreatResponse.ActivateThreatResponse` (`self.ThreatResponse`)) ; Activates threat response to deal with the target
      (return true) ; Combat Lock activation successful
    )))

(fn `ActivateTerminationProtocols`
  (params (`ExitPointCrossed?` :type Boolean))
  ;[1 0 0 0.5] Handles termination protocols through an event dispatcher call
  (`self.EnemyUnitPendingDeletion` self `ExitPointCrossed?`) ; Event Dispatcher called to notify all listeners about an Enemy Unit Deletion event
)

(fn `GetMovementSpeed`
  (returns (ReturnValue :type "Float (double-precision)"))
  ;[0 1 1 0.5] Version 2.8.2: Returns the movement speed based on navigation model
  (return (select `/Game/TowerDefenseStarterKit/Blueprints/WaveSpawningSystems/ENavigationModels` (`self.NavModel`) :`NewEnumerator0` (`KismetMathLibrary.VSize` (`self.GetVelocity`)) :`NewEnumerator2` (`self.SplineMovementSpeed`))))

(fn `GetPlayerScoreReduction`
  (returns (PlayerScoreReduction :type Integer))
  ;[0 1 1 0.5] Returns the amount by which player score gets reduced when this unit reaches the exit point
  (return (`self.PlayerScoreModifier`)))

(fn `GetThreatRating`
  (returns (ThreatRating :type "Float (double-precision)"))
  (return (`self.ThreatRating`)))

(fn `MoveAlongTheSpline`
  (bind _activesplinepath (`self.ActiveSplinePath`))
  (bind _splinemovementspeed (`self.SplineMovementSpeed`))
  (bind _currentsplinedistance (`self.CurrentSplineDistance`))
  (bind (_returnvalue_x _returnvalue_y) (`KismetMathLibrary.BreakVector` (`SplineComponent.GetLocationAtDistanceAlongSpline` _activesplinepath _currentsplinedistance "World")))
  (bind (_returnvalue_roll _returnvalue_pitch _returnvalue_yaw) (`KismetMathLibrary.BreakRotator` (`SplineComponent.GetRotationAtDistanceAlongSpline` _activesplinepath _currentsplinedistance "World")))
  ;[0 1 1 0.5] Move along the spline
  (if (> (`self.MaxSpeed`) _splinemovementspeed)
    (set `self.SplineMovementSpeed` (+ _splinemovementspeed (`self.SplineMovementAcceleration`))))
  (set `self.CurrentSplineDistance` (+ (`self.CurrentSplineDistance`) (* (`self.SplinePathUpdateTime`) (`self.SplineMovementSpeed`))))
  (`self.K2_SetActorLocationAndRotation` (`KismetMathLibrary.MakeVector` _returnvalue_x _returnvalue_y (.z (`self.K2_GetActorLocation`))) (`KismetMathLibrary.MakeRotator` 0.0 0.0 _returnvalue_yaw)))

(fn `MoveToExitPoint`
  ;[0 1 1 0.5] Move towards the Exit Point
  (switch `/Game/TowerDefenseStarterKit/Blueprints/WaveSpawningSystems/ENavigationModels` (`self.NavModel`)
    (:`NewEnumerator0`
      (`AIBlueprintHelperLibrary.SimpleMoveToLocation` (`AIBlueprintHelperLibrary.GetAIController` self) (`self.PrimaryObjectiveLocation`)))
    (:`NewEnumerator2`
      (bind _returnvalue (`KismetSystemLibrary.K2_SetTimer` null "MoveAlongTheSpline" (`self.SplinePathUpdateTime`) true))
      (set `self.SplineMovementTimerHandle` _returnvalue)))
  (return))

(fn `RetrieveCombatLockStatus`
  (returns (`IsLockedInCombat?` :type Boolean))
  ;[0 1 0.4 0.5] BPI_CombatLock interface function - Returns if the actor is lockedin combat or not
  (return (`self.LockedInCombat?`)))

(fn `RetrieveTargetInfo`
  (returns (Name :type Text) (Description :type Text) (Stats :type "Array of /Game/TowerDefenseStarterKit/Blueprints/HUDControl/Struct_HUDStats Structure"))
  ;[0 1 0.4 0.5] BPI_TargetInfoDisplay interface function
  (return (`self.ObjectName`) (`self.ObjectDescription`) (`|MakeArray` (make `/Game/TowerDefenseStarterKit/Blueprints/HUDControl/Struct_HUDStats` "Max Speed" (`KismetTextLibrary.Conv_DoubleToText` (`self.MaxSpeed`) "HalfToEven")) (make `/Game/TowerDefenseStarterKit/Blueprints/HUDControl/Struct_HUDStats` "Health" (`KismetTextLibrary.Conv_DoubleToText` (`self.UnitHealth`) "HalfToEven")))))

(fn `RetrieveTargetingSystemData`
  (returns (ActiveTarget :type "Actor Object Reference") (AttackRange :type "Float (double-precision)"))
  ;[0 1 0.4 0.5] BPI_ThreatResponse interface function - Returns information necessary for threat response evaluation
  (return (`self.ActiveTarget`) (`self.AttackRange`)))

(fn `UpdateHealth`
  (params (Increment :type "Float (double-precision)"))
  ;[0 1 1 0.5] Updates the health based on the input parameter
  (set `self.UnitHealth` (`KismetMathLibrary.FClamp` (+ Increment (`self.UnitHealth`)) 0.0 (`self.MaxHealth`)))
  (bind _aswidget_3dstats_bar (cast `/Game/TowerDefenseStarterKit/UI/Generic/Widget_3DStatsBar` (`WidgetComponent.GetUserWidgetObject` (`self.3DStatsBar`)))
    (:`then`
      (`/Engine/EditorBlueprintResources/StandardMacros.IsValid` _aswidget_3dstats_bar
        (:`Is Valid`
          (`/Game/TowerDefenseStarterKit/UI/Generic/Widget_3DStatsBar.UpdateHealthBar` _aswidget_3dstats_bar (/ (`self.UnitHealth`) (`self.MaxHealth`))))
        (:`Is Not Valid`
          _))
      (return))
    (:`CastFailed`
      (return))))

(fn `UserConstructionScript`
  ;[0 1 1 0.5] Increases Unit Resilience to ramp up the difficulty with each new wave cycle.
  (bind _output_get (set `self.MaxHealth` (* (`self.MaxHealth`) (`KismetMathLibrary.Sqrt` (`KismetMathLibrary.Conv_IntToDouble` (`self.CycleMultiplier`))))))
  (set `self.UnitHealth` _output_get)
  (set `CharacterMovementComponent.MaxWalkSpeed` (`self.MaxSpeed`) (`self.CharacterMovement`)) ; Sets max walk speed for nav mesh based movement
)