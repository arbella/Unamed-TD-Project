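; Healer enemy AI unit for the tower defense game that periodically restores health to nearby enemy units.
; BeginPlay runs the parent logic, then starts a looping timer on HealChargeTime that calls ActivateAoEHeal.
; The heal scans the wave spawn controller's EnemyUnits, using AttackRange as its radius, and lets each valid target apply HealingIncrement through UpdateHealth.
; RetrieveTargetInfo supplies name, description and speed, health and heal stats to the target info HUD.
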(event `self.ReceiveBeginPlay`
  ;[0 1 1 0.5] Executes parent begin play logic & starts AoE Heal timer
  (`parent.ReceiveBeginPlay`)
  (bind _returnvalue (`KismetSystemLibrary.K2_SetTimer` null "ActivateAoEHeal" (`self.HealChargeTime`) true))
  (set `self.HealTimerHandle` _returnvalue))

(fn `ActivateAoEHeal`
  ;[0 1 1 0.5] Heal all enemy AI units within range
  (for _array_element (`/Game/TowerDefenseStarterKit/Blueprints/WaveSpawningSystems/BP_WaveSpawnController.EnemyUnits` (`/Game/TowerDefenseStarterKit/Blueprints/FunctionLibraries/BPFL_GetterFunctions.GetWaveSpawnController` self))
    (if (<= (`KismetMathLibrary.VSize` (- (`self.K2_GetActorLocation` _array_element) (`self.K2_GetActorLocation`))) (`self.AttackRange`))
      (`/Engine/EditorBlueprintResources/StandardMacros.IsValid` _array_element
        (:`Is Valid`
          (`self.UpdateHealth` _array_element (`self.HealingIncrement`)) ; Let the target actor take care of the health restoration
        )))))

(fn `RetrieveTargetInfo`
  (returns (Name :type Text) (Description :type Text) (Stats :type "Array of /Game/TowerDefenseStarterKit/Blueprints/HUDControl/Struct_HUDStats Structure"))
  ;[0 1 0.4 0.5] BPI_TargetInfoDisplay interface function
  (return (`self.ObjectName`) (`self.ObjectDescription`) (`|MakeArray` (make `/Game/TowerDefenseStarterKit/Blueprints/HUDControl/Struct_HUDStats` "Max Speed" (`KismetTextLibrary.Conv_DoubleToText` (`self.MaxSpeed`) "HalfToEven")) (make `/Game/TowerDefenseStarterKit/Blueprints/HUDControl/Struct_HUDStats` "Health" (`KismetTextLibrary.Conv_DoubleToText` (`self.UnitHealth`) "HalfToEven")) (make `/Game/TowerDefenseStarterKit/Blueprints/HUDControl/Struct_HUDStats` "AoE Heal" (`KismetTextLibrary.Conv_DoubleToText` (`self.HealingIncrement`) "HalfToEven")))))

(fn `UserConstructionScript`
  (`parent.UserConstructionScript`))