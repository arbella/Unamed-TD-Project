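; BP_EnemyAI_Rusher is an enemy AI variant that breaks off its path to rush the objective when badly hurt.
; After the parent health update, a living unit on a fixed spline path, rush-enabled and not locked in combat, triggers once below a fraction of max health.
; Rushing stops the spline movement timer, switches navigation to NavMesh and moves the unit toward the exit point by pathfinding.
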(event `self.UpdateHealth`
  (params (Increment :type "Float (single-precision)"))
  (bind _unithealth (`self.UnitHealth`))
  ;[0 1 1 0.5] Version 2.8.3: Rush Mode Activation [Only relevant if AI using custom spline based navigation model by default]
  (`parent.UpdateHealth` Increment)
  (if (`self.CanActivateRushMode?`)
    (switch `/Game/TowerDefenseStarterKit/Blueprints/WaveSpawningSystems/ENavigationModels` (`self.NavModel`)
      (:`NewEnumerator2`
        (if (`self.LockedInCombat?`)
          _
          (elif (and (> _unithealth 0.0) (< _unithealth (* (`self.MaxHealth`) (`self.RushActivationHealth%`))))
            (`/Engine/EditorBlueprintResources/StandardMacros.DoOnce` false
              (:`Completed`
                (`self.RushToObjective`) ; Activates Rush Mode
              ))))))))

(event `RushToObjective`
  ;[0 1 1 0.5] Version 2.8.3: Rush Mode Navigation Setup [Uses nav mesh to find shortest path to Objective location]
  (`KismetSystemLibrary.K2_ClearAndInvalidateTimerHandle` (`self.SplineMovementTimerHandle`)) ; Spline based movement aborted
  (set `self.NavModel` "NewEnumerator0") ; Nav Model shifted to nav mesh pathfinding
  (`self.MoveToExitPoint`))

(fn `UserConstructionScript`
  (`parent.UserConstructionScript`))