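; Tower-disabling enemy unit for the tower defense game that periodically knocks out nearby towers with an EMP blast.
; BeginPlay runs the parent logic, then starts a looping timer on the EMP charge time that calls ActivateEMPBlast.
; Each blast sphere-overlaps for towers within attack range and deactivates them for the EMP effect duration.
; RetrieveTargetInfo supplies name, description and stats to the HUD through the target info interface.
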(event `self.ReceiveBeginPlay`
  ;[0 1 1 0.5] Executes parent begin play logic & starts AoE Heal timer
  (`parent.ReceiveBeginPlay`)
  (bind _returnvalue (`KismetSystemLibrary.K2_SetTimer` null "ActivateEMPBlast" (`self.EMPChargeTime`) true))
  (set `self.EMPBlastTimerHandle` _returnvalue))

(fn `ActivateEMPBlast`
  ;[0 1 1 0.5] Damages all enemy units in range
  (bind _outactors (`KismetSystemLibrary.SphereOverlapActors` (`self.K2_GetActorLocation`) (`self.AttackRange`) (`|MakeArray` "ObjectTypeQuery10" :!type "EObjectTypeQuery Enum") "/Game/TowerDefenseStarterKit/Blueprints/Towers/BP_Tower_Parent.BP_Tower_Parent_C"))
  (for _array_element _outactors
    (`/Engine/EditorBlueprintResources/StandardMacros.IsValid` _array_element
      (:`Is Valid`
        (bind _asbp_tower_parent (cast `/Game/TowerDefenseStarterKit/Blueprints/Towers/BP_Tower_Parent` _array_element))
        (`/Game/TowerDefenseStarterKit/Blueprints/Towers/BP_Tower_Parent.DeactivateTower` _asbp_tower_parent (`self.EMPEffectDuration`)))))
  (return))

(fn `RetrieveTargetInfo`
  (returns (Name :type Text) (Description :type Text) (Stats :type "Array of /Game/TowerDefenseStarterKit/Blueprints/HUDControl/Struct_HUDStats Structure"))
  ;[0 1 0.4 0.5] BPI_TargetInfoDisplay interface function
  (return (`self.ObjectName`) (`self.ObjectDescription`) (`|MakeArray` (make `/Game/TowerDefenseStarterKit/Blueprints/HUDControl/Struct_HUDStats` "Max Speed" (`KismetTextLibrary.Conv_DoubleToText` (`self.MaxSpeed`) "HalfToEven")) (make `/Game/TowerDefenseStarterKit/Blueprints/HUDControl/Struct_HUDStats` "Health" (`KismetTextLibrary.Conv_DoubleToText` (`self.UnitHealth`) "HalfToEven")) (make `/Game/TowerDefenseStarterKit/Blueprints/HUDControl/Struct_HUDStats` "EMP Effect Duration" (`KismetTextLibrary.Conv_DoubleToText` (`self.EMPEffectDuration`) "HalfToEven")))))

(fn `UserConstructionScript`
  (`parent.UserConstructionScript`))