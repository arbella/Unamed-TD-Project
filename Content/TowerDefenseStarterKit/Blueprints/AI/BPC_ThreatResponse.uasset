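; BPC_ThreatResponse is an actor component that runs the attack loop for an owner implementing BPI_ThreatResponse, warning otherwise.
; On activation it polls the owner's active target until within attack range, then has the owner stop moving and attack.
; After each attack it either turns the owner's yaw toward the target and attacks again, or reverts the owner to its default state.
; All owner communication goes through interface messages.
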(event `self.ReceiveBeginPlay`
  ;[0 1 1 0.5] Checks if the owner meets compatibility requirements
  (if (not (`KismetSystemLibrary.DoesImplementInterface` (`self.GetOwner`) "/Game/TowerDefenseStarterKit/Blueprints/AI/BPI_ThreatResponse.BPI_ThreatResponse_C"))
    (`self.DisplayOwnerIncompatibilityWarning`)))

(event `ActivateThreatResponse`
  ;[0 1 1 0.5] Activates the Threat Response system
  (message `/Game/TowerDefenseStarterKit/Blueprints/AI/BPI_ThreatResponse.PerformAttackOrderPreconditions` (`self.GetOwner`)) ; Makes sure that all preconditions are met for issuing an attack order
  (bind (_activetarget _attackrange) (message `/Game/TowerDefenseStarterKit/Blueprints/AI/BPI_ThreatResponse.RetrieveTargetingSystemData` (`self.GetOwner`) :!label _label))
  (`/Engine/EditorBlueprintResources/StandardMacros.IsValid` _activetarget
    (:`Is Valid`
      (if (`self.EvaluateAssaultCapabilities` _activetarget _attackrange)
        (message `/Game/TowerDefenseStarterKit/Blueprints/AI/BPI_ThreatResponse.CancelMovement` (`self.GetOwner`)) ; Stops movement before attacking the target
        (message `/Game/TowerDefenseStarterKit/Blueprints/AI/BPI_ThreatResponse.AttackActiveTarget` (`self.GetOwner`)) ; Issue an attack order to the owner
        (else
          (`KismetSystemLibrary.Delay` 0.2) ; Do an attack range check again after a short delay
          (goto _label))))
    (:`Is Not Valid`
      (`self.DeactivateThreatResponse`) ; Deactivates the threat response system if no active target exists
    )))

(event `DeactivateThreatResponse`
  ;[0 1 1 0.5] Deactivates the Threat Response System
  (message `/Game/TowerDefenseStarterKit/Blueprints/AI/BPI_ThreatResponse.RevertToDefaultState` (`self.GetOwner`)) ; Requests the owner to return to it's default state
)

(fn `AttackOrderExecuted`
  (params (`ContinueAttack?` :type Boolean))
  ;[0 1 1 0.5] Determines the next course of action once an attack order has been successfully executed
  (if `ContinueAttack?`
    (bind _activetarget (message `/Game/TowerDefenseStarterKit/Blueprints/AI/BPI_ThreatResponse.RetrieveTargetingSystemData` (`self.GetOwner`)))
    (`/Engine/EditorBlueprintResources/StandardMacros.IsValid` _activetarget
      (:`Is Valid`
        (`self.FocusOnTarget` _activetarget) ; Focus on the active target before initiating the attack
        (message `/Game/TowerDefenseStarterKit/Blueprints/AI/BPI_ThreatResponse.AttackActiveTarget` (`self.GetOwner`)) ; Continue with next round of assault as long as active target exists
      )
      (:`Is Not Valid`
        (`self.DeactivateThreatResponse` :!label _label) ; Deactivates the threat response system if no active target exists
      ))
    (else
      (goto _label))))

(fn `DisplayOwnerIncompatibilityWarning`
  ;[0 0 0 0.5] Prints a warning message if the owning actor does not implement the requisite interface
  (`KismetSystemLibrary.PrintString` (`KismetStringLibrary.Concat_StrStr` "Warning: [Class: BPC_ThreatResponse] Owning actor '" (`KismetSystemLibrary.GetDisplayName` (`self.GetOwner`)) "' does not implement requisite interface")))

(fn `EvaluateAssaultCapabilities`
  (params (TargetActor :type "Actor Object Reference") (OwnerAttackRange :type "Float (double-precision)"))
  (returns (`InRange?` :type Boolean))
  ;[0 1 1 0.5] Checks if the target is within the owner's attack range
  (return (< (`Actor.GetDistanceTo` (`self.GetOwner`) TargetActor) OwnerAttackRange)))

(fn `FocusOnTarget`
  (params (TargetActor :type "Actor Object Reference"))
  ;[0 1 1 0.5] Makes the owning actor focus on the target actor
  (`/Engine/EditorBlueprintResources/StandardMacros.IsValid` TargetActor
    (:`Is Valid`
      (`Actor.K2_SetActorRotation` (`self.GetOwner`) (`KismetMathLibrary.MakeRotator` (.roll (`Actor.K2_GetActorRotation` (`self.GetOwner`))) (.pitch (`Actor.K2_GetActorRotation` (`self.GetOwner`))) (.yaw (`KismetMathLibrary.FindLookAtRotation` (`Actor.K2_GetActorLocation` (`self.GetOwner`)) (`Actor.K2_GetActorLocation` TargetActor)))) false))))