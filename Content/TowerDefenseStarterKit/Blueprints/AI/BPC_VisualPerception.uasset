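; Actor component that gives its owner timed visual perception of targets, such as for AI in a tower defense game.
; If the owner implements BPI_VisualPerception, a looping timer fetches range, angle and candidates from it each check, otherwise a warning prints.
; Candidates pass distance, cone angle and visibility trace tests in turn.
; The owner ranks each visible one, can end the search early, and receives the top-priority target.
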(event `self.ReceiveBeginPlay`
  ;[0 1 1 0.5] Initiate timed vision checks if the owning actor meets the compabitibility requirements
  (if (`KismetSystemLibrary.DoesImplementInterface` (`self.GetOwner`) "/Game/TowerDefenseStarterKit/Blueprints/AI/BPI_VisualPerception.BPI_VisualPerception_C")
    (`self.ActivateVisualPerception`)
    (else
      (`self.DisplayOwnerIncompatibilityWarning`))))

(event `self.ReceiveEndPlay`
  (params (EndPlayReason :type "EEndPlayReason Enum" :default "Destroyed"))
  ;[0 1 1 0.5] Clear timers before getting destroyed
  (`self.StopVisionCheck`))

(event `ActivateVisualPerception`
  ;[0 1 1 0.5] Activates the vision check timer to start analyzing potential targets based on their spatial relation to the owner
  (if (not (`KismetSystemLibrary.K2_TimerExistsHandle` (`self.VisionCheckTimerHandle`)))
    (bind _returnvalue (`KismetSystemLibrary.K2_SetTimer` null "VisionCheck" (`self.VisionCheckTimerInterval`) true))
    (set `self.VisionCheckTimerHandle` _returnvalue)))

(fn `AngularCheck`
  (params (TargetLocation :type "Vector Structure") (OwnerLocation :type "Vector Structure") (OwnerForwardVector :type "Vector Structure") (AngularRange :type "Float (double-precision)"))
  (returns (ReturnValue :type Boolean))
  ;[0 1 1 0.5] Checks if the target is within the specified angular range from the owner's forward facing direction
  (return (<= (`KismetMathLibrary.DegAcos` (`KismetMathLibrary.Dot_VectorVector` (`KismetMathLibrary.Normal` (- TargetLocation OwnerLocation)) OwnerForwardVector)) AngularRange)))

(fn `DisplayOwnerIncompatibilityWarning`
  ;[0 0 0 0.5] Prints a warning message if the owning actor does not implement the requisite interface
  (`KismetSystemLibrary.PrintString` (`KismetStringLibrary.Concat_StrStr` "Warning: [Class: BPC_VisualPerception] Owning actor '" (`KismetSystemLibrary.GetDisplayName` (`self.GetOwner`)) "' does not implement requisite interface")))

(fn `DistanceCheck`
  (params (OwnerLocation :type "Vector Structure") (TargetLocation :type "Vector Structure") (DistanceRange :type "Float (double-precision)"))
  (returns (ReturnValue :type Boolean))
  ;[0 1 1 0.5] Checks if the target is within the specified distance from the owner
  (return (<= (`KismetMathLibrary.VSize` (- OwnerLocation TargetLocation)) DistanceRange)))

(fn `LineTraceCheck`
  (params (OwnerLocation :type "Vector Structure") (TargetLocation :type "Vector Structure") (TargetActor :type "Actor Object Reference"))
  (returns (`TraceSuccess?` :type Boolean) (TraceVector :type "Vector Structure"))
  ;[0 1 1 0.5] Checks if a direct line trace can be established between the owner & the target
  (bind _outhit (`KismetSystemLibrary.LineTraceSingle` OwnerLocation TargetLocation "TraceTypeQuery1")) ; Line trace checks
  (bind (_bblockinghit _binitialoverlap _time _distance _location _impactpoint _normal _impactnormal _physmat _hitactor) (`GameplayStatics.BreakHitResult` _outhit))
  (return (== TargetActor _hitactor) (- _location (`Actor.K2_GetActorLocation` (`self.GetOwner`)))))

(fn `StopVisionCheck`
  (bind _visionchecktimerhandle (`self.VisionCheckTimerHandle`))
  ;[0 1 1 0.5] Stops Vision Check timer
  (if (`KismetSystemLibrary.K2_TimerExistsHandle` _visionchecktimerhandle)
    (`KismetSystemLibrary.K2_ClearAndInvalidateTimerHandle` _visionchecktimerhandle)))

(fn `VisionCheck`
  (locals (Local_VisionRange :type "Float (double-precision)") (Local_VisionAngle :type "Float (double-precision)") (Local_TargetActor :type "Actor Object Reference") (Local_MaxPriorityTarget :type "Actor Object Reference") (Local_DistanceToMaxPriorityTarget :type "Float (double-precision)"))
  (bind (_tracesuccess_ _tracevector) (`self.LineTraceCheck` (`Actor.K2_GetActorLocation` (`self.GetOwner`)) (`Actor.K2_GetActorLocation` (`local.Local_TargetActor`)) (`local.Local_TargetActor`)))
  ;[0 1 1 0.5] Loops through a list of potential targets & returns information about the highest priority target to the owning actor
  (bind (_visionrange _visionangle _potentialtargets) (message `/Game/TowerDefenseStarterKit/Blueprints/AI/BPI_VisualPerception.RetrieveVisualPerceptionRequisites` (`self.GetOwner`))) ; Requests the owner for parameters pertinent to visual perception calculations
  (set `local.Local_VisionRange` _visionrange)
  (set `local.Local_VisionAngle` _visionangle)
  (for _array_element _potentialtargets
    (bind _output_get (set `local.Local_TargetActor` _array_element))
    (`/Engine/EditorBlueprintResources/StandardMacros.IsValid` _output_get
      (:`Is Valid`
        (if (`self.DistanceCheck` (`Actor.K2_GetActorLocation` (`self.GetOwner`)) (`Actor.K2_GetActorLocation` (`local.Local_TargetActor`)) (`local.Local_VisionRange`))
          (if (`self.AngularCheck` (`Actor.K2_GetActorLocation` (`local.Local_TargetActor`)) (`Actor.K2_GetActorLocation` (`self.GetOwner`)) (`Actor.GetActorForwardVector` (`self.GetOwner`)) (`local.Local_VisionAngle`))
            (if _tracesuccess_
              (bind (_newmaxprioritytarget _distancetonewmaxprioritytarget _searchformoretargets_) (message `/Game/TowerDefenseStarterKit/Blueprints/AI/BPI_VisualPerception.EvaluateVisualPerceptionTargets` (`self.GetOwner`) (`local.Local_MaxPriorityTarget`) (`local.Local_TargetActor`) (`local.Local_DistanceToMaxPriorityTarget`) (`KismetMathLibrary.VSize` _tracevector))) ; Requests the owner to evaluate the relevance of the current loop cycle target with respect to the existing highest priority target
              (set `local.Local_MaxPriorityTarget` _newmaxprioritytarget)
              (set `local.Local_DistanceToMaxPriorityTarget` _distancetonewmaxprioritytarget)
              (if (not _searchformoretargets_)
                (break))))))))
  (message `/Game/TowerDefenseStarterKit/Blueprints/AI/BPI_VisualPerception.UpdateVisualPerceptionData` (`self.GetOwner`) (`local.Local_MaxPriorityTarget`)) ; Relays information to the owner about the highest priority target obtained from the list of potential targets that it provided
)