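; Blueprint function library of static getters that give any Blueprint quick access to the tower defense kit's core systems.
; HUD state and the active HUD widget come from BP_GameInstance, so they work in any level that uses that Game Instance.
; Tower, grid, object pool, wave spawn and projectile spawn managers, plus grid data, come through BP_GameMode, returning empty values if that cast fails.
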(fn `GetActiveHUDWidget`
  (params (WorldContextObject :type "Object Object Reference"))
  (returns (ActiveHUDWidget :type "UserWidget Object Reference"))
  ;[0 1 1 0.5] Getter function to access the Active HUD Widget; Can be used from any level as long as the required Game Instance is set
  (return (`/Game/TowerDefenseStarterKit/Blueprints/BP_GameInstance.RetrieveActiveHUDWidget` (cast `/Game/TowerDefenseStarterKit/Blueprints/BP_GameInstance` (`GameplayStatics.GetGameInstance` WorldContextObject) :!pure true))))

(fn `GetGridDataArray`
  (params (WorldContextObject :type "Object Object Reference"))
  (returns (GridDataArray :type "Array of /Game/TowerDefenseStarterKit/Blueprints/GridSystems/Struct_GridData Structure"))
  ;[0 1 1 0.5] Getter function to retrieve the Grid Data Array
  (bind _asbp_game_mode (cast `/Game/TowerDefenseStarterKit/Blueprints/BP_GameMode` (`GameplayStatics.GetGameMode` WorldContextObject))
    (:`then`
      (return (`/Game/TowerDefenseStarterKit/Blueprints/GridSystems/BP_GridManager.GetGridData` (`/Game/TowerDefenseStarterKit/Blueprints/BP_GameMode.RetrieveGridManager` _asbp_game_mode))))
    (:`CastFailed`
      (return (`|MakeArray` (struct) :!type "/Game/TowerDefenseStarterKit/Blueprints/GridSystems/Struct_GridData Structure")))))

(fn `GetGridManager`
  (params (WorldContextObject :type "Object Object Reference"))
  (returns (GridManager :type "/Game/TowerDefenseStarterKit/Blueprints/GridSystems/BP_GridManager Object Reference"))
  ;[0 1 1 0.5] Getter function to retrieve the Grid Manager
  (bind _asbp_game_mode (cast `/Game/TowerDefenseStarterKit/Blueprints/BP_GameMode` (`GameplayStatics.GetGameMode` WorldContextObject))
    (:`then`
      (return (`/Game/TowerDefenseStarterKit/Blueprints/BP_GameMode.RetrieveGridManager` _asbp_game_mode)))
    (:`CastFailed`
      (return null))))

(fn `GetHUDState`
  (params (WorldContextObject :type "Object Object Reference"))
  (returns (HUDState :type "/Game/TowerDefenseStarterKit/Blueprints/HUDControl/EHUDState Enum"))
  ;[0 1 1 0.5] Getter function to retrieve the high level HUD state; Can be used from any level as long as the required Game Instance is set
  (return (`/Game/TowerDefenseStarterKit/Blueprints/BP_GameInstance.RetrieveHUDState` (cast `/Game/TowerDefenseStarterKit/Blueprints/BP_GameInstance` (`GameplayStatics.GetGameInstance` WorldContextObject) :!pure true))))

(fn `GetObjectPoolManager`
  (params (WorldContextObject :type "Object Object Reference"))
  (returns (ObjectPoolMgr :type "/Game/TowerDefenseStarterKit/Blueprints/Projectiles/BP_ObjectPoolManager Object Reference"))
  ;[0 1 1 0.5] Getter function to retrieve the Object Pool Manager
  (bind _asbp_game_mode (cast `/Game/TowerDefenseStarterKit/Blueprints/BP_GameMode` (`GameplayStatics.GetGameMode` WorldContextObject))
    (:`then`
      (return (`/Game/TowerDefenseStarterKit/Blueprints/BP_GameMode.RetrieveObjectPoolManager` _asbp_game_mode)))
    (:`CastFailed`
      (return null))))

(fn `GetProjectileSpawnController`
  (params (WorldContextObject :type "Object Object Reference"))
  (returns (ProjectileSpawnController :type "/Game/TowerDefenseStarterKit/Blueprints/Projectiles/BP_ProjectileSpawnController Object Reference"))
  ;[0 1 1 0.5] Getter function to retrieve the Projectile Spawn Controller
  (bind _asbp_game_mode (cast `/Game/TowerDefenseStarterKit/Blueprints/BP_GameMode` (`GameplayStatics.GetGameMode` WorldContextObject))
    (:`then`
      (return (`/Game/TowerDefenseStarterKit/Blueprints/BP_GameMode.RetrieveProjectileSpawnController` _asbp_game_mode)))
    (:`CastFailed`
      (return null))))

(fn `GetTowerManager`
  (params (WorldContextObject :type "Object Object Reference"))
  (returns (TowerManager :type "/Game/TowerDefenseStarterKit/Blueprints/Towers/BP_TowerManager Object Reference"))
  ;[0 1 1 0.5] Getter function to retrieve the Tower Manager
  (bind _asbp_game_mode (cast `/Game/TowerDefenseStarterKit/Blueprints/BP_GameMode` (`GameplayStatics.GetGameMode` WorldContextObject))
    (:`then`
      (return (`/Game/TowerDefenseStarterKit/Blueprints/BP_GameMode.RetrieveTowerManager` _asbp_game_mode)))
    (:`CastFailed`
      (return null))))

(fn `GetWaveSpawnController`
  (params (WorldContextObject :type "Object Object Reference"))
  (returns (WaveManager :type "/Game/TowerDefenseStarterKit/Blueprints/WaveSpawningSystems/BP_WaveSpawnController Object Reference"))
  ;[0 1 1 0.5] Getter function to retrieve the Wave Spawn Controller
  (bind _asbp_game_mode (cast `/Game/TowerDefenseStarterKit/Blueprints/BP_GameMode` (`GameplayStatics.GetGameMode` WorldContextObject))
    (:`then`
      (return (`/Game/TowerDefenseStarterKit/Blueprints/BP_GameMode.RetrieveWaveSpawnController` _asbp_game_mode)))
    (:`CastFailed`
      (return null))))