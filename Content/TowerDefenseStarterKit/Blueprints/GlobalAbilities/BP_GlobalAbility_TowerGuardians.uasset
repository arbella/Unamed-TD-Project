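; Tower Guardians global ability: a short-lived actor that spawns a set number of guardian actors around itself.
; On BeginPlay it spawns each guardian with a configured lifespan, ignoring collisions, then destroys itself.
; CalculateSpawnTransform supplies each transform; its graph builds a random navigable XY within a radius, raised by a height offset, but that expression appears unconnected.
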(event `self.ReceiveBeginPlay`
  ;[0 1 0 0.5] Initialization Protocols
  (`self.SpawnTowerGuardians`))

(event `SpawnTowerGuardians`
  ;[0 1 1 0.5] Spawns Tower Guardians in the designated target area
  (for _ (range 1 (+ (`self.TotalNumberOfGuardians`) 1))
    (`|SpawnActorFromClass` (`self.TowerGuardianClass`) (`KismetMathLibrary.Conv_VectorToTransform` (`KismetMathLibrary.MakeVector` (.x (`NavigationSystemV1.K2_GetRandomLocationInNavigableRadius` (`self.K2_GetActorLocation`) (`self.MaxSpawnPlaneOffset`) null null)) (.y (`NavigationSystemV1.K2_GetRandomLocationInNavigableRadius` (`self.K2_GetActorLocation`) (`self.MaxSpawnPlaneOffset`) null null)) (+ (.z (`self.K2_GetActorLocation`)) (`self.SpawnHeightOffset`)))) "AlwaysSpawn" "OverrideRootScale" null (`self.TowerGuardianLifeSpan`) null))
  (`self.EndSpawningSystem`))

(event `EndSpawningSystem`
  ;[1 0 0 0.5] Destroys once the ability activation is completed
  (`self.K2_DestroyActor`))

(fn `UserConstructionScript`)