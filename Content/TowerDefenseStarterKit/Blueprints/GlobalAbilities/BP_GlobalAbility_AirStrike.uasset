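; Tower defense global ability actor that runs an airstrike at its location, then destroys itself.
; On BeginPlay it sets a spawn point high overhead and starts a looping timer that fires until the strike count is reached.
; Each tick requests a damaging blast projectile from the ProjectileSpawnController at a randomly offset spawn point.
; Downward velocity is derived from spawn height divided by impact time.
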(event `self.ReceiveBeginPlay`
  ;[0 1 0 0.5] Initialization Protocols
  (set `self.DefaultProjectileSpawnLocation` (`KismetMathLibrary.MakeVector` (.x (`self.K2_GetActorLocation`)) (.y (`self.K2_GetActorLocation`)) (+ (.z (`self.K2_GetActorLocation`)) (`self.ProjectileSpawnHeight`))))
  (`self.OnBeginAirstrike`))

(event `OnBeginAirstrike`
  ;[0 1 1 0.5] Begin Session
  (bind _returnvalue (`KismetSystemLibrary.K2_SetTimerDelegate` (delegate `OnFireProjectile`) (`self.StrikeInterval`) true))
  (set `self.FireProjectileTimer` _returnvalue))

(event `OnFireProjectile`
  ;[0 1 1 0.5] Airstrike Firing Solution
  (`/Game/TowerDefenseStarterKit/Blueprints/Projectiles/BP_ProjectileSpawnController.CreateAirstrikeProjectile` (`/Game/TowerDefenseStarterKit/Blueprints/FunctionLibraries/BPFL_GetterFunctions.GetProjectileSpawnController` self) (`KismetMathLibrary.Conv_VectorToTransform` (+ (`self.DefaultProjectileSpawnLocation`) (* (`KismetMathLibrary.Normal` (`KismetMathLibrary.MakeVector` (`KismetMathLibrary.RandomFloatInRange` -1.0 1.0) (`KismetMathLibrary.RandomFloatInRange` -1.0 1.0))) (`KismetMathLibrary.RandomFloatInRange` (`self.MinImpactOffset`) (`self.MaxImpactOffset`))))) (`self.BlastRadius`) (`self.BaseDamage`) 0.0 0.0 (`GameplayStatics.GetPlayerPawn` 0) (`KismetMathLibrary.MakeVector` 0.0 0.0 (* (/ (`self.ProjectileSpawnHeight`) (`self.ImpactTime`)) -1.0)))
  (bind _output_get (set `self.CurrentStrikeNumber` (+ (`self.CurrentStrikeNumber`) 1))) ; Update the number of projectiles launched in current strike
  (if (not (< _output_get (`self.TotalNumberOfStrikes`)))
    (`self.EndAirstrike`) ; End the current Airstrike session
  ))

(event `EndAirstrike`
  (bind _fireprojectiletimer (`self.FireProjectileTimer`))
  ;[1 0 0 0.5] End Session
  (if (`KismetSystemLibrary.K2_TimerExistsHandle` _fireprojectiletimer)
    (`KismetSystemLibrary.K2_ClearAndInvalidateTimerHandle` _fireprojectiletimer))
  (`self.K2_DestroyActor`))

(fn `UserConstructionScript`)