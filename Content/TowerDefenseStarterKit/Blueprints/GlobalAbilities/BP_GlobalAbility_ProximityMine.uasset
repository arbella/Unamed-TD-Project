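; Global ability Blueprint for a tower defense game that deploys a proximity mine at the targeted location.
; On BeginPlay it spawns a BP_ProximityMine, passing in its damage, blast radius, trigger radius and auto-detonation time, then destroys itself.
; The actor is a one-shot spawner, with mine placement delegated to CalculateSpawnTransform.
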(event `self.ReceiveBeginPlay`
  (`self.DeployProximityMine`))

(event `DeployProximityMine`
  (bind _returnvalue (`self.K2_GetActorLocation`))
  (`|SpawnActorFromClass` "/Game/TowerDefenseStarterKit/Blueprints/Misc/BP_ProximityMine.BP_ProximityMine_C" (`KismetMathLibrary.Conv_VectorToTransform` (`KismetMathLibrary.MakeVector` (.x _returnvalue) (.y _returnvalue) (+ (.z _returnvalue) (`self.SpawnHeightOffset`)))) "Undefined" "OverrideRootScale" null (`self.BaseDamage`) (`self.BlastRadius`) (`self.AutoDetonationTime`) (`self.TriggerRadius`) null) ; Spawns a proximity mine at the targeted ability deployment location
  (`self.K2_DestroyActor`))

(fn `UserConstructionScript`)