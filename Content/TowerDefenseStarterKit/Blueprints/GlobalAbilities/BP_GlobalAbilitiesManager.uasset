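; Manager actor for the tower defense kit's global abilities, which are deployed at a targeted location.
; Construction maps each ability type to its row handle in DT_GlobalAbilities for later lookups of spawn class, recharge time and description.
; Targeting events track the active selection, and deploying spawns that ability's class at the location.
; The player controller receives messages on initialization and on deployment, the latter carrying the recharge time for the HUD.
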(event `Initialize`
  (params (SelectedAbilities :type "Array of /Game/TowerDefenseStarterKit/Blueprints/GlobalAbilities/EGlobalAbilities Enum (by ref)" :default _))
  ;[0 1 0 0.5] Initialization Protocols
  (set `self.SelectedAbilities` SelectedAbilities)
  (message `/Game/TowerDefenseStarterKit/Blueprints/Player/BPI_GlobalAbilityInteraction.OnGlobalAbilityManagerInitialized` (`GameplayStatics.GetPlayerController` 0) (`self.SelectedAbilities`) (`self.GlobalAbilitesDTMap`)))

(event `OnTargetingActivated`
  (params (GlobalAbility :type "/Game/TowerDefenseStarterKit/Blueprints/GlobalAbilities/EGlobalAbilities Enum" :default "NewEnumerator2"))
  ;[0 1 1 0.5] Active Ability Setup
  (set `self.ActiveAbilitySelection` GlobalAbility) ; Current active ability
)

(event `OnTargetingDeactivated`
  ;[0 1 1 0.5] Active Ability Setup
  (set `self.ActiveAbilitySelection` "NewEnumerator2"))

(event `OnDeployGlobalAbility`
  (params (AtLocation :type "Vector Structure"))
  ;[0 1 1 0.5] Ability Deployment
  (bind _globalabilitydata (`self.GetRowDataForGlobalAbility` (`self.ActiveAbilitySelection`))
    (:`Row Found`
      (bind ((`SpawnClass_39_ACFD31EE4D636018DC8D6CBCE640A8C9` _spawnclass) (`RechargeDuration_14_6169E75C413B5FB0B9BB50985652A400` _rechargeduration)) (break `/Game/TowerDefenseStarterKit/Blueprints/GlobalAbilities/Struct_GlobalAbilityData` _globalabilitydata))
      (`|SpawnActorFromClass` _spawnclass (`KismetMathLibrary.Conv_VectorToTransform` AtLocation) "AlwaysSpawn" "OverrideRootScale" null null) ; Spawns a Global Ability at the targeted location
      (message `/Game/TowerDefenseStarterKit/Blueprints/Player/BPI_GlobalAbilityInteraction.OnGlobalAbilityDeployed` (`GameplayStatics.GetPlayerController` 0) (`self.ActiveAbilitySelection`) _rechargeduration) ; HUD Update Intimation
    )))

(fn `GetInfoAboutGlobalAbility`
  (params (GlobalAbility :type "/Game/TowerDefenseStarterKit/Blueprints/GlobalAbilities/EGlobalAbilities Enum" :default "NewEnumerator2"))
  (returns (FunctionName :type Text) (FunctionDescription :type Text) (Stats :type "Array of /Game/TowerDefenseStarterKit/Blueprints/HUDControl/Struct_HUDStats Structure"))
  ;[0 1 1 0.5] Returns information about the specified Global Ability
  (bind _globalabilitydata (`self.GetRowDataForGlobalAbility` GlobalAbility)
    (:`Row Found`
      (bind ((`AbilityName_20_80AAD993468C8D2D9DE5E98E664EB399` _abilityname) (`Description_25_34BCBCFE4B64F07031C244AA950D7DF2` _description)) (break `/Game/TowerDefenseStarterKit/Blueprints/GlobalAbilities/Struct_GlobalAbilityData` _globalabilitydata))
      (return _abilityname _description (`|MakeArray` (struct) (struct) :!type "/Game/TowerDefenseStarterKit/Blueprints/HUDControl/Struct_HUDStats Structure")))
    (:`RowNotFound`
      (return "" ""))))

(fn `MapGlobalAbilitiesToRowHandles`
  ;[0 1 1 0.5] Creates a mapping between Global Abilities & their associated rows in the data table
  (bind _outrownames (`DataTableFunctionLibrary.GetDataTableRowNames` "/Game/TowerDefenseStarterKit/Blueprints/GlobalAbilities/DT_GlobalAbilities.DT_GlobalAbilities"))
  (for _array_element _outrownames
    (bind _returnvalue (`|GetDataTableRow` "/Game/TowerDefenseStarterKit/Blueprints/GlobalAbilities/DT_GlobalAbilities.DT_GlobalAbilities" _array_element)
      (:`then`
        (`BlueprintMapLibrary.Map_Add` (`self.GlobalAbilitesDTMap`) (`.AbilityType_2_366506684B3954C2DCD1F087ABD4BFD8` (break `/Game/TowerDefenseStarterKit/Blueprints/GlobalAbilities/Struct_GlobalAbilityData` _returnvalue)) (make `DataTableRowHandle` "/Game/TowerDefenseStarterKit/Blueprints/GlobalAbilities/DT_GlobalAbilities.DT_GlobalAbilities" _array_element)))))
  (return))

(fn `UserConstructionScript`
  ;[0 1 0 0.5] Initialization Protocols
  (`self.MapGlobalAbilitiesToRowHandles`))