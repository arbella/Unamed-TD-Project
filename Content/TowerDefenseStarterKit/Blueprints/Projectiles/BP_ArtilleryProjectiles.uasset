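; BP_ArtilleryProjectiles is an explosive projectile in the tower defense kit that damages enemy units around its impact point.
; On BeginPlay it raises its custom time dilation by SpeedBoost to appear faster.
; On hit it sphere-overlaps enemy AI pawns within ExplosionRange, sending each direct damage with crit parameters rather than using engine radial damage.
; It then spawns a small explosion emitter and has the projectile spawn controller remove it as an airstrike projectile.
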(event `self.ReceiveBeginPlay`
  (set `self.CustomTimeDilation` (`self.SpeedBoost`)) ; Alter the time dilation for this actor to increase it's perceived speed
)

(event `self.CollisionComponent.OnComponentHit`
  (params (HitComponent :type "PrimitiveComponent Object Reference") (OtherActor :type "Actor Object Reference") (OtherComp :type "PrimitiveComponent Object Reference") (NormalImpulse :type "Vector Structure") (Hit :type "HitResult Structure (by ref)"))
  ;[1 0 0 0.5] Apply Radial Damage at impact location & spawn explosion emitter
  (`self.ApplyExplosionDamage`)
  (`GameplayStatics.SpawnEmitterAtLocation` "/Game/TowerDefenseStarterKit/Effects/Explosion/P_Explosion_Small.P_Explosion_Small" (`self.K2_GetActorLocation`))
  (`/Game/TowerDefenseStarterKit/Blueprints/Projectiles/BP_ProjectileSpawnController.RemoveAirstrikeProjectile` (`/Game/TowerDefenseStarterKit/Blueprints/FunctionLibraries/BPFL_GetterFunctions.GetProjectileSpawnController` self) self))

(fn `ApplyExplosionDamage`
  ;[0 1 1 0.5] Damages all enemy units in range
  (bind _outactors (`KismetSystemLibrary.SphereOverlapActors` (`self.K2_GetActorLocation`) (`self.ExplosionRange`) (`|MakeArray` "ObjectTypeQuery3" :!type "EObjectTypeQuery Enum") "/Game/TowerDefenseStarterKit/Blueprints/AI/Enemy/BP_EnemyAI_Parent.BP_EnemyAI_Parent_C"))
  (for _array_element _outactors
    (`/Engine/EditorBlueprintResources/StandardMacros.IsValid` _array_element
      (:`Is Valid`
        (message `/Game/TowerDefenseStarterKit/Blueprints/GenericSystems/BPI_DamageApplicationSystem.ApplyDirectDamage` _array_element (`self.Damage`) (`self.CritHitChance`) (`self.CritDamageMultiplier`) self null))))
  (return))

(fn `UserConstructionScript`
  (`parent.UserConstructionScript`))