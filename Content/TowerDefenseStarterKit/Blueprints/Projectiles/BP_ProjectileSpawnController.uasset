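; Central controller in the tower defense kit that creates and removes bullet, artillery and airstrike projectiles.
; Bullets go through the Object Pool Manager's activate and deactivate calls when a bullet pool exists, otherwise they are spawned and destroyed directly.
; Artillery and airstrike projectiles are always spawned with their damage and crit parameters, given an initial velocity, and destroyed on removal.
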(fn `CreateAirstrikeProjectile`
  (params (SpawnTransform :type "Transform Structure") (BlastRadius :type "Float (double-precision)") (Damage :type "Float (double-precision)") (CritHitChance :type "Float (double-precision)") (CritDamageMultiplier :type "Float (double-precision)") (Instigator :type "Pawn Object Reference") (InitialVelocity :type "Vector Structure"))
  (bind _returnvalue (`|SpawnActorFromClass` (`self.AirstrikeProjectileClassRef`) SpawnTransform "AlwaysSpawn" "OverrideRootScale" null BlastRadius Damage null CritHitChance CritDamageMultiplier Instigator)) ; Spawn an airstrike projectile & sets it's default parameters
  (set `MovementComponent.Velocity` InitialVelocity (`/Game/TowerDefenseStarterKit/Blueprints/Projectiles/BP_Projectiles.ProjectileMovement` _returnvalue)))

(fn `CreateArtilleryProjectile`
  (params (SpawnTransform :type "Transform Structure") (Damage :type "Float (double-precision)") (CritHitChance :type "Float (double-precision)") (CritDamageMultiplier :type "Float (double-precision)") (ProjectileCreator :type "Actor Object Reference") (InitialVelocity :type "Vector Structure"))
  (bind _returnvalue (`|SpawnActorFromClass` (`self.ArtilleryProjectileClassRef`) SpawnTransform "AlwaysSpawn" "OverrideRootScale" null Damage ProjectileCreator CritHitChance CritDamageMultiplier null)) ; Spawns an artillery projectile & sets it's default parameters
  (set `MovementComponent.Velocity` InitialVelocity (`/Game/TowerDefenseStarterKit/Blueprints/Projectiles/BP_Projectiles.ProjectileMovement` _returnvalue)))

(fn `CreateBulletProjectile`
  (params (BulletDamage :type "Float (double-precision)") (CritHitChance :type "Float (double-precision)") (CritDamageMultiplier :type "Float (double-precision)") (ProjectileCreator :type "Actor Object Reference") (SpawnTransform :type "Transform Structure"))
  ;[0 1 0 0.5] Spawns a new bullet projectile or activates one from the object pool based on the specifications
  (if (`/Game/TowerDefenseStarterKit/Blueprints/Projectiles/BP_ObjectPoolManager.DoesBulletProjectilePoolExist?` (`/Game/TowerDefenseStarterKit/Blueprints/FunctionLibraries/BPFL_GetterFunctions.GetObjectPoolManager` self))
    (`/Game/TowerDefenseStarterKit/Blueprints/Projectiles/BP_ObjectPoolManager.ActivateBulletProjectile` (`/Game/TowerDefenseStarterKit/Blueprints/FunctionLibraries/BPFL_GetterFunctions.GetObjectPoolManager` self) BulletDamage CritHitChance CritDamageMultiplier ProjectileCreator SpawnTransform) ; Requests the Pool Manager to activate a Bullet Projectile using the given parameters
    (else
      (`|SpawnActorFromClass` (`self.BulletProjectileClassRef`) SpawnTransform "AdjustIfPossibleButAlwaysSpawn" "OverrideRootScale" null BulletDamage ProjectileCreator CritHitChance CritDamageMultiplier null) ; Spawns a bullet projectile & fires it along the given direction
    )))

(fn `GetBulletProjectileClassRef`
  (returns (BulletProjectileClassRef :type "/Game/TowerDefenseStarterKit/Blueprints/Projectiles/BP_BulletProjectiles Class Reference"))
  (return (`self.BulletProjectileClassRef`)))

(fn `RemoveAirstrikeProjectile`
  (params (ProjectileActor :type "Actor Object Reference"))
  (`self.K2_DestroyActor` ProjectileActor))

(fn `RemoveArtilleryProjectile`
  (params (ProjectileActor :type "Actor Object Reference"))
  (`self.K2_DestroyActor` ProjectileActor))

(fn `RemoveBulletProjectile`
  (params (ObjectPoolIndex :type Integer) (ProjectileActor :type "Actor Object Reference"))
  ;[1 0 0 0.5] Destroys the projectile or deactivates it based on the specifications
  (if (`/Game/TowerDefenseStarterKit/Blueprints/Projectiles/BP_ObjectPoolManager.DoesBulletProjectilePoolExist?` (`/Game/TowerDefenseStarterKit/Blueprints/FunctionLibraries/BPFL_GetterFunctions.GetObjectPoolManager` self))
    (`/Game/TowerDefenseStarterKit/Blueprints/Projectiles/BP_ObjectPoolManager.DeactivateBulletProjectile` (`/Game/TowerDefenseStarterKit/Blueprints/FunctionLibraries/BPFL_GetterFunctions.GetObjectPoolManager` self) ObjectPoolIndex) ; Requests the Pool Manager to deactivate the bullet projectile at given index
    (else
      (`self.K2_DestroyActor` ProjectileActor))))

(fn `UserConstructionScript`)