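; Pooled bullet projectile for the tower defense game that applies crit-capable direct damage to opposing actors on hit.
; Enemy-created bullets damage towers and tower guardians, others damage enemy AI, and every hit returns the bullet to the projectile spawn controller.
; BPI_Poolable events toggle movement, collision and visibility, storing next-free indices for a linked free list.
; Activation ignores the Pawn channel for enemy instigators to prevent AI friendly fire.
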(event `self.CollisionComponent.OnComponentHit`
  (params (HitComponent :type "PrimitiveComponent Object Reference") (OtherActor :type "Actor Object Reference") (OtherComp :type "PrimitiveComponent Object Reference") (NormalImpulse :type "Vector Structure") (Hit :type "HitResult Structure (by ref)"))
  ;[1 0 0 0.5] Collision Response - Destroy Projectile & Apply Damage based on the instigator and the colliding actor
  (cast `/Game/TowerDefenseStarterKit/Blueprints/AI/Enemy/BP_EnemyAI_Parent` (`self.ProjectileCreator`)
    (:`then`
      (if (or (`KismetMathLibrary.ClassIsChildOf` (`GameplayStatics.GetObjectClass` OtherActor) "/Game/TowerDefenseStarterKit/Blueprints/Towers/BP_Tower_Parent.BP_Tower_Parent_C") (`KismetMathLibrary.ClassIsChildOf` (`GameplayStatics.GetObjectClass` OtherActor) "/Game/TowerDefenseStarterKit/Blueprints/AI/Friendly/BP_FriendlyAI_TowerGuardian.BP_FriendlyAI_TowerGuardian_C"))
        (message `/Game/TowerDefenseStarterKit/Blueprints/GenericSystems/BPI_DamageApplicationSystem.ApplyDirectDamage` OtherActor (`self.Damage`) (`self.CritHitChance`) (`self.CritDamageMultiplier`) self null :!label _label)))
    (:`CastFailed`
      (if (`KismetMathLibrary.ClassIsChildOf` (`GameplayStatics.GetObjectClass` OtherActor) "/Game/TowerDefenseStarterKit/Blueprints/AI/Enemy/BP_EnemyAI_Parent.BP_EnemyAI_Parent_C")
        (goto _label)
        (else
          _))))
  (`/Game/TowerDefenseStarterKit/Blueprints/Projectiles/BP_ProjectileSpawnController.RemoveBulletProjectile` (`/Game/TowerDefenseStarterKit/Blueprints/FunctionLibraries/BPFL_GetterFunctions.GetProjectileSpawnController` self) (`.ObjectPoolIndex_2_014935D445493FB84B6535B8DF074402` (break `/Game/TowerDefenseStarterKit/Blueprints/Projectiles/Struct_ObjectPoolData` (`self.ObjectPoolData`))) self))

(event `/Game/TowerDefenseStarterKit/Blueprints/Projectiles/BPI_Poolable.ActivatePoolableObject`
  (params (NewTransform :type "Transform Structure"))
  (bind _collisioncomponent (`self.CollisionComponent`))
  ;[0 1 0.4 0.5] BPI_Poolable Interface functions
  (setmembers `/Game/TowerDefenseStarterKit/Blueprints/Projectiles/Struct_ObjectPoolData` :`StructRef` (`self.ObjectPoolData`) :`NextFreeObjectIndex` -1 :`IsActive?` true) ; Sets object state to active & makes the link to next free object invalid
  (`self.K2_SetActorTransform` NewTransform false true)
  (cast `/Game/TowerDefenseStarterKit/Blueprints/AI/Enemy/BP_EnemyAI_Parent` (`self.Instigator`)
    (:`then`
      (`PrimitiveComponent.SetCollisionResponseToChannel` _collisioncomponent "ECC_Pawn" "ECR_Ignore") ; Cancels out friendly fire collisions among AI Bots
    )
    (:`CastFailed`
      (`PrimitiveComponent.SetCollisionResponseToChannel` _collisioncomponent "ECC_Pawn" "ECR_Block")))
  (`self.SetActorHiddenInGame` false)
  (`ProjectileMovementComponent.SetVelocityInLocalSpace` (`self.ProjectileMovement`) (`self.LocalProjectileVelocity`))
  (`ActorComponent.Activate` (`self.ProjectileMovement`) false)
  (`PrimitiveComponent.SetCollisionEnabled` (`self.CollisionComponent`) "QueryAndPhysics"))

(event `/Game/TowerDefenseStarterKit/Blueprints/Projectiles/BPI_Poolable.DeactivatePoolableObject`
  ;[0 1 0.4 0.5] BPI_Poolable Interface functions
  (`ActorComponent.Deactivate` (`self.ProjectileMovement`))
  (`PrimitiveComponent.SetCollisionEnabled` (`self.CollisionComponent`) "NoCollision")
  (`self.SetActorHiddenInGame` true))

(event `/Game/TowerDefenseStarterKit/Blueprints/Projectiles/BPI_Poolable.InitializeObjectPoolData`
  (params (ObjectPoolIndex :type Integer))
  ;[0 1 0.4 0.5] BPI_Poolable Interface functions
  (setmembers `/Game/TowerDefenseStarterKit/Blueprints/Projectiles/Struct_ObjectPoolData` :`StructRef` (`self.ObjectPoolData`) :`ObjectPoolIndex` ObjectPoolIndex) ; Stores the pool array index for this object
)

(event `/Game/TowerDefenseStarterKit/Blueprints/Projectiles/BPI_Poolable.StoreIndexForNextFreeObject`
  (params (ObjectPoolIndex :type Integer))
  ;[0 1 0.4 0.5] BPI_Poolable Interface functions
  (setmembers `/Game/TowerDefenseStarterKit/Blueprints/Projectiles/Struct_ObjectPoolData` :`StructRef` (`self.ObjectPoolData`) :`NextFreeObjectIndex` ObjectPoolIndex) ; Stores the index for next free object within the pool array
)

(fn `ResetBulletAttributes`
  (set `self.Damage` 0.0)
  (set `self.ProjectileCreator` null)
  (return))

(fn `RetrieveIndexForNextFreeObject`
  (returns (ObjectPoolIndex :type Integer))
  ;[0 1 0.4 0.5] BPI_Poolable Interface function - Retrieves the index of the next free object in the linked pool system
  (return (`.NextFreeObjectIndex_4_D461E28745DFD32188A0EF87C6E35422` (break `/Game/TowerDefenseStarterKit/Blueprints/Projectiles/Struct_ObjectPoolData` (`self.ObjectPoolData`)))))

(fn `SetNewBulletAttributes`
  (params (BulletDamage :type "Float (double-precision)") (CritHitChance :type "Float (double-precision)") (CritDamageMultiplier :type "Float (double-precision)") (ProjectileCreator :type "Actor Object Reference"))
  (set `self.Damage` BulletDamage)
  (set `self.CritHitChance` CritHitChance)
  (set `self.CritDamageMultiplier` CritDamageMultiplier)
  (set `self.ProjectileCreator` ProjectileCreator)
  (return))

(fn `UserConstructionScript`)