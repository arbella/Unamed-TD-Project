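; Object pool manager for the tower defense kit that pre-spawns and recycles bullet projectiles when pooling is enabled.
; Construction sizes the array, and initialization fills it with deactivated projectiles of the class supplied by the projectile spawn controller.
; Free slots form a linked list stored inside the projectiles, so activation and deactivation simply move the head index without searching.
; An exhausted pool prints a warning rather than growing.
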(event `InitializeObjectPoolMgr`
  ;[0 1 1 0.5] Handles Initialization Protocols
  (`self.PopulateBulletProjectilePool`))

(fn `ActivateBulletProjectile`
  (params (Damage :type "Float (double-precision)") (CritHitChance :type "Float (double-precision)") (CritDamageMultiplier :type "Float (double-precision)") (ProjectileCreator :type "Actor Object Reference") (NewTransform :type "Transform Structure"))
  (locals (Local_LinkedIndex :type Integer))
  (bind _output (`|GetArrayItem` (`self.ObjectPool_BulletProjectiles`) (`self.FirstFreeObjectIndex_BulletProjectiles`)))
  ;[0 1 0 0.5] Activates the next available Bullet Projectile actor from the pool array
  (if (>= (`self.FirstFreeObjectIndex_BulletProjectiles`) 0)
    (bind _objectpoolindex (message `/Game/TowerDefenseStarterKit/Blueprints/Projectiles/BPI_Poolable.RetrieveIndexForNextFreeObject` (`|GetArrayItem` (`self.ObjectPool_BulletProjectiles`) (`self.FirstFreeObjectIndex_BulletProjectiles`)))) ; Retrieves the index for next free object through the linked data stored in the object
    (set `local.Local_LinkedIndex` _objectpoolindex)
    (`/Game/TowerDefenseStarterKit/Blueprints/Projectiles/BP_BulletProjectiles.SetNewBulletAttributes` _output Damage CritHitChance CritDamageMultiplier ProjectileCreator)
    (message `/Game/TowerDefenseStarterKit/Blueprints/Projectiles/BPI_Poolable.ActivatePoolableObject` _output NewTransform)
    (set `self.FirstFreeObjectIndex_BulletProjectiles` (`local.Local_LinkedIndex`)) ; Updates the index to point to the next free object
    (else
      (`KismetSystemLibrary.PrintString` "Warning: No free Bullet Projectile in pool array"))))

(fn `DeactivateBulletProjectile`
  (params (PoolIndex :type Integer))
  (locals (Local_ExistingFirstFreeObjectIndex :type Integer :default 0))
  (bind _output (`|GetArrayItem` (`self.ObjectPool_BulletProjectiles`) PoolIndex))
  ;[1 0 0 0.5] Deactivates the object associated with the input index, within the pool array
  (`/Game/TowerDefenseStarterKit/Blueprints/Projectiles/BP_BulletProjectiles.ResetBulletAttributes` _output)
  (message `/Game/TowerDefenseStarterKit/Blueprints/Projectiles/BPI_Poolable.DeactivatePoolableObject` _output)
  (set `local.Local_ExistingFirstFreeObjectIndex` (`self.FirstFreeObjectIndex_BulletProjectiles`)) ; Stores the index of the next known free object
  (set `self.FirstFreeObjectIndex_BulletProjectiles` PoolIndex) ; Sets the deactivated object as the next available object
  (message `/Game/TowerDefenseStarterKit/Blueprints/Projectiles/BPI_Poolable.StoreIndexForNextFreeObject` _output (`local.Local_ExistingFirstFreeObjectIndex`)) ; Sets up a link to the previous first index through the new first index object
)

(fn `DoesBulletProjectilePoolExist?`
  (returns (`Yes?` :type Boolean))
  ;[0 0.4 1 0.5] Returns if an object pool is being used for Bullet Projectiles
  (return (`self.PoolBulletProjectiles?`)))

(fn `PopulateBulletProjectilePool`
  ;[0 1 0 0.5] Populates the Bullet Projectile object pool array & performs pool initialization protocols
  (if (`self.PoolBulletProjectiles?`)
    (for (_ _array_index) (`self.ObjectPool_BulletProjectiles`)
      (bind _returnvalue (`|SpawnActorFromClass` (`/Game/TowerDefenseStarterKit/Blueprints/Projectiles/BP_ProjectileSpawnController.GetBulletProjectileClassRef` (`/Game/TowerDefenseStarterKit/Blueprints/FunctionLibraries/BPFL_GetterFunctions.GetProjectileSpawnController` self)) (`self.GetTransform`) "AlwaysSpawn" "OverrideRootScale" null 0.0 null 0.0 0.0 null)) ; Spawns Bullet Projectiles
      (`KismetArrayLibrary.Array_Set` (`self.ObjectPool_BulletProjectiles`) _array_index _returnvalue) ; Adds an actor reference to the object pool array
      (message `/Game/TowerDefenseStarterKit/Blueprints/Projectiles/BPI_Poolable.DeactivatePoolableObject` _returnvalue) ; Sets the object to deactivated state by default
      (message `/Game/TowerDefenseStarterKit/Blueprints/Projectiles/BPI_Poolable.InitializeObjectPoolData` _returnvalue _array_index)
      (if (< _array_index (- (`self.PoolSize_BulletProjectile`) 1))
        (message `/Game/TowerDefenseStarterKit/Blueprints/Projectiles/BPI_Poolable.StoreIndexForNextFreeObject` _returnvalue (+ _array_index 1)) ; Stores the index for next free object within the current object to form a link
        (else
          (message `/Game/TowerDefenseStarterKit/Blueprints/Projectiles/BPI_Poolable.StoreIndexForNextFreeObject` _returnvalue -1) ; Stores an invalid index for the last object in the pool as there are no more free objects
        )))))

(fn `UserConstructionScript`
  ;[0 1 0 0.5] Resizes the pool arrays based on the requirements
  (if (`self.PoolBulletProjectiles?`)
    (`KismetArrayLibrary.Array_Resize` (`self.ObjectPool_BulletProjectiles`) (`self.PoolSize_BulletProjectile`)) ; Sets the size of the pool array to the specified value
  ))