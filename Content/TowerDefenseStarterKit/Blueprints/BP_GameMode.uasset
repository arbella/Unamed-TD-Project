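; Tower defense game mode that bootstraps a mission by gathering and initializing the core gameplay managers.
; After a tiny delay on BeginPlay it finds the grid, tower, wave, object pool and projectile actors and spawns the global abilities manager.
; It then either opens the HUD loadout menu or directly loads the in-game HUD and initializes managers and player controller.
; Retrieve functions expose most stored references.
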(event `self.ReceiveBeginPlay`
  ;[0 1 1 0.5] Start Mission
  (`KismetSystemLibrary.Delay` 0.005) ; Add a small delay to ensure that all core actors are spawned
  (`self.StoreCoreGameplayObjectReferences`) ; Get references to all core actors
  (if (`self.EnableTowerSelectionAtLevelStart?`)
    (bind _asbp_player_hud (cast `/Game/TowerDefenseStarterKit/Blueprints/Player/BP_PlayerHUD` (`PlayerController.GetHUD` (`GameplayStatics.GetPlayerController` 0))))
    (`/Game/TowerDefenseStarterKit/Blueprints/Player/BP_PlayerHUD.DisplayLoadoutMenu` _asbp_player_hud) ; Request the player HUD to display the Loadout menu
    (else
      (`self.InitializeCoreGameplayObjects` (`|MakeArray`) (`|MakeArray`)) ; Manually initialize the core actors
    )))

(fn `InitializeCoreGameplayObjects`
  (params (SelectedBaseTowerModels :type "Array of /Game/TowerDefenseStarterKit/Blueprints/Towers/ETowerModels Enum (by ref)" :default _) (SelectedAbilities :type "Array of /Game/TowerDefenseStarterKit/Blueprints/GlobalAbilities/EGlobalAbilities Enum (by ref)" :default _))
  ;[0 1 1 0.5] Load In-Game HUD & Initialize the core gameplay actors manually
  (`/Game/TowerDefenseStarterKit/Blueprints/BP_GameInstance.UpdateHUDState` (cast `/Game/TowerDefenseStarterKit/Blueprints/BP_GameInstance` (`GameplayStatics.GetGameInstance`) :!pure true) "NewEnumerator2") ; Load In-Game HUD
  (`/Game/TowerDefenseStarterKit/Blueprints/GridSystems/BP_GridManager.InitializeGridManager` (`self.GridManager`))
  (`/Game/TowerDefenseStarterKit/Blueprints/WaveSpawningSystems/BP_WaveSpawnController.InitializeWaveManager` (`self.WaveSpawnController`))
  (`/Game/TowerDefenseStarterKit/Blueprints/Towers/BP_TowerManager.InitializeTowerManager` (`self.TowerManager`) (`self.EnableTowerSelectionAtLevelStart?`) SelectedBaseTowerModels)
  (`/Game/TowerDefenseStarterKit/Blueprints/GlobalAbilities/BP_GlobalAbilitiesManager.Initialize` (`self.GlobalAbilityManager`) SelectedAbilities)
  (`/Game/TowerDefenseStarterKit/Blueprints/Projectiles/BP_ObjectPoolManager.InitializeObjectPoolMgr` (`self.ObjectPoolMgr`))
  (bind _asbp_player_controller (cast `/Game/TowerDefenseStarterKit/Blueprints/Player/BP_PlayerController` (`GameplayStatics.GetPlayerController` 0)))
  (`/Game/TowerDefenseStarterKit/Blueprints/Player/BP_PlayerController.InitializePlayerController` _asbp_player_controller (`self.GlobalAbilityManager`)))

(fn `RetrieveGridManager`
  (returns (GridManager :type "/Game/TowerDefenseStarterKit/Blueprints/GridSystems/BP_GridManager Object Reference"))
  (return (`self.GridManager`)))

(fn `RetrieveObjectPoolManager`
  (returns (ObjectPoolMgr :type "/Game/TowerDefenseStarterKit/Blueprints/Projectiles/BP_ObjectPoolManager Object Reference"))
  (return (`self.ObjectPoolMgr`)))

(fn `RetrieveProjectileSpawnController`
  (returns (ProjectileSpawnController :type "/Game/TowerDefenseStarterKit/Blueprints/Projectiles/BP_ProjectileSpawnController Object Reference"))
  (return (`self.ProjectileSpawnController`)))

(fn `RetrieveTowerManager`
  (returns (TowerManager :type "/Game/TowerDefenseStarterKit/Blueprints/Towers/BP_TowerManager Object Reference"))
  (return (`self.TowerManager`)))

(fn `RetrieveWaveSpawnController`
  (returns (WaveSpawnController :type "/Game/TowerDefenseStarterKit/Blueprints/WaveSpawningSystems/BP_WaveSpawnController Object Reference"))
  (return (`self.WaveSpawnController`)))

(fn `StoreCoreGameplayObjectReferences`
  ;[0 1 0 0.5] Store references to all core gameplay actors
  (bind _outactors (`GameplayStatics.GetAllActorsOfClass` (`self.GridManagerClass`)))
  (set `self.GridManager` (`|GetArrayItem` _outactors))
  (bind _outactors_2 (`GameplayStatics.GetAllActorsOfClass` (`self.TowerManagerClass`)))
  (set `self.TowerManager` (`|GetArrayItem` _outactors_2))
  (bind _outactors_3 (`GameplayStatics.GetAllActorsOfClass` (`self.WaveManagerClass`)))
  (set `self.WaveSpawnController` (`|GetArrayItem` _outactors_3))
  (bind _returnvalue (`|SpawnActorFromClass` "/Game/TowerDefenseStarterKit/Blueprints/GlobalAbilities/BP_GlobalAbilitiesManager.BP_GlobalAbilitiesManager_C" (`KismetMathLibrary.MakeTransform` (0.0 0.0 0.0)) "AlwaysSpawn" "OverrideRootScale" null null))
  (set `self.GlobalAbilityManager` _returnvalue)
  (bind _outactors_4 (`GameplayStatics.GetAllActorsOfClass` (`self.ObjectPoolMgrClass`)))
  (set `self.ObjectPoolMgr` (`|GetArrayItem` _outactors_4))
  (bind _outactors_5 (`GameplayStatics.GetAllActorsOfClass` (`self.ProjectileSpawnControllerClass`)))
  (set `self.ProjectileSpawnController` (`|GetArrayItem` _outactors_5))
  (return))

(fn `UserConstructionScript`)