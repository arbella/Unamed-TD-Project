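; Game state Blueprint for the tower defense kit that holds shared level data: mission success and the wave countdown time.
; Other Blueprints set or read mission status through simple update and retrieve functions.
; Countdown changes, absolute or by an offset, go through one setter that stores the value and notifies player controller 0 of the new time.
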(fn `ModifyWaveCountDownTime`
  (params (By :type "Float (double-precision)"))
  (returns (UpdatedTimer :type "Float (double-precision)"))
  ;[0 1 1 0.5] Version 2.8: Modifies the wave count down timer by the specified amount
  (`self.SetWaveCountDownTime` (+ (`self.WaveCountDownTime`) By))
  (return (`self.WaveCountDownTime`)))

(fn `RetrieveMissionStatus`
  (returns (`MissionSuccess?` :type Boolean))
  ;[0 1 1 0.5] Getter function used by other blueprints to retrieve the mission status
  (return (`self.MissionSuccess?`)))

(fn `SetWaveCountDownTime`
  (params (WaveCountDownTime :type "Float (double-precision)"))
  ;[0 1 1 0.5] Version 2.8: Updates the Wave Count Tower Timer value
  (bind _output_get (set `self.WaveCountDownTime` WaveCountDownTime))
  (message `/Game/TowerDefenseStarterKit/Blueprints/Player/BPI_GameInfoDisplay.OnWaveCountdownTimerUpdated` (`GameplayStatics.GetPlayerController` 0) _output_get)
  (return))

(fn `UpdateMissionStatus`
  (params (`Success?` :type Boolean))
  ;[0 1 1 0.5] Update the mission status of the current level
  (set `self.MissionSuccess?` `Success?`)
  (return))

(fn `UserConstructionScript`)