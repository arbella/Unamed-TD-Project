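; Tower defense wave controller that spawns randomly weighted enemy mixes within a per-wave threat budget and calculates player resources, both growing linearly.
; Initialization links spawn entries to DT_EnemyAIStats and sorts them by ascending threat.
; Each wave builds cumulative weight bands from eligible enemies, then spawns at random points with random delays.
; An over-budget roll caps later rolls at that band, ending spawning once the lowest-threat band cannot fit.
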(event `self.InitializeWaveManager`
  ;[0 1 0 0.5] Initialization protocols
  (`parent.InitializeWaveManager`)
  (`self.LinkAISpawnDataToDataTableEntries`)
  (`self.SortAISpawnDataInIncreasingThreatOrder`))

(event `self.RunWaveSpawningSystem`
  ;[0 1 1 0.5] Runs the Wave Spawning System
  (`self.SetThreatRatingForNewWave`)
  (bind _success_ (`self.PrepareAISpawnWeightDistArrayForNewWave`))
  (if _success_
    (bind (_id _lowerweightcutoff _upperweightcutoff) (`self.GetWeightedDistributionDataAtIndex` (`KismetArrayLibrary.Array_LastIndex` (`self.WeightedAISpawnProbDistribution`))))
    (set `self.WeightedAISpawnProbDistUpperThreshold` _upperweightcutoff)
    (bind (_newweightedaispawnprobdistupperthreshold _aispawnscompletedforcurrentwave_ _aispawned_) (`self.RunBotSpawningSystem` (`self.WeightedAISpawnProbDistUpperThreshold`) :!label _label))
    (set `self.WeightedAISpawnProbDistUpperThreshold` _newweightedaispawnprobdistupperthreshold)
    (set `self.AISpawnsCompletedForCurrentWave?` _aispawnscompletedforcurrentwave_)
    (if _aispawned_
      (`KismetSystemLibrary.Delay` (`self.CalculateDurationBeforeNextSpawn`)) ; IF a spawn operation is succesful, then wait for a small duration before the next spawn
      (goto _label)
      (elif (not (`self.AISpawnsCompletedForCurrentWave?`))
        (goto _label)))
    (else
      (`KismetSystemLibrary.PrintString` "WARNING: [Class: BP_WeightedWaveSpawnController] [Message: AISpawnWeightDistributionArray generated with zero elements"))))

(fn `CalculateDurationBeforeNextSpawn`
  (returns (Duration :type "Float (double-precision)"))
  (bind ((`SpawnInterval_MinValue_38_08E554D540488FB3CD9341A06348D9C1` _spawninterval_minvalue) (`SpawnInterval_MaxValue_39_FBA999444FF0D6C91738B8BD3A573638` _spawninterval_maxvalue)) (break `/Game/TowerDefenseStarterKit/Blueprints/WaveSpawningSystems/Struct_WeightedWaveSpawnData` (`self.WeightedWaveSpawnData`)))
  ;[0 1 1 0.5] Calculates a random float between the specified min & max spawn interval values
  (return (`KismetMathLibrary.RandomFloatInRange` _spawninterval_minvalue _spawninterval_maxvalue)))

(fn `GetResourceDistributionAmountForUpcomingWave`
  (returns (ResourceDistributionAmount :type Integer))
  (bind ((`ResourceAllocation_BaseValue_44_71FFA9D8449F830E4F67539A68698CAF` _resourceallocation_basevalue) (`ResourceAllocation_LinearGrowthMultiplier_45_FE42D14147FEC4AF8B74E78C8FF0160B` _resourceallocation_lineargrowthmultiplier)) (break `/Game/TowerDefenseStarterKit/Blueprints/WaveSpawningSystems/Struct_WeightedWaveSpawnData` (`self.WeightedWaveSpawnData`)))
  ;[0 1 1 0.5] Returns the amount of resources to be provided to the player for dealing with the upcoming wave
  (return (+ _resourceallocation_basevalue (`KismetMathLibrary.FTrunc` (* _resourceallocation_basevalue (* (- (`self.CurrentWave`) 1) (- _resourceallocation_lineargrowthmultiplier 1.0)))))))

(fn `GetWeightedDistributionDataAtIndex`
  (params (Index :type Integer))
  (returns (ID :type Name) (LowerWeightCutoff :type "Float (double-precision)") (UpperWeightCutoff :type "Float (double-precision)"))
  (bind (_id _lowerweightcutoff _upperweightcutoff) (break `/Game/TowerDefenseStarterKit/Blueprints/WaveSpawningSystems/Struct_WeightDistribution` (`|GetArrayItem` (`self.WeightedAISpawnProbDistribution`) Index)))
  (return _id _lowerweightcutoff _upperweightcutoff))

(fn `LinkAISpawnDataToDataTableEntries`
  ;[0 1 0 0.5] Loops through all elements of the AI Spawn Data Array, & sets the data table row names corresponding to each entry
  (for (_array_element _array_index) (`self.AISpawnWeightingDataArray`)
    (bind _outrownames (`DataTableFunctionLibrary.GetDataTableRowNames` "/Game/TowerDefenseStarterKit/Blueprints/AI/Enemy/DT_EnemyAIStats.DT_EnemyAIStats"))
    (for _array_element_2 _outrownames
      (bind _returnvalue (`|GetDataTableRow` "/Game/TowerDefenseStarterKit/Blueprints/AI/Enemy/DT_EnemyAIStats.DT_EnemyAIStats" _array_element_2)
        (:`then`
          (bind ((`AIType_21_587FB5FF45E38551F85FC3B0CA047615` _aitype) (`BaseWeighting_22_CCB0A5D64725EE3F58FC2CBA9D668E47` _baseweighting) (`CanBeSpawned?_13_95F746854ADB84436D7EF8A773C4CC7D` _canbespawned_) (`StartSpawningFromWave_25_19DE1FBF46C661E22834AEBB0A5D65F5` _startspawningfromwave)) (break `/Game/TowerDefenseStarterKit/Blueprints/WaveSpawningSystems/Struct_AISpawnWeightingData` _array_element))
          (if (`|EnumEquality` _aitype (`.AIType_5_600117EE4DC052F4F1ADB19022B8C5E6` (break `/Game/TowerDefenseStarterKit/Blueprints/AI/Enemy/Struct_EnemyAIData` _returnvalue)))
            (`KismetArrayLibrary.Array_Set` (`self.AISpawnWeightingDataArray`) _array_index (make `/Game/TowerDefenseStarterKit/Blueprints/WaveSpawningSystems/Struct_AISpawnWeightingData` _aitype _baseweighting _canbespawned_ _startspawningfromwave _array_element_2)) ; Stores the data table row name corresponding to the AI type
          )))))
  (return))

(fn `PrepareAISpawnWeightDistArrayForNewWave`
  (returns (`Success?` :type Boolean))
  (locals (Local_UpperWeightCutOffForPreviousIteration :type "Float (double-precision)" :default 0.0) (Local_MaxThreatRatingForIndividualAIUnit :type "Float (double-precision)" :default 0.0))
  (bind _local_upperweightcutoffforpreviousiteration (`local.Local_UpperWeightCutOffForPreviousIteration`))
  ;[0 1 1 0.5] Prepares the AI Spawn Weight Distribution Array for the new wave
  (set `local.Local_MaxThreatRatingForIndividualAIUnit` (/ (`self.MaxThreatRatingOfActiveWave`) (`.MaxUnitToWaveThreatRatio_48_D50C4FD34FED2B1CD67A6594943E4B61` (break `/Game/TowerDefenseStarterKit/Blueprints/WaveSpawningSystems/Struct_WeightedWaveSpawnData` (`self.WeightedWaveSpawnData`)))))
  (`KismetArrayLibrary.Array_Clear` (`self.WeightedAISpawnProbDistribution`)) ; Resets the prob dist array before creating a new distribution
  (for _array_element (`self.AISpawnWeightingDataArray`)
    (bind ((`BaseWeighting_22_CCB0A5D64725EE3F58FC2CBA9D668E47` _baseweighting) (`CanBeSpawned?_13_95F746854ADB84436D7EF8A773C4CC7D` _canbespawned_) (`StartSpawningFromWave_25_19DE1FBF46C661E22834AEBB0A5D65F5` _startspawningfromwave) (`DataTableRowName_19_D228155D4BC5E303DD57AEB83B411059` _datatablerowname)) (break `/Game/TowerDefenseStarterKit/Blueprints/WaveSpawningSystems/Struct_AISpawnWeightingData` _array_element))
    (if _canbespawned_
      (if (>= (`self.CurrentWave`) _startspawningfromwave)
        (bind _returnvalue (`|GetDataTableRow` "/Game/TowerDefenseStarterKit/Blueprints/AI/Enemy/DT_EnemyAIStats.DT_EnemyAIStats" _datatablerowname)
          (:`then`
            (if (not (> (`.ThreatRating_26_15D68C9C43222FAF4E328F94E8BB4337` (break `/Game/TowerDefenseStarterKit/Blueprints/AI/Enemy/Struct_EnemyAIData` _returnvalue)) (`local.Local_MaxThreatRatingForIndividualAIUnit`)))
              (bind _returnvalue_2 (+ _local_upperweightcutoffforpreviousiteration _baseweighting))
              (`KismetArrayLibrary.Array_Add` (`self.WeightedAISpawnProbDistribution`) (make `/Game/TowerDefenseStarterKit/Blueprints/WaveSpawningSystems/Struct_WeightDistribution` _datatablerowname _local_upperweightcutoffforpreviousiteration _returnvalue_2))
              (set `local.Local_UpperWeightCutOffForPreviousIteration` _returnvalue_2)))))))
  (return (> (`KismetArrayLibrary.Array_Length` (`self.WeightedAISpawnProbDistribution`)) 0)))

(fn `RetrieveNumberOfWavesPerCycle`
  (returns (NumberOfWaves :type Integer))
  (return (`.NumberOfWaves_11_A2E87D5C478FD539FEB21A8979E714F3` (break `/Game/TowerDefenseStarterKit/Blueprints/WaveSpawningSystems/Struct_WeightedWaveSpawnData` (`self.WeightedWaveSpawnData`)))))

(fn `RunBotSpawningSystem`
  (params (WeightedAISpawnProbDistUpperThreshold :type "Float (double-precision)"))
  (returns (NewWeightedAISpawnProbDistUpperThreshold :type "Float (double-precision)") (`AISpawnsCompletedForCurrentWave?` :type Boolean) (`AISpawned?` :type Boolean))
  (locals (Local_RandomProbWeightage :type "Float (double-precision)" :default 0.0) (`Local_AISpawned?` :type Boolean :default false) (`Local_AISpawnsCompleteForCurrentWave?` :type Boolean :default false) (Local_WeightedAISpawnProbDistUpperThreshold :type "Float (double-precision)") (Local_CurrentIterationIndex :type Integer))
  (bind _spawnpoints (`self.SpawnPoints`))
  ;[0 1 1 0.5] Calculates a random spawn weight value & checks it against Weighted Probability Distribution to spawn the AI class associated with the distribution range
  (bind _output_get (set `local.Local_WeightedAISpawnProbDistUpperThreshold` WeightedAISpawnProbDistUpperThreshold))
  (set `local.Local_RandomProbWeightage` (`KismetMathLibrary.RandomFloatInRange` 0.0 _output_get)) ; Calculates a random value within the weight distribution range
  (for _index (range (+ (`KismetArrayLibrary.Array_LastIndex` (`self.WeightedAISpawnProbDistribution`)) 1))
    (bind _output_get_2 (set `local.Local_CurrentIterationIndex` _index))
    (bind (_id _lowerweightcutoff _upperweightcutoff) (`self.GetWeightedDistributionDataAtIndex` _output_get_2))
    (if (`KismetMathLibrary.InRange_FloatFloat` (`local.Local_RandomProbWeightage`) _lowerweightcutoff _upperweightcutoff false)
      (bind _returnvalue (`|GetDataTableRow` "/Game/TowerDefenseStarterKit/Blueprints/AI/Enemy/DT_EnemyAIStats.DT_EnemyAIStats" _id)
        (:`then`
          (bind _returnvalue_2 (+ (`self.CurrentThreatRatingOfActiveWave`) (`.ThreatRating_26_15D68C9C43222FAF4E328F94E8BB4337` (break `/Game/TowerDefenseStarterKit/Blueprints/AI/Enemy/Struct_EnemyAIData` _returnvalue))))
          (if (> _returnvalue_2 (`self.MaxThreatRatingOfActiveWave`))
            (if (== (`local.Local_CurrentIterationIndex`) 0)
              (set `local.Local_AISpawnsCompleteForCurrentWave?` true)
              (else
                (bind (_id_2 _lowerweightcutoff_2 _upperweightcutoff_2) (`self.GetWeightedDistributionDataAtIndex` (`local.Local_CurrentIterationIndex`)))
                (set `local.Local_WeightedAISpawnProbDistUpperThreshold` _upperweightcutoff_2) ; Updates the upper weight threshold to restrict AI spawns only to classes within that range
              ))
            (set `local.Local_AISpawned?` false)
            (break)
            (else
              (set `self.CurrentThreatRatingOfActiveWave` _returnvalue_2) ; Updates the threat rating of the active wave based on the newly spawned unit
              (`/Game/TowerDefenseStarterKit/Blueprints/SpawnPoints/BP_SpawnPoint.SpawnEnemyAIBot` (`|GetArrayItem` _spawnpoints (`KismetMathLibrary.RandomInteger` (`KismetArrayLibrary.Array_Length` _spawnpoints))) 1 _id)
              (set `local.Local_AISpawned?` true)
              (break))))
        (:`RowNotFound`
          _)))
    (set `local.Local_AISpawned?` false))
  (return (`local.Local_WeightedAISpawnProbDistUpperThreshold`) (`local.Local_AISpawnsCompleteForCurrentWave?`) (`local.Local_AISpawned?`)))

(fn `SetThreatRatingForNewWave`
  (bind ((`WaveThreatRating_BaseValue_49_EFEE37EF4A25893711DFB18AF7AACBCA` _wavethreatrating_basevalue) (`WaveThreatRating_LinearGrowthMultiplier_50_0C7098934749D52EA66421A06CE12B4B` _wavethreatrating_lineargrowthmultiplier)) (break `/Game/TowerDefenseStarterKit/Blueprints/WaveSpawningSystems/Struct_WeightedWaveSpawnData` (`self.WeightedWaveSpawnData`)))
  ;[0 1 1 0.5] Sets the Threat Rating for new wave by applying the linear growth multiplier to the base value
  (set `self.MaxThreatRatingOfActiveWave` (+ _wavethreatrating_basevalue (* _wavethreatrating_basevalue (* (- (`self.CurrentWave`) 1) (- _wavethreatrating_lineargrowthmultiplier 1.0)))))
  (set `self.CurrentThreatRatingOfActiveWave` 0.0) ; Resets threat rating of the wave to zero
  (return))

(fn `SortAISpawnDataInIncreasingThreatOrder`
  (locals (Local_CurrentOuterLoopIndex :type Integer) (Local_HighestThreatRating :type "Float (double-precision)") (Local_IndexForHighestThreatRating :type Integer))
  ;[0 1 0 0.5] Sorts the AISpawnDataArray in increasing order of their threat ratings
  (for _index (range (+ (- (`KismetArrayLibrary.Array_Length` (`self.AISpawnWeightingDataArray`)) 2) 1))
    (set `local.Local_CurrentOuterLoopIndex` _index)
    (set `local.Local_HighestThreatRating` 0.0)
    (for _index_2 (range (+ (- (`KismetArrayLibrary.Array_LastIndex` (`self.AISpawnWeightingDataArray`)) (`local.Local_CurrentOuterLoopIndex`)) 1))
      (bind _returnvalue (`|GetDataTableRow` "/Game/TowerDefenseStarterKit/Blueprints/AI/Enemy/DT_EnemyAIStats.DT_EnemyAIStats" (`.DataTableRowName_19_D228155D4BC5E303DD57AEB83B411059` (break `/Game/TowerDefenseStarterKit/Blueprints/WaveSpawningSystems/Struct_AISpawnWeightingData` (`|GetArrayItem` (`self.AISpawnWeightingDataArray`) _index_2))))
        (:`then`
          (bind ((`MaxAccelerationSplineMotion_44_A39C3EA34E168B98B024928775F6BD15` _maxaccelerationsplinemotion) (`ThreatRating_26_15D68C9C43222FAF4E328F94E8BB4337` _threatrating)) (break `/Game/TowerDefenseStarterKit/Blueprints/AI/Enemy/Struct_EnemyAIData` _returnvalue))
          (if (> _threatrating (`local.Local_HighestThreatRating`))
            (set `local.Local_IndexForHighestThreatRating` _index_2)
            (set `local.Local_HighestThreatRating` _threatrating)))))
    (`KismetArrayLibrary.Array_Swap` (`self.AISpawnWeightingDataArray`) (`local.Local_IndexForHighestThreatRating`) (- (`KismetArrayLibrary.Array_LastIndex` (`self.AISpawnWeightingDataArray`)) (`local.Local_CurrentOuterLoopIndex`))) ; Moves elements with higher threat ratings toward the end of the array
  )
  (return))

(fn `UserConstructionScript`
  (`parent.UserConstructionScript`))