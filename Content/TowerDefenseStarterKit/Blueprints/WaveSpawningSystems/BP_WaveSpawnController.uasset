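; Base wave controller for the tower defense game, running waves and cycles, manual or timed starts, HUD updates and tower point payouts.
; Child classes supply the spawning logic, waves per cycle and per-wave resources.
; Spawn point and enemy events maintain the live enemy list and reward kills by threat rating and cycle.
; When spawning completes and the list empties, it advances the wave or shows mission success, with zero cycles meaning endless mode.
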(event `StartNextWave`
  ;[0 1 1 0.5] Initializes AI spawning system based on the Wave Generator type
  (if (not (`self.NewWaveInitiated?`))
    (set `self.NewWaveInitiated?` true)
    (if (`KismetSystemLibrary.K2_TimerExistsHandle` (`self.StartWaveTimerHandle`))
      (`KismetSystemLibrary.K2_ClearAndInvalidateTimerHandle` (`self.StartWaveTimerHandle`)) ; If player manually starts the next wave, cancel any existing Start Wave Timer
    )
    (switch `/Game/TowerDefenseStarterKit/Blueprints/WaveSpawningSystems/EWaveSpawnModel` (`self.WaveSpawnModel`)
      (:`NewEnumerator1`
        (for _array_element (`self.SpawnPoints`)
          (`/Game/TowerDefenseStarterKit/Blueprints/SpawnPoints/BP_SpawnPoint.HideWaveDataDisplay` _array_element)))
      (:`NewEnumerator2`
        _))
    (set `self.AISpawnsCompletedForCurrentWave?` false)
    ;;[1 1 1] Version 2.8: New dedicated interface for general game info HUD updates
    (message `/Game/TowerDefenseStarterKit/Blueprints/Player/BPI_GameInfoDisplay.HideWaveCountdownTimer` (`GameplayStatics.GetPlayerController` 0))
    (message `/Game/TowerDefenseStarterKit/Blueprints/Player/BPI_GameInfoDisplay.OnNewWaveStarted` (`GameplayStatics.GetPlayerController` 0) (`self.CurrentWave`))
    (`self.RunWaveSpawningSystem`)))

(event `RunWaveSpawningSystem`
  ;[1 1 1] Implemented through child classes
)

(fn `AllocateTowerResourcesForNewWave`
  ;[0 1 1 0.5] Allocates specified amount of tower resources for the wave
  ;;[1 1 1] Version 2.8: Tower Points now stored in Player State
  (bind _asbp_player_state (cast `/Game/TowerDefenseStarterKit/Blueprints/Player/BP_PlayerState` (`Controller.PlayerState` (`GameplayStatics.GetPlayerController` 0)))
    (:`then`
      (`/Game/TowerDefenseStarterKit/Blueprints/Player/BP_PlayerState.ModifyTowerPoints` _asbp_player_state (`self.GetResourceDistributionAmountForUpcomingWave`)))
    (:`CastFailed`
      _))
  (return))

(fn `AllocateTowerResourcesUponDestroyingEnemyUnit`
  (params (EnemyUnit :type "/Game/TowerDefenseStarterKit/Blueprints/AI/Enemy/BP_EnemyAI_Parent Object Reference"))
  ;[0 1 1 0.5] If resources are to be provided to the player upon deletion of an enemy unit, allocate tower points based on its threat rating
  ;;[1 1 1] Version 2.8: Tower Points now stored in Player State
  (if (`self.ProvideResourcesUponDestroyingEnemyUnit`)
    (bind _asbp_player_state (cast `/Game/TowerDefenseStarterKit/Blueprints/Player/BP_PlayerState` (`Controller.PlayerState` (`GameplayStatics.GetPlayerController` 0)))
      (:`then`
        (`/Game/TowerDefenseStarterKit/Blueprints/Player/BP_PlayerState.ModifyTowerPoints` _asbp_player_state (`KismetMathLibrary.FTrunc` (* (`/Game/TowerDefenseStarterKit/Blueprints/AI/Enemy/BP_EnemyAI_Parent.GetThreatRating` EnemyUnit) (`self.ResourcesAllocatedPerEnemyThreatRatingUnit`) (`KismetMathLibrary.Sqrt` (`KismetMathLibrary.Conv_IntToDouble` (`self.CurrentCycle`)))))))
      (:`CastFailed`
        _)))
  (return))

(fn `CalculateWaveIndexWithinCurrentCycle`
  (returns (WaveIndex :type Integer))
  ;[0 1 1 0.5] Calculate the index of the active wave within the current cycle [Index in this context being information stored about the corresponding wave in relevant arrays]
  (return (mod (- (`self.CurrentWave`) 1) (`self.RetrieveNumberOfWavesPerCycle`))))

(fn `DestroyEnemyUnit`
  (params (EnemyUnitRef :type "/Game/TowerDefenseStarterKit/Blueprints/AI/Enemy/BP_EnemyAI_Parent Object Reference"))
  ;[0 1 1 0.5] Destroys the enemy unit & updates the tracker variables
  (`KismetArrayLibrary.Array_RemoveItem` (`self.EnemyUnits`) EnemyUnitRef) ; Remove unit reference from the list
  (`self.K2_DestroyActor` EnemyUnitRef) ; Destroy the unit
  (return))

(fn `EvaluateWaveTerminationStatus`
  (params (EnemyUnitPendingDeletion :type "/Game/TowerDefenseStarterKit/Blueprints/AI/Enemy/BP_EnemyAI_Parent Object Reference") (`ReachedExitPoint?` :type Boolean))
  (locals (Local_EnemyUnitPendingDeletion :type "/Game/TowerDefenseStarterKit/Blueprints/AI/Enemy/BP_EnemyAI_Parent Object Reference"))
  ;[0 1 1 0.5] Wave Termination & End Game logic
  (set `local.Local_EnemyUnitPendingDeletion` EnemyUnitPendingDeletion)
  (if (not `ReachedExitPoint?`)
    (`self.AllocateTowerResourcesUponDestroyingEnemyUnit` (`local.Local_EnemyUnitPendingDeletion`)))
  (`self.DestroyEnemyUnit` (`local.Local_EnemyUnitPendingDeletion`))
  (if (`self.AISpawnsCompletedForCurrentWave?`)
    (if (== (`KismetArrayLibrary.Array_Length` (`self.EnemyUnits`)) 0)
      (if (== (+ (`self.CalculateWaveIndexWithinCurrentCycle`) 1) (`self.RetrieveNumberOfWavesPerCycle`))
        (if (== (`self.CurrentCycle`) (`self.NumberOfWaveCycles`))
          (bind _asbp_player_hud (cast `/Game/TowerDefenseStarterKit/Blueprints/Player/BP_PlayerHUD` (`PlayerController.GetHUD` (`GameplayStatics.GetPlayerController` 0))))
          (`/Game/TowerDefenseStarterKit/Blueprints/Player/BP_PlayerHUD.DisplayMissionSummary` _asbp_player_hud true) ; Mission Success: Request Player HUD to display Mission Summary screen
          (else
            (`self.IncrementWaveCycle`)
            (`self.IncrementWaveNumber` :!label _label)
            (`self.AllocateTowerResourcesForNewWave`)
            (for _array_element (`self.SpawnPoints`)
              (`/Game/TowerDefenseStarterKit/Blueprints/SpawnPoints/BP_SpawnPoint.DisplayWaveInformation` _array_element) ; Display enemy AI spawn counter data for the next wave
            )
            (if (`self.TimedWaveStarts?`)
              (`self.StartWaveCountDownTimer`)
              (set `self.NewWaveInitiated?` false)
              (else
                (set `self.NewWaveInitiated?` false)))))
        (else
          (goto _label))))))

(fn `ExecuteWaveTimer`
  ;[0 1 1 0.5] Updates the wave timer countdown in the Game HUD; Starts new wave once the timer runs out
  (bind _asbp_game_state (cast `/Game/TowerDefenseStarterKit/Blueprints/BP_GameState` (`GameplayStatics.GetGameState`)))
  (bind _updatedtimer (`/Game/TowerDefenseStarterKit/Blueprints/BP_GameState.ModifyWaveCountDownTime` _asbp_game_state -1.0))
  (if (not (> _updatedtimer 0.0))
    (`self.StartNextWave`)
    (set `self.WaveTimerCountDownValue` 0.0)))

(fn `GetEnemyUnitList`
  (returns (EnemyUnitList :type "Array of /Game/TowerDefenseStarterKit/Blueprints/AI/Enemy/BP_EnemyAI_Parent Object Reference"))
  (return (`self.EnemyUnits`)))

(fn `GetResourceDistributionAmountForUpcomingWave`
  (returns (ResourceDistributionAmount :type Integer))
  ;[1 1 1] Implemented through child classes
  (return 0))

(fn `IncrementWaveCycle`
  (set `self.CurrentCycle` (+ (`self.CurrentCycle`) 1))
  (return))

(fn `IncrementWaveNumber`
  (set `self.CurrentWave` (+ (`self.CurrentWave`) 1))
  (return))

(fn `InitializeWaveManager`
  ;[0 1 1 0.5] Initializes the Wave Manager actor manually instead of relying on the Begin Play event
  (bind _outactors (`GameplayStatics.GetAllActorsOfClass` "/Game/TowerDefenseStarterKit/Blueprints/SpawnPoints/BP_SpawnPoint.BP_SpawnPoint_C"))
  (bind _output_get (set `self.SpawnPoints` _outactors))
  (for _array_element _output_get
    (add `/Game/TowerDefenseStarterKit/Blueprints/SpawnPoints/BP_SpawnPoint.EnemyUnitSpawned` _array_element (`|CreateDelegate` :!event `UpdateEnemyUnitList`)) ; Starts listening to Enemy Unit Spawn Events
    (`/Game/TowerDefenseStarterKit/Blueprints/SpawnPoints/BP_SpawnPoint.InitializeSpawnPoint` _array_element))
  (`self.SetWaveMode`)
  (`self.AllocateTowerResourcesForNewWave`)
  ;;[1 1 1] Version 2.8: New dedicated interface for general game info HUD updates
  (message `/Game/TowerDefenseStarterKit/Blueprints/Player/BPI_GameInfoDisplay.DisplayTotalWaveCount` (`GameplayStatics.GetPlayerController` 0) (== (`self.NumberOfWaveCycles`) 0) (* (`self.NumberOfWaveCycles`) (`self.RetrieveNumberOfWavesPerCycle`)))
  (message `/Game/TowerDefenseStarterKit/Blueprints/Player/BPI_GameInfoDisplay.OnNewWaveStarted` (`GameplayStatics.GetPlayerController` 0) (`self.CurrentWave`))
  (if (`self.TimedWaveStarts?`)
    (`self.StartWaveCountDownTimer`))
  (return))

(fn `RetrieveNumberOfWavesPerCycle`
  (returns (NumberOfWaves :type Integer))
  ;[1 1 1] Implemented through child classes
  (return 0))

(fn `SetWaveMode`
  ;[0 1 1 0.5] Set wave mode based on the selection from the level selection menu
  (if (`/Game/TowerDefenseStarterKit/Blueprints/BP_GameInstance.UseEndlessMode?` (cast `/Game/TowerDefenseStarterKit/Blueprints/BP_GameInstance` (`GameplayStatics.GetGameInstance`) :!pure true))
    (set `self.NumberOfWaveCycles` 0) ; 0 cycles default to endless mode
    (return)
    (else
      (return))))

(fn `StartWaveCountDownTimer`
  ;[0 1 1 0.5] Start timer to update the wave timer count down
  (bind _asbp_game_state (cast `/Game/TowerDefenseStarterKit/Blueprints/BP_GameState` (`GameplayStatics.GetGameState`)))
  ;;[1 1 1] Version 2.8: Wave Countdown Time now stored in Game State
  (`/Game/TowerDefenseStarterKit/Blueprints/BP_GameState.SetWaveCountDownTime` _asbp_game_state (`self.WaveTimerInterval`)) ; Countdown timer starting value set
  ;;[1 1 1] Version 2.8: New dedicated interface for general game info HUD updates
  (message `/Game/TowerDefenseStarterKit/Blueprints/Player/BPI_GameInfoDisplay.DisplayWaveCountdownTimer` (`GameplayStatics.GetPlayerController` 0))
  (`self.ExecuteWaveTimer`)
  (bind _returnvalue (`KismetSystemLibrary.K2_SetTimer` null "ExecuteWaveTimer" 1.0 true))
  (set `self.StartWaveTimerHandle` _returnvalue)
  (return))

(fn `UpdateEnemyUnitList`
  (params (EnemyUnit :type "/Game/TowerDefenseStarterKit/Blueprints/AI/Enemy/BP_EnemyAI_Parent Object Reference"))
  (locals (Local_SpawnTransform :type "Transform Structure") (`Local_Spline Path` :type "SplineComponent Object Reference"))
  ;[0 1 1 0.5] Updates the list containing references to all enemy bots present in the level
  (`KismetArrayLibrary.Array_Add` (`self.EnemyUnits`) EnemyUnit)
  (add `/Game/TowerDefenseStarterKit/Blueprints/AI/Enemy/BP_EnemyAI_Parent.EnemyUnitPendingDeletion` EnemyUnit (`|CreateDelegate` :!event `EvaluateWaveTerminationStatus`)) ; Starts listening to Enemy Unit Deletion Events
  (return))

(fn `UserConstructionScript`)