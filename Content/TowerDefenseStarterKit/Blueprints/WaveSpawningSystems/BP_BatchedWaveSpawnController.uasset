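; Wave spawn controller for the tower defense game that spawns enemy AI in timed batches defined per wave within repeating cycles.
; On initialization it links each batch to the first DT_EnemyAIStats row matching its AI type.
; Each wave sends batches to spawn points by class with the cycle multiplier, counting active groups to flag spawn completion.
; It also reports waves per cycle, upcoming spawn counts per point and pre-wave resource amounts.
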(event `self.InitializeWaveManager`
  ;[0 1 0 0.5] Initialization protocols
  (`self.LinkWaveSpawnDataToDataTableEntries`)
  (`parent.InitializeWaveManager`))

(event `self.RunWaveSpawningSystem`
  (bind _currentcycle (`self.CurrentCycle`))
  ;[0 1 1 0.5] Spawns AI bots in batches based on the information specified in the BatchedWaveSpawnDataArray
  (set `self.NumberOfActiveSpawnGroups` 0) ; Resets the number of spawn groups to zero at the start of a wave
  (for _array_element (`.BatchedAISpawnDataArray_11_4D8ECDD849ED9633A9F4F8A4A88BA188` (break `/Game/TowerDefenseStarterKit/Blueprints/WaveSpawningSystems/Struct_BatchedWaveSpawnData` (`|GetArrayItem` (`self.BatchedWaveSpawnData`) (`self.CalculateWaveIndexWithinCurrentCycle`))))
    (bind (_aitype _spawnpoint _spawnstartingtime _numberofunits _spawninterval _enemyaidatatablerowname) (break `/Game/TowerDefenseStarterKit/Blueprints/WaveSpawningSystems/Struct_BatchedAISpawnData` _array_element))
    (`/Engine/EditorBlueprintResources/StandardMacros.IsValid` _spawnpoint
      (:`Is Valid`
        (set `self.NumberOfActiveSpawnGroups` (+ (`self.NumberOfActiveSpawnGroups`) 1))
        (switch `/Game/TowerDefenseStarterKit/Blueprints/AI/Enemy/EEnemyAIType` _aitype
          (:`NewEnumerator0`
            (`/Game/TowerDefenseStarterKit/Blueprints/SpawnPoints/BP_SpawnPoint.SpawnAIBatch_TankClass` _spawnpoint _spawnstartingtime _numberofunits _spawninterval _currentcycle _enemyaidatatablerowname))
          (:`NewEnumerator1`
            (`/Game/TowerDefenseStarterKit/Blueprints/SpawnPoints/BP_SpawnPoint.SpawnAIBatch_HealerClass` _spawnpoint _spawnstartingtime _numberofunits _spawninterval _currentcycle _enemyaidatatablerowname))
          (:`NewEnumerator2`
            (`/Game/TowerDefenseStarterKit/Blueprints/SpawnPoints/BP_SpawnPoint.SpawnAIBatch_RangedClass` _spawnpoint _spawnstartingtime _numberofunits _spawninterval _currentcycle _enemyaidatatablerowname))
          (:`NewEnumerator4`
            (`/Game/TowerDefenseStarterKit/Blueprints/SpawnPoints/BP_SpawnPoint.SpawnAIBatch_RunnerClass` _spawnpoint _spawnstartingtime _numberofunits _spawninterval _currentcycle _enemyaidatatablerowname))
          (:`NewEnumerator5`
            (`/Game/TowerDefenseStarterKit/Blueprints/SpawnPoints/BP_SpawnPoint.SpawnAIBatch_DisablerClass` _spawnpoint _spawnstartingtime _numberofunits _spawninterval _currentcycle _enemyaidatatablerowname))))
      (:`Is Not Valid`
        (`KismetSystemLibrary.PrintString` "Warning: Invalid Enemy Spawn Point; Terminating Wave Generation")))))

(event `DecrementNumberOfActiveSpawnGroups`
  ;[1 0.4 0.1 0.5] Decrements the number of batched spawning orders active at the moment
  (bind _output_get (set `self.NumberOfActiveSpawnGroups` (- (`self.NumberOfActiveSpawnGroups`) 1))) ; Decrement the number of active batch spawners
  (if (not (> _output_get 0))
    (set `self.AISpawnsCompletedForCurrentWave?` true)))

(fn `GetResourceDistributionAmountForUpcomingWave`
  (returns (ResourceDistributionAmount :type Integer))
  ;[0 1 1 0.5] Returns the amount of resources to be provided to the player for dealing with the upcoming wave
  (return (`.PreWaveResourceDistributionAmount_15_F4AB40C64C11EF4C856989A2EBCAA339` (break `/Game/TowerDefenseStarterKit/Blueprints/WaveSpawningSystems/Struct_BatchedWaveSpawnData` (`|GetArrayItem` (`self.BatchedWaveSpawnData`) (`self.CalculateWaveIndexWithinCurrentCycle`))))))

(fn `LinkWaveSpawnDataToDataTableEntries`
  (locals (Local_BatchedWaveSpawnData :type "/Game/TowerDefenseStarterKit/Blueprints/WaveSpawningSystems/Struct_BatchedWaveSpawnData Structure") (Local_BatchedAISpawnData :type "/Game/TowerDefenseStarterKit/Blueprints/WaveSpawningSystems/Struct_BatchedAISpawnData Structure"))
  (bind (_batchedaispawndataarray _prewaveresourcedistributionamount) (break `/Game/TowerDefenseStarterKit/Blueprints/WaveSpawningSystems/Struct_BatchedWaveSpawnData` (`local.Local_BatchedWaveSpawnData`)))
  ;[0 1 0 0.5] Loops through every element (information about each wave) of the Wave Spawn Data Array, & sets the data table row names corresponding to each AI spawn data entry
  (for (_array_element _array_index) (`self.BatchedWaveSpawnData`)
    (bind _output_get (set `local.Local_BatchedWaveSpawnData` _array_element))
    (for (_array_element_2 _array_index_2) (`.BatchedAISpawnDataArray_11_4D8ECDD849ED9633A9F4F8A4A88BA188` (break `/Game/TowerDefenseStarterKit/Blueprints/WaveSpawningSystems/Struct_BatchedWaveSpawnData` _output_get))
      (bind _output_get_2 (set `local.Local_BatchedAISpawnData` _array_element_2))
      (bind _outrownames (`DataTableFunctionLibrary.GetDataTableRowNames` "/Game/TowerDefenseStarterKit/Blueprints/AI/Enemy/DT_EnemyAIStats.DT_EnemyAIStats"))
      (for _array_element_3 _outrownames
        (bind _returnvalue (`|GetDataTableRow` "/Game/TowerDefenseStarterKit/Blueprints/AI/Enemy/DT_EnemyAIStats.DT_EnemyAIStats" _array_element_3)
          (:`then`
            (bind ((`AIType_33_FD4424C54EF07978BB6D639333A56175` _aitype) (`SpawnPoint_10_06E7A01249153DA814D07690434C1BA6` _spawnpoint) (`SpawnStartingTime_16_5FF716FF446A3009296C0C8A9566C7C6` _spawnstartingtime) (`NumberOfUnits_19_164F63CC4C1BF6CE86D26580DF0D477F` _numberofunits) (`SpawnInterval_30_211B1FF64D7B7DCCCB742BB2AFFBB2A6` _spawninterval)) (break `/Game/TowerDefenseStarterKit/Blueprints/WaveSpawningSystems/Struct_BatchedAISpawnData` _output_get_2))
            (if (`|EnumEquality` _aitype (`.AIType_5_600117EE4DC052F4F1ADB19022B8C5E6` (break `/Game/TowerDefenseStarterKit/Blueprints/AI/Enemy/Struct_EnemyAIData` _returnvalue)))
              (`KismetArrayLibrary.Array_Set` (`.BatchedAISpawnDataArray_11_4D8ECDD849ED9633A9F4F8A4A88BA188` (break `/Game/TowerDefenseStarterKit/Blueprints/WaveSpawningSystems/Struct_BatchedWaveSpawnData` (`local.Local_BatchedWaveSpawnData`))) _array_index_2 (make `/Game/TowerDefenseStarterKit/Blueprints/WaveSpawningSystems/Struct_BatchedAISpawnData` _aitype _spawnpoint _spawnstartingtime _numberofunits _spawninterval _array_element_3)) ; Updates the AI Spawn Data Array with the associated data table row name information
              (break))))))
    (`KismetArrayLibrary.Array_Set` (`self.BatchedWaveSpawnData`) _array_index (make `/Game/TowerDefenseStarterKit/Blueprints/WaveSpawningSystems/Struct_BatchedWaveSpawnData` _batchedaispawndataarray _prewaveresourcedistributionamount)) ; Replaces the defaut AI Spawn Data Array with the new one containing data table row names
  )
  (return))

(fn `RetrieveNumberOfWavesPerCycle`
  (returns (NumberOfWaves :type Integer))
  (return (`KismetArrayLibrary.Array_Length` (`self.BatchedWaveSpawnData`))))

(fn `RetrieveSpawnCountDataForUpcomingWave`
  (params (EnemySpawnPoint :type "/Game/TowerDefenseStarterKit/Blueprints/SpawnPoints/BP_SpawnPoint Object Reference"))
  (returns (EnemySpawnCountData :type "Array of /Game/TowerDefenseStarterKit/Blueprints/WaveSpawningSystems/Struct_EnemyAISpawnCounter Structure"))
  (locals (Local_EnemySpawnPoint :type "/Game/TowerDefenseStarterKit/Blueprints/SpawnPoints/BP_SpawnPoint Object Reference") (Local_EnemySpawnCountData :type "Array of /Game/TowerDefenseStarterKit/Blueprints/WaveSpawningSystems/Struct_EnemyAISpawnCounter Structure"))
  ;[0 1 1 0.5] Return enemy spawn count data for the given spawn point during the upcoming wave
  (set `local.Local_EnemySpawnPoint` EnemySpawnPoint)
  (for _array_element (`.BatchedAISpawnDataArray_11_4D8ECDD849ED9633A9F4F8A4A88BA188` (break `/Game/TowerDefenseStarterKit/Blueprints/WaveSpawningSystems/Struct_BatchedWaveSpawnData` (`|GetArrayItem` (`self.BatchedWaveSpawnData`) (`self.CalculateWaveIndexWithinCurrentCycle`))))
    (bind ((`SpawnPoint_10_06E7A01249153DA814D07690434C1BA6` _spawnpoint) (`NumberOfUnits_19_164F63CC4C1BF6CE86D26580DF0D477F` _numberofunits) (`EnemyAIDataTableRowName_36_DCE67F6944AA4FB49F8FB7B4649C4B35` _enemyaidatatablerowname)) (break `/Game/TowerDefenseStarterKit/Blueprints/WaveSpawningSystems/Struct_BatchedAISpawnData` _array_element))
    (if (== (`local.Local_EnemySpawnPoint`) _spawnpoint)
      (`KismetArrayLibrary.Array_Set` (`local.Local_EnemySpawnCountData`) (`KismetArrayLibrary.Array_Length` (`local.Local_EnemySpawnCountData`)) (make `/Game/TowerDefenseStarterKit/Blueprints/WaveSpawningSystems/Struct_EnemyAISpawnCounter` _enemyaidatatablerowname _numberofunits) true)))
  (return (`local.Local_EnemySpawnCountData`)))

(fn `UserConstructionScript`
  (`parent.UserConstructionScript`))