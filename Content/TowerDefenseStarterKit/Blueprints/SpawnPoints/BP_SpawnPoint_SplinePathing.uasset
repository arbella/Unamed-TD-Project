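; Tower defense spawn point whose AI paths are defined by splines, with optional parallel lanes.
; Construction raises the primary spline and generates extra lanes alternately on either side, sampling it at mesh-spacing intervals and offsetting along its right vector.
; On initialization it stores each lane's start as a bot spawn transform and displays wave information.
; The primary spline's last point serves as the AI objective location.
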(event `self.InitializeSpawnPoint`
  ;[0 1 0 0.5] Initialization Protocols
  (`self.SetSpawnTransforms`)
  (`self.DisplayWaveInformation`)
  (`parent.InitializeSpawnPoint`))

(event `self.SetSpawnTransforms`
  ;[0 1 1 0.5] Stores the starting locations of different path lanes in the BotSpawnTansformArray
  (`KismetArrayLibrary.Array_Resize` (`self.BotSpawnTransforms`) (`KismetArrayLibrary.Array_Length` (`self.SplineComponents`)))
  (for (_array_element _array_index) (`self.SplineComponents`)
    (`KismetArrayLibrary.Array_Set` (`self.BotSpawnTransforms`) _array_index (`KismetMathLibrary.MakeTransform` (+ (`SplineComponent.GetLocationAtSplinePoint` _array_element 0 "World") (`KismetMathLibrary.MakeVector` 0.0 0.0 (- (`self.SpawnHeightOffset`) (`self.SplineHeight`)))) (`SplineComponent.GetRotationAtSplinePoint` _array_element 0 "World")) true)))

(fn `AddMultipleLanesForCustomSplinePath`
  (locals (Local_DirectionalMultiplier :type Integer) (Local_CurrentSpline :type "SplineComponent Object Reference") (Local_CurrentDistanceAlongSpline :type "Float (double-precision)"))
  (bind _local_currentdistancealongspline (`local.Local_CurrentDistanceAlongSpline`))
  (bind _primarypath (`self.PrimaryPath`))
  (bind (_remainder _returnvalue) (`KismetMathLibrary.FMod` (`SplineComponent.GetSplineLength` (`self.PrimaryPath`)) (`self.AIPathMeshSpacing`)))
  ;[0 1 1 0.5] Adds multiple lanes on either sides of the primary spline [Works only with curved splines]
  (for _index (range 2 (+ (`self.NumberOfLanes`) 1))
    (switch `int` (mod _index 2) ; Assigns new spline to right & left sides of the primary spline based on the index
      (:`0`
        (bind _returnvalue_2 (/ _index 2))
        (set `local.Local_DirectionalMultiplier` (* _returnvalue_2 1)))
      (:`1`
        (set `local.Local_DirectionalMultiplier` (* _returnvalue_2 -1))))
    (bind _returnvalue_3 (`AddComponent|NODE_AddSplineComponent-0`))
    (bind _output_get (set `local.Local_CurrentSpline` _returnvalue_3))
    (`SplineComponent.ClearSplinePoints` _output_get true) ; Clears the default spline point
    (`SceneComponent.K2_AddLocalOffset` _output_get (`KismetMathLibrary.MakeVector` 0.0 0.0 (`self.SplineHeight`)) false true)
    (`KismetArrayLibrary.Array_Add` (`self.SplineComponents`) (`local.Local_CurrentSpline`))
    (for _index_2 (range (+ _returnvalue 1))
      (set `local.Local_CurrentDistanceAlongSpline` (* _index_2 (`self.AIPathMeshSpacing`)))
      (`SplineComponent.AddSplinePoint` (`local.Local_CurrentSpline`) (+ (`SplineComponent.GetLocationAtDistanceAlongSpline` _primarypath _local_currentdistancealongspline "Local") (* (`SplineComponent.GetRightVectorAtDistanceAlongSpline` _primarypath _local_currentdistancealongspline "Local") (* (`local.Local_DirectionalMultiplier`) (`self.LaneGapDistance`)))) "Local" true :!label _label))
    (if (> _remainder 0.0)
      (set `local.Local_CurrentDistanceAlongSpline` (`SplineComponent.GetSplineLength` (`self.PrimaryPath`)))
      (goto _label)))
  (return))

(fn `GetAIObjectiveLocation`
  (returns (ReturnValue :type "Vector Structure"))
  ;[0 1 1 0.5] Version 2.8.3: Returns the final Objective Location for AI units starting from this spawn point
  (return (`SplineComponent.GetLocationAtSplinePoint` (`self.PrimaryPath`) (- (`SplineComponent.GetNumberOfSplinePoints` (`self.PrimaryPath`)) 1) "World")) ; Location at the final spline point on path spline
)

(fn `UserConstructionScript`
  (`parent.UserConstructionScript`)
  ;[0 1 0 0.5] Parallel MultiLane Path Generation
  (`SceneComponent.K2_AddLocalOffset` (`self.PrimaryPath`) (`KismetMathLibrary.MakeVector` 0.0 0.0 (`self.SplineHeight`)) false true) ; Lifts up the spline a few units above the ground level
  (`KismetArrayLibrary.Array_Add` (`self.SplineComponents`) (`self.PrimaryPath`))
  (if (> (`self.NumberOfLanes`) 1)
    (`self.AddMultipleLanesForCustomSplinePath`)))