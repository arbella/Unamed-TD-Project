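; Tower defense spawn point that builds spline paths along the nav mesh to its objectives, either every exit point or one designated objective.
; On initialization it finds a synchronous nav path to each objective and turns it into a raised spline with evenly spaced points, warning if none exists.
; It also sets a height-offset bot spawn transform and returns a random or designated objective location for AI units.
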(event `self.InitializeSpawnPoint`
  ;[0 1 0 0.5] Initialization Protocols
  (if (`self.UseRandomObjective?`)
    (bind _outactors (`GameplayStatics.GetAllActorsOfClass` "/Game/TowerDefenseStarterKit/Blueprints/Misc/BP_ExitPoint.BP_ExitPoint_C"))
    (set `self.ObjectivesList` _outactors)
    (else
      (`KismetArrayLibrary.Array_Add` (`self.ObjectivesList`) (`self.DesignatedObjective`))))
  (`self.CreateSplinePointsForNavMeshPath`)
  (`self.SetSpawnTransforms`)
  (`parent.InitializeSpawnPoint`))

(event `self.SetSpawnTransforms`
  ;[0 1 1 0.5] Set default bot spawn transform
  (`KismetArrayLibrary.Array_Add` (`self.BotSpawnTransforms`) (`KismetMathLibrary.MakeTransform` (+ (`self.K2_GetActorLocation`) (`KismetMathLibrary.MakeVector` 0.0 0.0 (`self.SpawnHeightOffset`))))))

(fn `CreateSplinePointsForNavMeshPath`
  (locals (Local_NavMeshPathPoints :type "Array of Vector Structure") (Local_Spline :type "SplineComponent Object Reference") (Local_CurrentPathPointIndex :type Integer) (Local_CurrentPathLength :type "Float (double-precision)") (Local_CurrentPathUnitVector :type "Vector Structure") (Local_CurrentPathStartingPoint :type "Vector Structure"))
  (bind (_remainder _returnvalue) (`KismetMathLibrary.FMod` (`local.Local_CurrentPathLength`) (`self.AIPathMeshSpacing`)))
  ;[0 1 1 0.5] Creates spline points based on the nav mesh path points from the Spawn Point to the Exit Point
  (for _array_element (`self.ObjectivesList`)
    (`/Engine/EditorBlueprintResources/StandardMacros.IsValid` _array_element
      (:`Is Valid`
        (bind _returnvalue_2 (`NavigationSystemV1.FindPathToLocationSynchronously` (`NavigationSystemV1.K2_ProjectPointToNavigation` (`self.K2_GetActorLocation`)) (`NavigationSystemV1.K2_ProjectPointToNavigation` (`self.K2_GetActorLocation` _array_element)) null null))
        (set `local.Local_NavMeshPathPoints` (`NavigationPath.PathPoints` _returnvalue_2))
        (if (> (`KismetArrayLibrary.Array_Length` (`local.Local_NavMeshPathPoints`)) 1)
          (bind _returnvalue_3 (`AddComponent|NODE_AddSplineComponent-0`))
          (bind _output_get (set `local.Local_Spline` _returnvalue_3))
          (`KismetArrayLibrary.Array_Add` (`self.SplineComponents`) _output_get)
          (`SceneComponent.K2_AddLocalOffset` (`local.Local_Spline`) (`KismetMathLibrary.MakeVector` 0.0 0.0 (`self.SplineHeight`)) false true) ; Lifts up the spline a few units above the ground level
          (`SplineComponent.ClearSplinePoints` (`local.Local_Spline`) true) ; Clears the default spline point
          (`SplineComponent.AddSplinePoint` (`local.Local_Spline`) (`|GetArrayItem` (`local.Local_NavMeshPathPoints`)) "World" true) ; Add a spline point at the path starting location
          (for _index (range (+ (- (`KismetArrayLibrary.Array_Length` (`local.Local_NavMeshPathPoints`)) 2) 1))
            (bind _output_get_2 (set `local.Local_CurrentPathPointIndex` _index))
            (bind _returnvalue_4 (- (`|GetArrayItem` (`local.Local_NavMeshPathPoints`) (+ _output_get_2 1)) (`|GetArrayItem` (`local.Local_NavMeshPathPoints`) (`local.Local_CurrentPathPointIndex`))))
            (set `local.Local_CurrentPathLength` (`KismetMathLibrary.VSize` _returnvalue_4)) ; Distance from current path point to next
            (set `local.Local_CurrentPathUnitVector` (`KismetMathLibrary.Normal` _returnvalue_4)) ; Unit vector from current path point to next
            (set `local.Local_CurrentPathStartingPoint` (`|GetArrayItem` (`local.Local_NavMeshPathPoints`) (`local.Local_CurrentPathPointIndex`))) ; World location at the current path point
            (if (> _returnvalue 0)
              (for _index_2 (range 1 (+ _returnvalue 1))
                (`SplineComponent.AddSplinePoint` (`local.Local_Spline`) (+ (`local.Local_CurrentPathStartingPoint`) (* (`local.Local_CurrentPathUnitVector`) (* _index_2 (`self.AIPathMeshSpacing`)))) "World" true)))
            (`SplineComponent.AddSplinePoint` (`local.Local_Spline`) (`|GetArrayItem` (`local.Local_NavMeshPathPoints`) (+ (`local.Local_CurrentPathPointIndex`) 1)) "World" true) ; Add a spline point at the next path point location
          )
          (else
            (`KismetSystemLibrary.PrintString` "Warning: Exit Point cannot be reached from SpawnPoint"))))))
  (return))

(fn `GetAIObjectiveLocation`
  (returns (ReturnValue :type "Vector Structure"))
  ;[0 1 1 0.5] Returns the final Objective Location for AI units starting from this spawn point
  (if (`self.UseRandomObjective?`)
    (return (`self.K2_GetActorLocation` (`|GetArrayItem` (`self.ObjectivesList`) (`KismetMathLibrary.RandomInteger` (`KismetArrayLibrary.Array_Length` (`self.ObjectivesList`)))))) ; Location of an objective selected at random
    (else
      (return (`self.K2_GetActorLocation` (`self.DesignatedObjective`))) ; Location of the designated objective
    )))

(fn `UserConstructionScript`
  (`parent.UserConstructionScript`))