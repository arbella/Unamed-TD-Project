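; Base enemy spawn point for a tower defense game, spawning delayed batches of AI bots and showing their paths and upcoming wave counts.
; Separate events per enemy class avoid conflicts between overlapping batches, each notifying the batched wave controller when done.
; Bots get data table stats and a random spawn transform with matching spline, while child classes supply transforms and objective location.
; Paths render as spline meshes or instanced static meshes.
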(event `InitializeSpawnPoint`
  ;[0 1 0 0.5] Initialization Protocols
  (switch `/Game/TowerDefenseStarterKit/Blueprints/WaveSpawningSystems/EAIPathDisplayModel` (`self.AIPathVisualizationModel`)
    (:`NewEnumerator1`
      (`self.DisplayAIPathUsingSplineMeshes`))
    (:`NewEnumerator0`
      (`self.DisplayAIPathUsingInstancedStaticMeshes`))))

(event `SetSpawnTransforms`
  ;[0 1 1 0.5] Implemented through Child Classes
)

(event `SpawnAIBatch_TankClass`
  (params (StartDelay :type "Float (double-precision)") (NumberOfUnits :type Integer) (SpawnInterval :type "Float (double-precision)") (CycleMultiplier :type Integer) (DataTableRowName :type Name))
  ;[0 1 1 0.5] Spawns batches of enemy bots based on the specified input parameters [Moved here from the Wave Manager to prevent a bug that arises from event access conflict when multiple groups of the same AI class are spawned from multiple enemy spawn points in the same time frame. Now with the spawn logic moved to the spawn points, each spawn point has it's own set of events that can be called upon without interfering with the other spawn points.]
  (`KismetSystemLibrary.Delay` StartDelay)
  (`self.ForLoopWithDelay` 1 NumberOfUnits SpawnInterval
    (:`LoopBody`
      (`self.SpawnEnemyAIBot` CycleMultiplier DataTableRowName))
    (:`Completed`
      (bind _asbp_batched_wave_spawn_controller (cast `/Game/TowerDefenseStarterKit/Blueprints/WaveSpawningSystems/BP_BatchedWaveSpawnController` (`/Game/TowerDefenseStarterKit/Blueprints/FunctionLibraries/BPFL_GetterFunctions.GetWaveSpawnController` self)))
      (`/Game/TowerDefenseStarterKit/Blueprints/WaveSpawningSystems/BP_BatchedWaveSpawnController.DecrementNumberOfActiveSpawnGroups` _asbp_batched_wave_spawn_controller) ; Spawn group decrement required only for batched spawning system
    )))

(event `SpawnAIBatch_HealerClass`
  (params (StartDelay :type "Float (double-precision)") (NumberOfUnits :type Integer) (SpawnInterval :type "Float (double-precision)") (CycleMultiplier :type Integer) (DataTableRowName :type Name))
  ;[0 1 1 0.5] Spawns batches of enemy bots based on the specified input parameters [Moved here from the Wave Manager to prevent a bug that arises from event access conflict when multiple groups of the same AI class are spawned from multiple enemy spawn points in the same time frame. Now with the spawn logic moved to the spawn points, each spawn point has it's own set of events that can be called upon without interfering with the other spawn points.]
  (`KismetSystemLibrary.Delay` StartDelay)
  (`self.ForLoopWithDelay` 1 NumberOfUnits SpawnInterval
    (:`LoopBody`
      (`self.SpawnEnemyAIBot` CycleMultiplier DataTableRowName))
    (:`Completed`
      (bind _asbp_batched_wave_spawn_controller (cast `/Game/TowerDefenseStarterKit/Blueprints/WaveSpawningSystems/BP_BatchedWaveSpawnController` (`/Game/TowerDefenseStarterKit/Blueprints/FunctionLibraries/BPFL_GetterFunctions.GetWaveSpawnController` self)))
      (`/Game/TowerDefenseStarterKit/Blueprints/WaveSpawningSystems/BP_BatchedWaveSpawnController.DecrementNumberOfActiveSpawnGroups` _asbp_batched_wave_spawn_controller) ; Spawn group decrement required only for batched spawning system
    )))

(event `SpawnAIBatch_RangedClass`
  (params (StartDelay :type "Float (double-precision)") (NumberOfUnits :type Integer) (SpawnInterval :type "Float (double-precision)") (CycleMultiplier :type Integer) (DataTableRowName :type Name))
  ;[0 1 1 0.5] Spawns batches of enemy bots based on the specified input parameters [Moved here from the Wave Manager to prevent a bug that arises from event access conflict when multiple groups of the same AI class are spawned from multiple enemy spawn points in the same time frame. Now with the spawn logic moved to the spawn points, each spawn point has it's own set of events that can be called upon without interfering with the other spawn points.]
  (`KismetSystemLibrary.Delay` StartDelay)
  (`self.ForLoopWithDelay` 1 NumberOfUnits SpawnInterval
    (:`LoopBody`
      (`self.SpawnEnemyAIBot` CycleMultiplier DataTableRowName))
    (:`Completed`
      (bind _asbp_batched_wave_spawn_controller (cast `/Game/TowerDefenseStarterKit/Blueprints/WaveSpawningSystems/BP_BatchedWaveSpawnController` (`/Game/TowerDefenseStarterKit/Blueprints/FunctionLibraries/BPFL_GetterFunctions.GetWaveSpawnController` self)))
      (`/Game/TowerDefenseStarterKit/Blueprints/WaveSpawningSystems/BP_BatchedWaveSpawnController.DecrementNumberOfActiveSpawnGroups` _asbp_batched_wave_spawn_controller) ; Spawn group decrement required only for batched spawning system
    )))

(event `SpawnAIBatch_RunnerClass`
  (params (StartDelay :type "Float (double-precision)") (NumberOfUnits :type Integer) (SpawnInterval :type "Float (double-precision)") (CycleMultiplier :type Integer) (DataTableRowName :type Name))
  ;[0 1 1 0.5] Spawns batches of enemy bots based on the specified input parameters [Moved here from the Wave Manager to prevent a bug that arises from event access conflict when multiple groups of the same AI class are spawned from multiple enemy spawn points in the same time frame. Now with the spawn logic moved to the spawn points, each spawn point has it's own set of events that can be called upon without interfering with the other spawn points.]
  (`KismetSystemLibrary.Delay` StartDelay)
  (`self.ForLoopWithDelay` 1 NumberOfUnits SpawnInterval
    (:`LoopBody`
      (`self.SpawnEnemyAIBot` CycleMultiplier DataTableRowName))
    (:`Completed`
      (bind _asbp_batched_wave_spawn_controller (cast `/Game/TowerDefenseStarterKit/Blueprints/WaveSpawningSystems/BP_BatchedWaveSpawnController` (`/Game/TowerDefenseStarterKit/Blueprints/FunctionLibraries/BPFL_GetterFunctions.GetWaveSpawnController` self)))
      (`/Game/TowerDefenseStarterKit/Blueprints/WaveSpawningSystems/BP_BatchedWaveSpawnController.DecrementNumberOfActiveSpawnGroups` _asbp_batched_wave_spawn_controller) ; Spawn group decrement required only for batched spawning system
    )))

(event `SpawnAIBatch_DisablerClass`
  (params (StartDelay :type "Float (double-precision)") (NumberOfUnits :type Integer) (SpawnInterval :type "Float (double-precision)") (CycleMultiplier :type Integer) (DataTableRowName :type Name))
  ;[0 1 1 0.5] Spawns batches of enemy bots based on the specified input parameters [Moved here from the Wave Manager to prevent a bug that arises from event access conflict when multiple groups of the same AI class are spawned from multiple enemy spawn points in the same time frame. Now with the spawn logic moved to the spawn points, each spawn point has it's own set of events that can be called upon without interfering with the other spawn points.]
  (`KismetSystemLibrary.Delay` StartDelay)
  (`self.ForLoopWithDelay` 1 NumberOfUnits SpawnInterval
    (:`LoopBody`
      (`self.SpawnEnemyAIBot` CycleMultiplier DataTableRowName))
    (:`Completed`
      (bind _asbp_batched_wave_spawn_controller (cast `/Game/TowerDefenseStarterKit/Blueprints/WaveSpawningSystems/BP_BatchedWaveSpawnController` (`/Game/TowerDefenseStarterKit/Blueprints/FunctionLibraries/BPFL_GetterFunctions.GetWaveSpawnController` self)))
      (`/Game/TowerDefenseStarterKit/Blueprints/WaveSpawningSystems/BP_BatchedWaveSpawnController.DecrementNumberOfActiveSpawnGroups` _asbp_batched_wave_spawn_controller) ; Spawn group decrement required only for batched spawning system
    )))

(fn `ComputeSpawnParameters`
  (returns (SpawnTransform :type "Transform Structure") (SplinePath :type "SplineComponent Object Reference"))
  (locals (Local_SpawnPathIndex :type Integer))
  (bind _output (`|GetArrayItem` (`self.BotSpawnTransforms`) (`local.Local_SpawnPathIndex`)))
  ;[0 1 1 0.5] Returns information necessary for spawning enemy units
  (set `local.Local_SpawnPathIndex` (`KismetMathLibrary.RandomInteger` (`KismetArrayLibrary.Array_Length` (`self.BotSpawnTransforms`))))
  (if (> (`KismetArrayLibrary.Array_Length` (`self.SplineComponents`)) (`local.Local_SpawnPathIndex`))
    (return _output (`|GetArrayItem` (`self.SplineComponents`) (`local.Local_SpawnPathIndex`)))
    (else
      (return _output null))))

(fn `DisplayAIPathUsingInstancedStaticMeshes`
  (locals (Local_Spline :type "SplineComponent Object Reference"))
  ;[0 1 1 0.5] Displays AI path using Instanced Static Meshes
  (for _array_element (`self.SplineComponents`)
    (set `local.Local_Spline` _array_element)
    (for _index (range (+ (`.ReturnValue` (`KismetMathLibrary.FMod` (`SplineComponent.GetSplineLength` (`local.Local_Spline`)) (`self.AIPathMeshSpacing`))) 1))
      (`InstancedStaticMeshComponent.AddInstance` (`self.PathMarker`) (`KismetMathLibrary.MakeTransform` (.location (`SplineComponent.GetTransformAtDistanceAlongSpline` (`local.Local_Spline`) (* _index (`self.AIPathMeshSpacing`)) "Local" false)) (`KismetMathLibrary.MakeRotator` (.roll (.rotation (`SplineComponent.GetTransformAtDistanceAlongSpline` (`local.Local_Spline`) (* _index (`self.AIPathMeshSpacing`)) "Local" false))) (.pitch (.rotation (`SplineComponent.GetTransformAtDistanceAlongSpline` (`local.Local_Spline`) (* _index (`self.AIPathMeshSpacing`)) "Local" false))) (+ (.yaw (.rotation (`SplineComponent.GetTransformAtDistanceAlongSpline` (`local.Local_Spline`) (* _index (`self.AIPathMeshSpacing`)) "Local" false))) 90.0)) (.scale (`SplineComponent.GetTransformAtDistanceAlongSpline` (`local.Local_Spline`) (* _index (`self.AIPathMeshSpacing`)) "Local" false))))))
  (return))

(fn `DisplayAIPathUsingSplineMeshes`
  (locals (Local_CurrentSplineMesh :type "SplineMeshComponent Object Reference") (Local_CurrentSpline :type "SplineComponent Object Reference"))
  (bind _local_currentspline (`local.Local_CurrentSpline`))
  (bind _aipathmeshspacing (`self.AIPathMeshSpacing`))
  ;[0 1 1 0.5] Displays AI path using Spline Meshes
  (for _array_element (`self.SplineComponents`)
    (set `local.Local_CurrentSpline` _array_element)
    (for _index (range (+ (`.ReturnValue` (`KismetMathLibrary.FMod` (`SplineComponent.GetSplineLength` (`local.Local_CurrentSpline`)) (`self.AIPathMeshSpacing`))) 1))
      (bind _returnvalue (`AddComponent|NODE_AddSplineMeshComponent-0` :`bManualAttachment` true))
      (bind _output_get (set `local.Local_CurrentSplineMesh` _returnvalue))
      (`StaticMeshComponent.SetStaticMesh` _output_get "/Game/TowerDefenseStarterKit/Meshes/SM_PlaneSpline.SM_PlaneSpline")
      (`PrimitiveComponent.SetMaterial` (`local.Local_CurrentSplineMesh`) 0 "/Game/TowerDefenseStarterKit/Materials/M_Emissive.M_Emissive")
      (bind _returnvalue_2 (* _index _aipathmeshspacing))
      (bind _returnvalue_3 (+ _returnvalue_2 _aipathmeshspacing))
      (`SplineMeshComponent.SetStartAndEnd` (`local.Local_CurrentSplineMesh`) (`SplineComponent.GetLocationAtDistanceAlongSpline` _local_currentspline _returnvalue_2 "World") (* (`SplineComponent.GetDirectionAtDistanceAlongSpline` _local_currentspline _returnvalue_2 "World") (`self.AIPathMeshSpacing`)) (`SplineComponent.GetLocationAtDistanceAlongSpline` _local_currentspline _returnvalue_3 "World") (* (`SplineComponent.GetDirectionAtDistanceAlongSpline` _local_currentspline _returnvalue_3 "World") (`self.AIPathMeshSpacing`)) true)))
  (return))

(fn `DisplayWaveInformation`
  (locals (Local_EnemySpawnCountData :type "Array of /Game/TowerDefenseStarterKit/Blueprints/WaveSpawningSystems/Struct_EnemyAISpawnCounter Structure"))
  ;[0 1 1 0.5] Display enemy spawn count information about the upcoming wave [for Unit Based & Group Based Wave Generation]
  (bind _asbp_batched_wave_spawn_controller (cast `/Game/TowerDefenseStarterKit/Blueprints/WaveSpawningSystems/BP_BatchedWaveSpawnController` (`/Game/TowerDefenseStarterKit/Blueprints/FunctionLibraries/BPFL_GetterFunctions.GetWaveSpawnController` self))
    (:`then`
      (bind _enemyspawncountdata (`/Game/TowerDefenseStarterKit/Blueprints/WaveSpawningSystems/BP_BatchedWaveSpawnController.RetrieveSpawnCountDataForUpcomingWave` _asbp_batched_wave_spawn_controller self))
      (set `local.Local_EnemySpawnCountData` _enemyspawncountdata)
      (if (> (`KismetArrayLibrary.Array_Length` (`local.Local_EnemySpawnCountData`)) 0)
        (for _array_element (`local.Local_EnemySpawnCountData`)
          (bind _returnvalue (`|CreateWidget` (`self.EnemyDataWidgetClass`) (`GameplayStatics.GetPlayerController` 0)))
          (bind (_datatablerowname _spawncount) (break `/Game/TowerDefenseStarterKit/Blueprints/WaveSpawningSystems/Struct_EnemyAISpawnCounter` _array_element))
          (bind _returnvalue_2 (`|GetDataTableRow` "/Game/TowerDefenseStarterKit/Blueprints/AI/Enemy/DT_EnemyAIStats.DT_EnemyAIStats" _datatablerowname)
            (:`then`
              (`/Game/TowerDefenseStarterKit/UI/Generic/Widget_Stats.UpdateStatsData` _returnvalue (`.AIName_10_DC22B5F74D0BFCF9CA947099FA3F938E` (break `/Game/TowerDefenseStarterKit/Blueprints/AI/Enemy/Struct_EnemyAIData` _returnvalue_2)) (`KismetTextLibrary.Conv_IntToText` _spawncount))
              (bind _aswidget_wave_spawn_details (cast `/Game/TowerDefenseStarterKit/UI/Generic/Widget_WaveSpawnDetails` (`WidgetComponent.GetUserWidgetObject` (`self.WaveDataDisplay`))))
              (`/Game/TowerDefenseStarterKit/UI/Generic/Widget_WaveSpawnDetails.AddNewStatsToWaveData` _aswidget_wave_spawn_details _returnvalue))
            (:`RowNotFound`
              (`KismetSystemLibrary.PrintString` "WARNING: [BP_EnemySpawnPoint] Function 'DisplayWaveInformation' could not get the requested row from Data Table 'DT_EnemeyAIStats'"))))
        (`SceneComponent.SetHiddenInGame` (`self.WaveDataDisplay`) false false)
        (else
          (`SceneComponent.SetHiddenInGame` (`self.WaveDataDisplay`) true false :!label _label))))
    (:`CastFailed`
      (goto _label))))

(fn `GetAIObjectiveLocation`
  (returns (ReturnValue :type "Vector Structure"))
  ;[0 1 1 0.5] Returns the final Objective Location for AI units starting from this spawn point [Implemented through Child Classes]
  (return (0.0 0.0 0.0)))

(fn `HideWaveDataDisplay`
  ;[0 1 1 0.5] Hides the Wave Data Display widget & clears existing wave data
  (`SceneComponent.SetHiddenInGame` (`self.WaveDataDisplay`) true false)
  (bind _aswidget_wave_spawn_details (cast `/Game/TowerDefenseStarterKit/UI/Generic/Widget_WaveSpawnDetails` (`WidgetComponent.GetUserWidgetObject` (`self.WaveDataDisplay`))))
  (`/Game/TowerDefenseStarterKit/UI/Generic/Widget_WaveSpawnDetails.ResetWaveData` _aswidget_wave_spawn_details))

(fn `SpawnEnemyAIBot`
  (params (CycleMultiplier :type Integer) (DataTableRowName :type Name))
  (locals (Local_SpawnTransform :type "Transform Structure") (Local_SplinePath :type "SplineComponent Object Reference"))
  ;[0 1 1 0.5] Spawns an Enemy AI bot
  (bind _returnvalue (`|GetDataTableRow` "/Game/TowerDefenseStarterKit/Blueprints/AI/Enemy/DT_EnemyAIStats.DT_EnemyAIStats" DataTableRowName)
    (:`then`
      (bind (_spawntransform _splinepath) (`self.ComputeSpawnParameters`))
      (set `local.Local_SpawnTransform` _spawntransform)
      (set `local.Local_SplinePath` _splinepath)
      (bind (_aiclass _aitype _ainame _aidescription _hp _attackdamage _crithitchance _crithitdamagemultiplier _attackanimduration _visionangle _visionrange _attackrange _maxmovementspeed _maxaccelerationsplinemotion _threatrating _playerscoremodifier) (break `/Game/TowerDefenseStarterKit/Blueprints/AI/Enemy/Struct_EnemyAIData` _returnvalue))
      (bind _returnvalue_2 (`|SpawnActorFromClass` _aiclass (`local.Local_SpawnTransform`) "AlwaysSpawn" "OverrideRootScale" null CycleMultiplier DataTableRowName _aitype _ainame _aidescription _hp _attackdamage _crithitchance _crithitdamagemultiplier _attackanimduration _visionangle _visionrange _attackrange _maxmovementspeed _maxaccelerationsplinemotion _threatrating _playerscoremodifier (`local.Local_SplinePath`) (`self.GetAIObjectiveLocation`) (`self.AINavigationModel`) null))
      (`self.EnemyUnitSpawned` _returnvalue_2) ; Event Dispatcher called to notify all listeners about an Enemy Unit Spawn event
      (return))
    (:`RowNotFound`
      (`KismetSystemLibrary.PrintString` "WARNING: [BP_EnemySpawnPoint] Function 'SpawnEnemyAIBot' could not get the requested row from Data Table 'DT_EnemeyAIStats'"))))

(fn `UserConstructionScript`)