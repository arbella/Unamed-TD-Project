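; Support tower that raises the output multiplier of non-Boost towers within its range sphere by its own true output per cycle.
; Towers are boosted on overlap or when core systems are enabled, and unboosted when systems are disabled or play ends.
; Output changes, upgrades and level-ups remove the boost before calling the parent, then reapply it.
; A count of boosted towers drives a looping recharge-time timer that grants tower XP.
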(event `self.RangeSphere.OnComponentBeginOverlap`
  (params (OverlappedComponent :type "PrimitiveComponent Object Reference") (OtherActor :type "Actor Object Reference") (OtherComp :type "PrimitiveComponent Object Reference") (OtherBodyIndex :type Integer) (bFromSweep :type Boolean) (SweepResult :type "HitResult Structure (by ref)"))
  ;[0 1 1 0.5] Boost new overlapping towers
  (bind _asbp_tower_parent (cast `/Game/TowerDefenseStarterKit/Blueprints/Towers/BP_Tower_Parent` OtherActor))
  (`self.BoostSelectedTower` _asbp_tower_parent))

(event `self.RangeSphere.OnComponentEndOverlap`
  (params (OverlappedComponent :type "PrimitiveComponent Object Reference") (OtherActor :type "Actor Object Reference") (OtherComp :type "PrimitiveComponent Object Reference") (OtherBodyIndex :type Integer))
  ;[0 1 1 0.5] Keeps track of boosted towers whose link gets cut off
  (cast `/Game/TowerDefenseStarterKit/Blueprints/Towers/BP_Tower_Parent` OtherActor)
  (`self.DecrementNumberOfBoostedTowers`))

(event `self.ModifyOutputMultiplier`
  (params (By :type "Float (single-precision)"))
  ;[0 1 1 0.5] Every time this tower gets an output boost, apply the new updated boost to all towers in range
  (`self.RemoveBoostForAllTowersInRange`)
  (`parent.ModifyOutputMultiplier` By)
  (`self.BoostAllTowersInRange`))

(event `self.DisableCoreTowerSystems`
  ;[0 1 1 0.5] Turns on/off core tower functionality
  (`self.RemoveBoostForAllTowersInRange`))

(event `self.EnableCoreTowerSystems`
  ;[0 1 1 0.5] Turns on/off core tower functionality
  (`self.BoostAllTowersInRange`))

(event `self.ReceiveEndPlay`
  (params (EndPlayReason :type "EEndPlayReason Enum" :default "Destroyed"))
  ;[1 0 0 0.5] Remove Boost when before tower is destroyed
  (`self.RemoveBoostForAllTowersInRange`)
  (`parent.ReceiveEndPlay` EndPlayReason))

(event `self.UpgradeTower`
  (params (TowerModel :type "/Game/TowerDefenseStarterKit/Blueprints/Towers/ETowerModels Enum" :default "NewEnumerator2") (OutputPerCycle :type "Float (single-precision)") (RechargeTime :type "Float (single-precision)") (MaxArmor :type "Float (single-precision)") (Range :type "Float (single-precision)") (ResourceCap :type "Float (single-precision)") (TowerMesh :type "StaticMesh Object Reference") (TowerName :type Text) (ShortDescription :type Text))
  ;[0 1 1 0.5] Override function used to upgrade tower
  (`self.RemoveBoostForAllTowersInRange`)
  (`parent.UpgradeTower` TowerModel OutputPerCycle RechargeTime MaxArmor Range ResourceCap TowerMesh TowerName ShortDescription)
  (`self.BoostAllTowersInRange`))

(event `/Game/TowerDefenseStarterKit/Blueprints/Towers/SupportSystems/BPI_TowerLevelUpSystem.TowerSkillLevelUpgraded`
  (params (NewLevel :type Integer) (LevelUpStatModifiers :type "/Game/TowerDefenseStarterKit/Blueprints/Towers/SupportSystems/Struct_TowerLevelUpStatModifiers Structure"))
  ;[0 1 0.4 0.5] BPI_TowerLevelUpSystem interface functions
  (`self.RemoveBoostForAllTowersInRange`)
  (`parent.TowerSkillLevelUpgraded` NewLevel LevelUpStatModifiers)
  (`self.BoostAllTowersInRange`))

(fn `BoostAllTowersInRange`
  ;[0 1 1 0.5] Boost all other non-Boost Towers in Range
  (for _array_element (`PrimitiveComponent.GetOverlappingActors` (`self.RangeSphere`) "/Game/TowerDefenseStarterKit/Blueprints/Towers/BP_Tower_Parent.BP_Tower_Parent_C")
    (bind _asbp_tower_parent (cast `/Game/TowerDefenseStarterKit/Blueprints/Towers/BP_Tower_Parent` _array_element))
    (`self.BoostSelectedTower` _asbp_tower_parent))
  (return))

(fn `BoostSelectedTower`
  (params (Tower :type "/Game/TowerDefenseStarterKit/Blueprints/Towers/BP_Tower_Parent Object Reference"))
  ;[0 1 1 0.5] Boost nearby tower as long as it's not a Boost Tower itself
  (cast `/Game/TowerDefenseStarterKit/Blueprints/Towers/BP_BoostTower` Tower ; Do not boost other Boost Towers
    (:`CastFailed`
      (`self.ModifyOutputMultiplier` Tower (`self.CalculateTrueOutputPerCycle`))
      (`self.IncrementNumberOfBoostedTowers`))))

(fn `DecrementNumberOfBoostedTowers`
  ;[0 1 1 0.5] Decrements the number of boosted towers data & disables the output tracker if necessary
  (bind _output_get (set `self.NumberOfTowersBoosted` (- (`self.NumberOfTowersBoosted`) 1)))
  (if (== _output_get 0)
    (`self.DisableBoostOutputTracker`) ; Disables tracking if there no towers are being boosted
  ))

(fn `DisableBoostOutputTracker`
  ;[0 1 1 0.5] Disables the timer that tracks the boost output over time
  (if (`KismetSystemLibrary.K2_TimerExistsHandle` (`self.BoostOutputTrackerTimer`))
    (`KismetSystemLibrary.K2_ClearAndInvalidateTimerHandle` (`self.BoostOutputTrackerTimer`)))
  (set `self.NumberOfTowersBoosted` 0))

(fn `EnableBoostOutputTracker`
  ;[0 1 1 0.5] Activates a timer to keep track of boost output over time [Used only as a means to measure the experience gain]
  (if (not (`KismetSystemLibrary.K2_TimerExistsHandle` (`self.BoostOutputTrackerTimer`)))
    (bind _returnvalue (`KismetSystemLibrary.K2_SetTimer` null "TrackBoostOutputGeneration" (`self.RechargeTime`) true))
    (set `self.BoostOutputTrackerTimer` _returnvalue))
  (return))

(fn `IncrementNumberOfBoostedTowers`
  ;[0 1 1 0.5] Increments the number of boosted towers data & starts the output tracker if necessary
  (set `self.NumberOfTowersBoosted` (+ (`self.NumberOfTowersBoosted`) 1))
  (`self.EnableBoostOutputTracker`)
  (return))

(fn `RemoveBoostForAllTowersInRange`
  ;[1 0.5 0.2 0.5] Remove Boost for all other non-Boost Towers in Range
  (for _array_element (`PrimitiveComponent.GetOverlappingActors` (`self.RangeSphere`) "/Game/TowerDefenseStarterKit/Blueprints/Towers/BP_Tower_Parent.BP_Tower_Parent_C")
    (bind _asbp_tower_parent (cast `/Game/TowerDefenseStarterKit/Blueprints/Towers/BP_Tower_Parent` _array_element))
    (`self.RemoveBoostForSelectedTower` _asbp_tower_parent))
  (return))

(fn `RemoveBoostForSelectedTower`
  (params (Tower :type "/Game/TowerDefenseStarterKit/Blueprints/Towers/BP_Tower_Parent Object Reference"))
  ;[1 0.5 0.2 0.5] Remove boost from nearby tower if it's not a Boost Tower itself
  (cast `/Game/TowerDefenseStarterKit/Blueprints/Towers/BP_BoostTower` Tower ; Do not boost other Boost Towers
    (:`CastFailed`
      (`self.ModifyOutputMultiplier` Tower (* (`self.CalculateTrueOutputPerCycle`) -1.0))
      (`self.DecrementNumberOfBoostedTowers`))))

(fn `TrackBoostOutputGeneration`
  ;[0 1 1 0.5] Reports the boost output
  (`/Game/TowerDefenseStarterKit/Blueprints/Towers/SupportSystems/BPC_TowerXPManager.IncrementTowerXP` (`self.TowerXPManager`)) ; XP incremented for every output cycle
  (return))

(fn `UserConstructionScript`
  (`parent.UserConstructionScript`))