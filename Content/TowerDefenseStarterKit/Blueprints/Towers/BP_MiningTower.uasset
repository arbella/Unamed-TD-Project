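; Tower defense mining tower that earns Tower Points for the player from a finite resource pool.
; A looping timer harvests each recharge cycle, draining the pool, granting tower XP and adding points to BP_PlayerState until depleted.
; Upgrades restart harvesting, while system toggles stop it or resume it if resources remain.
; A dynamic material color shows active or stopped state, and the unneeded range sphere collision is disabled.
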(event `self.ReceiveBeginPlay`
  ;[0 1 1 0.5] Start Resource Generation at Begin Play Event; If resource generation has stopped due to depleted resources, an Upgrade event will kickstart it again using the new resource pool; Charged color [White] represents a functional Mining Tower
  (`parent.ReceiveBeginPlay`)
  (`self.EnableResourceHarvester` :!label _label))

(event `self.UpgradeTower`
  (params (TowerModel :type "/Game/TowerDefenseStarterKit/Blueprints/Towers/ETowerModels Enum" :default "NewEnumerator2") (OutputPerCycle :type "Float (single-precision)") (RechargeTime :type "Float (single-precision)") (MaxArmor :type "Float (single-precision)") (Range :type "Float (single-precision)") (ResourceCap :type "Float (single-precision)") (TowerMesh :type "StaticMesh Object Reference") (TowerName :type Text) (ShortDescription :type Text))
  ;[0 1 1 0.5] Start Resource Generation at Begin Play Event; If resource generation has stopped due to depleted resources, an Upgrade event will kickstart it again using the new resource pool; Charged color [White] represents a functional Mining Tower
  (`parent.UpgradeTower` TowerModel OutputPerCycle RechargeTime MaxArmor Range ResourceCap TowerMesh TowerName ShortDescription)
  (goto _label))

(event `self.DisableCoreTowerSystems`
  ;[0 1 1 0.5] Turns on/off core tower functionality
  (`self.DisableResourceHarvester`))

(event `self.EnableCoreTowerSystems`
  ;[0 1 1 0.5] Turns on/off core tower functionality
  (if (> (`self.ResourcesLeft`) 0.0)
    (`self.EnableResourceHarvester`) ; Restarts the resource harvester if resources are left to be mined
  ))

(fn `DisableResourceHarvester`
  ;[0 1 1 0.5] Stop the resoure harvest timer
  (if (`KismetSystemLibrary.K2_TimerExistsHandle` (`self.HarvestResourcesTimer`))
    (`KismetSystemLibrary.K2_ClearAndInvalidateTimerHandle` (`self.HarvestResourcesTimer`))
    (`MaterialInstanceDynamic.SetVectorParameterValue` (`self.MID_TowerMaterial`) "Color" (`self.DischargedColor`))))

(fn `EnableResourceHarvester`
  ;[0 1 1 0.5] Starts timer based resource harvesting operations
  (if (not (`KismetSystemLibrary.K2_TimerExistsHandle` (`self.HarvestResourcesTimer`)))
    (bind _returnvalue (`KismetSystemLibrary.K2_SetTimer` null "HarvestResources" (`self.RechargeTime`) true))
    (set `self.HarvestResourcesTimer` _returnvalue)
    (`MaterialInstanceDynamic.SetVectorParameterValue` (`self.MID_TowerMaterial`) "Color" (`self.ChargedColor`))))

(fn `HarvestResources`
  (locals (Local_TowerPointsGenerated :type "Float (double-precision)"))
  (bind _value (`self.CalculateTrueOutputPerCycle`))
  ;[0 1 1 0.5] Update Tower Points & Reduce available resources; If no resources left, stop timer; Discharged color [Grey] represents depleted resources
  (if (> (`self.ResourcesLeft`) _value)
    (set `local.Local_TowerPointsGenerated` _value)
    (else
      (set `local.Local_TowerPointsGenerated` (`self.ResourcesLeft`))
      (`self.DisableResourceHarvester`)))
  (set `self.ResourcesLeft` (- (`self.ResourcesLeft`) (`local.Local_TowerPointsGenerated`)))
  (`/Game/TowerDefenseStarterKit/Blueprints/Towers/SupportSystems/BPC_TowerXPManager.IncrementTowerXP` (`self.TowerXPManager`)) ; XP incremented for every output cycle
  ;;[1 0.8203 0] Version 2.8: Tower Points now stored in Player State
  (bind _asbp_player_state (cast `/Game/TowerDefenseStarterKit/Blueprints/Player/BP_PlayerState` (`Controller.PlayerState` (`GameplayStatics.GetPlayerController` 0))))
  (`/Game/TowerDefenseStarterKit/Blueprints/Player/BP_PlayerState.ModifyTowerPoints` _asbp_player_state (`KismetMathLibrary.FTrunc` (`local.Local_TowerPointsGenerated`))))

(fn `RetrieveTargetInfo`
  (returns (Name :type Text) (Description :type Text) (Stats :type "Array of /Game/TowerDefenseStarterKit/Blueprints/HUDControl/Struct_HUDStats Structure"))
  ;[0 1 0.4 0.5] BPI_TargetInfoDisplay interface function
  (return (`self.TowerName`) (`self.ShortDescription`) (`|MakeArray` (make `/Game/TowerDefenseStarterKit/Blueprints/HUDControl/Struct_HUDStats` (`self.UIStatName_CoreFunction`) (`KismetTextLibrary.Conv_DoubleToText` (/ (`self.OutputPerCycle`) (`self.RechargeTime`)) "HalfToEven")) (make `/Game/TowerDefenseStarterKit/Blueprints/HUDControl/Struct_HUDStats` (`self.UIStatName_Defense`) (`KismetTextLibrary.Conv_IntToText` (`KismetMathLibrary.Round` (`self.MaxArmor`)))) (make `/Game/TowerDefenseStarterKit/Blueprints/HUDControl/Struct_HUDStats` (`self.UIStatName_LimitingFactor`) (`KismetTextLibrary.Conv_IntToText` (`KismetMathLibrary.Round` (`self.ResourcesLeft`)))))))

(fn `UserConstructionScript`
  (bind _tower (`self.Tower`))
  (`parent.UserConstructionScript`)
  ;[0 1 1 0.5] Deactivate range sphere collision as it's not required for this tower; Create Dynamic material instance to display working status of the tower
  (`PrimitiveComponent.SetCollisionEnabled` (`self.RangeSphere`) "NoCollision")
  (bind _returnvalue (`PrimitiveComponent.CreateDynamicMaterialInstance` _tower 0 (`PrimitiveComponent.GetMaterial` _tower 0) "None"))
  (set `self.MID_TowerMaterial` _returnvalue))