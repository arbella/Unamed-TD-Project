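; Actor component for tower defense towers that runs an optional XP-based leveling system.
; On BeginPlay it requires the owner to implement CommunicationInterface, sets the first XP target and notifies the owner.
; IncrementTowerXP adds a fixed boost per output cycle, raising the level at the target and sending the owner stat modifiers.
; Targets grow by level times base XP, and upgrades recurse to absorb multiple level-ups.
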(event `self.ReceiveBeginPlay`
  ;[0 1 0 0.5] Initialization
  (if (`self.ActivateLevelUpSystem?`)
    (if (`KismetSystemLibrary.DoesImplementInterface` (`self.GetOwner`) (`self.CommunicationInterface`))
      (`self.ExecuteInitializationProtocols`)
      (message `/Game/TowerDefenseStarterKit/Blueprints/Towers/SupportSystems/BPI_TowerLevelUpSystem.TowerLevelUpSystemInitialized` (`self.GetOwner`)) ; Reports to the owning actor that the component has been initialized
      (else
        (`KismetSystemLibrary.PrintString` "WARNING: Owner does not meet interface requirements; Class: BPC_TowerXPManager")))))

(fn `ExecuteInitializationProtocols`
  ;[0 1 1 0.5] Initialization Protocols
  (`self.SetXPTargetForNextLevel`)
  (return))

(fn `IncrementTowerXP`
  ;[0 1 1 0.5] Increments the experience points of the tower based on the output & upgrades the level if necessary
  (if (`self.ActivateLevelUpSystem?`)
    (bind _output_get (set `self.CurrentXP` (+ (`self.CurrentXP`) (`self.XPBoostPerOutputCycle`))))
    (if (not (< _output_get (`self.XPTargetForNextLevel`)))
      (`self.UpgradeTowerSkillLevel`))
    (return)))

(fn `SetXPTargetForNextLevel`
  ;[0 1 1 0.5] Sets the XP gain required to reach the next level
  (set `self.XPTargetForNextLevel` (+ (`self.XPTargetForNextLevel`) (* (`self.TowerLevel`) (`self.BaseXPTarget`))))
  (return))

(fn `UpgradeTowerSkillLevel`
  ;[0 1 1 0.5] Upgrades tower level & passes the necessary information back to the owning actor
  (set `self.TowerLevel` (+ (`self.TowerLevel`) 1)) ; Tower level raised
  (message `/Game/TowerDefenseStarterKit/Blueprints/Towers/SupportSystems/BPI_TowerLevelUpSystem.TowerSkillLevelUpgraded` (`self.GetOwner`) (`self.TowerLevel`) (`self.LevelUpStatModifierData`)) ; Reports to the owning actor about the Skill Level Upgrade
  (`self.SetXPTargetForNextLevel`) ; Sets a new target
  (if (not (< (`self.CurrentXP`) (`self.XPTargetForNextLevel`)))
    (`self.UpgradeTowerSkillLevel`))
  (return))