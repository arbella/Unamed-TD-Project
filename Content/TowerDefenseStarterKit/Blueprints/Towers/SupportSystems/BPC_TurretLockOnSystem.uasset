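; Turret lock-on component for the tower defense kit that picks and tracks enemy targets for an owner implementing BPI_TurretLockOnSystem.
; A looping acquisition timer selects the first potential target with line of sight, stopping when none remain.
; A second timer at the turret's recharge interval rechecks sight, then orders an attack or drops the lock and resumes searching.
; The owner handles sight checks, turret tracking and attacks through interface messages.
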(event `self.ReceiveBeginPlay`
  ;[0 1 1 0.5] Component Initialization logic
  (if (`KismetSystemLibrary.DoesImplementInterface` (`self.GetOwner`) "/Game/TowerDefenseStarterKit/Blueprints/Towers/SupportSystems/BPI_TurretLockOnSystem.BPI_TurretLockOnSystem_C")
    (`self.EnableLockOnSystem`) ; Enables the Lock-on sytem by default
    (else
      (`self.DisplayOwnerIncompatibilityWarning`) ; Prints out a warning message if the owning actor meets the compatibility requirements
    )))

(fn `AcquireNewTarget`
  ;[0 1 1 0.5] Target Acquisition
  (if (`self.CheckPotentialTargetsAvailability`)
    (`/Engine/EditorBlueprintResources/StandardMacros.IsValid` (`self.ActiveTarget`)
      (:`Is Not Valid`
        (bind _success_ (`self.SelectNewLockOnTarget`)) ; Selects a new active target from a pool of potential targets
        (if _success_
          (`self.LockOnToActiveTarget`))))
    (else
      (`self.TerminateTargetAcquisition`) ; Terminates target acquisition ops if the owner has no potential targets
    )))

(fn `CancelLockOnToActiveTarget`
  ;[0 1 1 0.5] Cancels lock-on targeting operations
  (`KismetSystemLibrary.K2_ClearAndInvalidateTimerHandle` (`self.EvaluateLockOnStatusTimerHandle`))
  (message `/Game/TowerDefenseStarterKit/Blueprints/Towers/SupportSystems/BPI_TurretLockOnSystem.DisableTurretTracking` (`self.GetOwner`)) ; Alerts the owner to stop the turrets from focusing on anything
  (`self.UpdateActiveTarget` null) ; Remove reference to any existing active target actor
  (return))

(fn `CheckPotentialTargetsAvailability`
  (returns (`Success?` :type Boolean))
  ;[0 1 1 0.5] Check if the owning actor has any potential targets within it's range
  (return (> (`KismetArrayLibrary.Array_Length` (`self.PotentialTargets`)) 0)))

(fn `DisableLockOnSystem`
  ;[0 1 1 0.5] Disables the lock on system & aborts all associated operations
  (set `self.LockOnSystemEnabled?` false)
  (`self.CancelLockOnToActiveTarget`) ; Cancels any existing target lock on functions
  (`self.TerminateTargetAcquisition`) ; Prevents further target acquisitions
  (return))

(fn `DisplayOwnerIncompatibilityWarning`
  ;[0 0 0 0.5] Prints a warning message if the owning actor does not implement the requisite interface
  (`KismetSystemLibrary.PrintString` (`KismetStringLibrary.Concat_StrStr` "Warning: [Class: BPC_TurretLockOnSystem] Owning actor '" (`KismetSystemLibrary.GetDisplayName` (`self.GetOwner`)) "' does not implement requisite interface")))

(fn `EnableLockOnSystem`
  ;[0 1 1 0.5] Enables the lock on system & starts target acquisition operations
  (set `self.LockOnSystemEnabled?` true)
  (`self.InitiateTargetAcquisition`)
  (return))

(fn `EvaluateLockOnStatus`
  ;[0 1 1 0.5] Performs validation & line of sight/projectile path checks toward the active target & determines appropriate course of action
  (`/Engine/EditorBlueprintResources/StandardMacros.IsValid` (`self.ActiveTarget`)
    (:`Is Valid`
      (bind _success_ (message `/Game/TowerDefenseStarterKit/Blueprints/Towers/SupportSystems/BPI_TurretLockOnSystem.EvaluateLoSToTarget` (`self.GetOwner`) (`self.ActiveTarget`))) ; Requests the owning actor to determine if the necessary Line of Sight requirements are met
      (if _success_
        (message `/Game/TowerDefenseStarterKit/Blueprints/Towers/SupportSystems/BPI_TurretLockOnSystem.AttackActiveTarget` (`self.GetOwner`)) ; Requests the owning actor to attack the active target
        (else
          (`self.CancelLockOnToActiveTarget` :!label _label)
          (`self.InitiateTargetAcquisition`) ; Initializes target acquisition operations to find a new target
        )))
    (:`Is Not Valid`
      (goto _label))))

(fn `InitiateTargetAcquisition`
  ;[0 1 1 0.5] Initiates the target acquisition checks if it hasn't been activated already
  (if (not (`self.IsTargetAcquisitionActive?`))
    (bind _returnvalue (`KismetSystemLibrary.K2_SetTimer` self "AcquireNewTarget" (`self.TargetAcquisitionTimerInterval`) true))
    (set `self.TargetAcquisitionTimerHandle` _returnvalue)))

(fn `IsLockOnSystemActive?`
  (returns (`SystemActivated?` :type Boolean))
  (return (`self.LockOnSystemEnabled?`)))

(fn `IsTargetAcquisitionActive?`
  (returns (`Yes?` :type Boolean))
  (return (`KismetSystemLibrary.K2_TimerExistsHandle` (`self.TargetAcquisitionTimerHandle`))))

(fn `LockOnToActiveTarget`
  ;[0 1 1 0.5] Activates a timer driven Targeting system
  (bind _rechargetime (message `/Game/TowerDefenseStarterKit/Blueprints/Towers/SupportSystems/BPI_TurretLockOnSystem.RetrieveTurretRechargeTime` (`self.GetOwner`)))
  (bind _returnvalue (`KismetSystemLibrary.K2_SetTimer` self "EvaluateLockOnStatus" _rechargetime true))
  (set `self.EvaluateLockOnStatusTimerHandle` _returnvalue)
  (message `/Game/TowerDefenseStarterKit/Blueprints/Towers/SupportSystems/BPI_TurretLockOnSystem.EnableTurretTracking` (`self.GetOwner`)) ; Alerts the owner to focus it's turrets, if any
  (return))

(fn `NewPotentialTargetDetected`
  (params (TargetActor :type "Actor Object Reference"))
  ;[0 1 1 0.5] Handles target acquisition logic when a new potential target has been detected by the owning actor
  (bind _asbp_enemy_ai_parent (cast `/Game/TowerDefenseStarterKit/Blueprints/AI/Enemy/BP_EnemyAI_Parent` TargetActor))
  (`KismetArrayLibrary.Array_Add` (`self.PotentialTargets`) _asbp_enemy_ai_parent) ; Updates the potential targets array
  (if (`self.LockOnSystemEnabled?`)
    (`self.InitiateTargetAcquisition`)))

(fn `PotentialTargetLost`
  (params (TargetActor :type "Actor Object Reference"))
  ;[0 1 1 0.5] Handles potential targets list updates when a target has been lost
  (bind _asbp_enemy_ai_parent (cast `/Game/TowerDefenseStarterKit/Blueprints/AI/Enemy/BP_EnemyAI_Parent` TargetActor))
  (if (`KismetArrayLibrary.Array_Contains` (`self.PotentialTargets`) _asbp_enemy_ai_parent)
    (`KismetArrayLibrary.Array_RemoveItem` (`self.PotentialTargets`) _asbp_enemy_ai_parent)
    (if (== TargetActor (`self.ActiveTarget`))
      (`self.UpdateActiveTarget` null))))

(fn `RetrieveActiveTarget`
  (returns (ActiveTarget :type "/Game/TowerDefenseStarterKit/Blueprints/AI/Enemy/BP_EnemyAI_Parent Object Reference"))
  (return (`self.ActiveTarget`)))

(fn `SelectNewLockOnTarget`
  (returns (`Success?` :type Boolean))
  (locals (`Local_TargetAcquired?` :type Boolean))
  ;[0 1 1 0.5] Selects a new target for the owner from a pool of it's potential targets
  (set `local.Local_TargetAcquired?` false)
  (for _array_element (`self.PotentialTargets`)
    (`/Engine/EditorBlueprintResources/StandardMacros.IsValid` _array_element
      (:`Is Valid`
        (bind _success_ (message `/Game/TowerDefenseStarterKit/Blueprints/Towers/SupportSystems/BPI_TurretLockOnSystem.EvaluateLoSToTarget` (`self.GetOwner`) _array_element)) ; Check if line of sight can be established
        (bind _output_get (set `local.Local_TargetAcquired?` _success_))
        (if _output_get
          (`self.UpdateActiveTarget` _array_element) ; Sets a new active target
          (break)))))
  (return (`local.Local_TargetAcquired?`)))

(fn `TerminateTargetAcquisition`
  ;[0 1 1 0.5] Stops target acquisition checks
  (`KismetSystemLibrary.K2_ClearAndInvalidateTimerHandle` (`self.TargetAcquisitionTimerHandle`))
  (return))

(fn `UpdateActiveTarget`
  (params (NewTarget :type "/Game/TowerDefenseStarterKit/Blueprints/AI/Enemy/BP_EnemyAI_Parent Object Reference"))
  (set `self.ActiveTarget` NewTarget)
  (return))