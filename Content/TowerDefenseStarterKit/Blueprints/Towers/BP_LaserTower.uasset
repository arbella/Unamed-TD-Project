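; Laser tower for a tower defense game that damages its locked-on target with a beam and earns XP each attack cycle.
; Range sphere overlaps feed candidates to TurretLockOnSystem, which calls back through an interface for line-of-sight traces, recharge time, tracking and attacks.
; A single beam emitter spawned at BeginPlay is toggled with tracking rather than respawned, staying hidden with tick off when idle.
; Each attack moves the beam end to the target.
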(event `self.ReceiveBeginPlay`
  ;[0 1 0 0.5] Initialization Protocols
  (`parent.ReceiveBeginPlay`)
  (bind _returnvalue (`GameplayStatics.SpawnEmitterAtLocation` (`self.LaserBeamParticleSystem`) (`SceneComponent.K2_GetComponentLocation` (`self.Arrow`)))) ; Spawns the laser beam emitter
  (set `self.LaserBeamEmitter` _returnvalue)
  (`self.DisableLaserBeamEmitter`) ; Keeps the emitter disabled by default
)

(event `self.RangeSphere.OnComponentBeginOverlap`
  (params (OverlappedComponent :type "PrimitiveComponent Object Reference") (OtherActor :type "Actor Object Reference") (OtherComp :type "PrimitiveComponent Object Reference") (OtherBodyIndex :type Integer) (bFromSweep :type Boolean) (SweepResult :type "HitResult Structure (by ref)"))
  ;[0 1 1 0.5] If enemy units are detected, activate the lock on system
  (`/Game/TowerDefenseStarterKit/Blueprints/Towers/SupportSystems/BPC_TurretLockOnSystem.NewPotentialTargetDetected` (`self.TurretLockOnSystem`) OtherActor))

(event `self.RangeSphere.OnComponentEndOverlap`
  (params (OverlappedComponent :type "PrimitiveComponent Object Reference") (OtherActor :type "Actor Object Reference") (OtherComp :type "PrimitiveComponent Object Reference") (OtherBodyIndex :type Integer))
  ;[0 1 1 0.5] Updates the Enemy Units in range array as targets move out of range
  (`/Game/TowerDefenseStarterKit/Blueprints/Towers/SupportSystems/BPC_TurretLockOnSystem.PotentialTargetLost` (`self.TurretLockOnSystem`) OtherActor))

(event `self.DisableCoreTowerSystems`
  ;[0 1 1 0.5] Turns on/off core tower functionality
  (`/Game/TowerDefenseStarterKit/Blueprints/Towers/SupportSystems/BPC_TurretLockOnSystem.DisableLockOnSystem` (`self.TurretLockOnSystem`)))

(event `self.EnableCoreTowerSystems`
  ;[0 1 1 0.5] Turns on/off core tower functionality
  (`/Game/TowerDefenseStarterKit/Blueprints/Towers/SupportSystems/BPC_TurretLockOnSystem.EnableLockOnSystem` (`self.TurretLockOnSystem`)))

(event `EnableLaserBeamEmitter`
  ;[0 1 1 0.5] Laser Beam Emitter On/Off Controls
  (`ActorComponent.Activate` (`self.LaserBeamEmitter`) true)
  (`ParticleSystemComponent.SetBeamSourcePoint` (`self.LaserBeamEmitter`) 0 (`SceneComponent.K2_GetComponentLocation` (`self.Arrow`)) 0)
  (`ParticleSystemComponent.SetBeamEndPoint` (`self.LaserBeamEmitter`) 0 (`SceneComponent.K2_GetComponentLocation` (`self.Arrow`)))
  (`ActorComponent.SetComponentTickEnabled` (`self.LaserBeamEmitter`) true)
  (`KismetSystemLibrary.Delay` 0.0)
  (`SceneComponent.SetHiddenInGame` (`self.LaserBeamEmitter`) false false))

(event `DisableLaserBeamEmitter`
  ;[0 1 1 0.5] Laser Beam Emitter On/Off Controls
  (`ActorComponent.Deactivate` (`self.LaserBeamEmitter`))
  (`SceneComponent.SetHiddenInGame` (`self.LaserBeamEmitter`) true false)
  (`ActorComponent.SetComponentTickEnabled` (`self.LaserBeamEmitter`) false))

(event `self.ReceiveEndPlay`
  (params (EndPlayReason :type "EEndPlayReason Enum" :default "Destroyed"))
  ;[1 0 0 0.5] Destroy the laser beam emitter before executing parent end play logic
  (`/Engine/EditorBlueprintResources/StandardMacros.IsValid` (`self.LaserBeamEmitter`)
    (:`Is Valid`
      (`ActorComponent.K2_DestroyComponent` (`self.LaserBeamEmitter`)))
    (:`Is Not Valid`
      _))
  (`parent.ReceiveEndPlay` "Destroyed"))

(event `/Game/TowerDefenseStarterKit/Blueprints/Towers/SupportSystems/BPI_TurretLockOnSystem.AttackActiveTarget`
  ;[0 1 0.4 0.5] BPI_TurretLockOnSystem interface functions
  (`ParticleSystemComponent.SetBeamEndPoint` (`self.LaserBeamEmitter`) 0 (`self.K2_GetActorLocation` (`/Game/TowerDefenseStarterKit/Blueprints/Towers/SupportSystems/BPC_TurretLockOnSystem.RetrieveActiveTarget` (`self.TurretLockOnSystem`)))) ; Updates the laser beam end point based on the active target location
  (message `/Game/TowerDefenseStarterKit/Blueprints/GenericSystems/BPI_DamageApplicationSystem.ApplyDirectDamage` (`/Game/TowerDefenseStarterKit/Blueprints/Towers/SupportSystems/BPC_TurretLockOnSystem.RetrieveActiveTarget` (`self.TurretLockOnSystem`)) (`self.CalculateTrueOutputPerCycle`) (`self.CritHitChance`) (`self.CritHitDamageMultiplier`) self null)
  (`/Game/TowerDefenseStarterKit/Blueprints/Towers/SupportSystems/BPC_TowerXPManager.IncrementTowerXP` (`self.TowerXPManager`)) ; XP incremented for every output cycle
)

(event `/Game/TowerDefenseStarterKit/Blueprints/Towers/SupportSystems/BPI_TurretLockOnSystem.EnableTurretTracking`
  ;[0 1 0.4 0.5] BPI_TurretLockOnSystem interface functions
  (`self.EnableLaserBeamEmitter`))

(event `/Game/TowerDefenseStarterKit/Blueprints/Towers/SupportSystems/BPI_TurretLockOnSystem.DisableTurretTracking`
  ;[0 1 0.4 0.5] BPI_TurretLockOnSystem interface functions
  (`self.DisableLaserBeamEmitter`))

(fn `DisableLaserBeamEmitteryo`
  ;[0 1 1 0.5] Disables the emitter to reduce operational costs
  (`SceneComponent.SetHiddenInGame` (`self.LaserBeamEmitter`) true false)
  (`ActorComponent.SetComponentTickEnabled` (`self.LaserBeamEmitter`) false)
  (return))

(fn `EvaluateLoSToTarget`
  (params (Target :type "/Game/TowerDefenseStarterKit/Blueprints/AI/Enemy/BP_EnemyAI_Parent Object Reference"))
  (returns (`Success?` :type Boolean))
  (locals (Local_TargetActor :type "/Game/TowerDefenseStarterKit/Blueprints/AI/Enemy/BP_EnemyAI_Parent Object Reference"))
  ;[0 1 0.4 0.5] BPI_TurretLockOnSystem interface function - Determines if the tower has direct line of sight to the target
  (set `local.Local_TargetActor` Target)
  (bind _outhit (`KismetSystemLibrary.LineTraceSingle` (`SceneComponent.K2_GetComponentLocation` (`self.Arrow`)) (`self.K2_GetActorLocation` (`local.Local_TargetActor`)) "TraceTypeQuery1"))
  (return (== (`local.Local_TargetActor`) (`.HitActor` (`GameplayStatics.BreakHitResult` _outhit)))))

(fn `RetrieveTurretRechargeTime`
  (returns (RechargeTime :type "Float (double-precision)"))
  ;[0 1 0.4 0.5] BPI_TurretLockOnSystem interface function
  (return (`self.RechargeTime`)))

(fn `UserConstructionScript`
  (`parent.UserConstructionScript`))