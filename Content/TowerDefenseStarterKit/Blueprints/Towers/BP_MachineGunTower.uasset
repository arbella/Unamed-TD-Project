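; Machine gun tower Blueprint for a tower defense game that tracks enemies in range and fires bullet projectiles at them.
; A range sphere feeds overlaps to a TurretLockOnSystem component, which calls back through interface functions for line-of-sight traces, recharge time, tracking and attacks.
; While tracking, a looping timer turns the gun's yaw toward the active target.
; Each shot spawns a bullet with crit stats, plays a sound and adds tower XP.
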(event `self.RangeSphere.OnComponentBeginOverlap`
  (params (OverlappedComponent :type "PrimitiveComponent Object Reference") (OtherActor :type "Actor Object Reference") (OtherComp :type "PrimitiveComponent Object Reference") (OtherBodyIndex :type Integer) (bFromSweep :type Boolean) (SweepResult :type "HitResult Structure (by ref)"))
  ;[0 1 1 0.5] Store reference to overlapping targets; Initialize target acquisition
  (`/Game/TowerDefenseStarterKit/Blueprints/Towers/SupportSystems/BPC_TurretLockOnSystem.NewPotentialTargetDetected` (`self.TurretLockOnSystem`) OtherActor))

(event `self.RangeSphere.OnComponentEndOverlap`
  (params (OverlappedComponent :type "PrimitiveComponent Object Reference") (OtherActor :type "Actor Object Reference") (OtherComp :type "PrimitiveComponent Object Reference") (OtherBodyIndex :type Integer))
  ;[0 1 1 0.5] Remove stored enemy unit references based on end overlap events
  (`/Game/TowerDefenseStarterKit/Blueprints/Towers/SupportSystems/BPC_TurretLockOnSystem.PotentialTargetLost` (`self.TurretLockOnSystem`) OtherActor))

(event `self.DisableCoreTowerSystems`
  ;[0 1 1 0.5] Turns on/off core tower functionality
  (`/Game/TowerDefenseStarterKit/Blueprints/Towers/SupportSystems/BPC_TurretLockOnSystem.DisableLockOnSystem` (`self.TurretLockOnSystem`)))

(event `self.EnableCoreTowerSystems`
  ;[0 1 1 0.5] Turns on/off core tower functionality
  (`/Game/TowerDefenseStarterKit/Blueprints/Towers/SupportSystems/BPC_TurretLockOnSystem.EnableLockOnSystem` (`self.TurretLockOnSystem`)))

(event `/Game/TowerDefenseStarterKit/Blueprints/Towers/SupportSystems/BPI_TurretLockOnSystem.AttackActiveTarget`
  ;[0 1 0.4 0.5] BPI_LockOnSystem interface functions
  (`/Game/TowerDefenseStarterKit/Blueprints/Projectiles/BP_ProjectileSpawnController.CreateBulletProjectile` (`/Game/TowerDefenseStarterKit/Blueprints/FunctionLibraries/BPFL_GetterFunctions.GetProjectileSpawnController` self) (`self.CalculateTrueOutputPerCycle`) (`self.CritHitChance`) (`self.CritHitDamageMultiplier`) self (`SceneComponent.K2_GetComponentToWorld` (`self.BulletDirectionArrow`))) ; Fires a bullet projectile along the turret direction
  (`GameplayStatics.PlaySoundAtLocation` "/Game/TowerDefenseStarterKit/Audio/SW_BulletFire.SW_BulletFire" (`SceneComponent.K2_GetComponentLocation` (`self.BulletDirectionArrow`)) (struct) 1.0 1.0 0.0 null null null) ; Play firing sound
  (`/Game/TowerDefenseStarterKit/Blueprints/Towers/SupportSystems/BPC_TowerXPManager.IncrementTowerXP` (`self.TowerXPManager`)) ; XP incremented for every output cycle
)

(event `/Game/TowerDefenseStarterKit/Blueprints/Towers/SupportSystems/BPI_TurretLockOnSystem.EnableTurretTracking`
  ;[0 1 0.4 0.5] BPI_LockOnSystem interface functions
  (bind _returnvalue (`KismetSystemLibrary.K2_SetTimer` null "FocusTowerGunOnActiveTarget" 0.016667 true)) ; Starts timer to keep the turret focused on the active target
  (set `self.FocusTowerGunTimer` _returnvalue))

(event `/Game/TowerDefenseStarterKit/Blueprints/Towers/SupportSystems/BPI_TurretLockOnSystem.DisableTurretTracking`
  ;[0 1 0.4 0.5] BPI_LockOnSystem interface functions
  (`KismetSystemLibrary.K2_ClearAndInvalidateTimerHandle` (`self.FocusTowerGunTimer`)) ; Stops the timer used to focus the turret
)

(fn `EvaluateLoSToTarget`
  (params (Target :type "/Game/TowerDefenseStarterKit/Blueprints/AI/Enemy/BP_EnemyAI_Parent Object Reference"))
  (returns (`Success?` :type Boolean))
  (locals (Local_TargetActor :type "/Game/TowerDefenseStarterKit/Blueprints/AI/Enemy/BP_EnemyAI_Parent Object Reference"))
  ;[0 1 0.4 0.5] BPI_TurretLockOnSystem interface function - Determines if the tower has direct line of sight to the target
  (set `local.Local_TargetActor` Target)
  (bind _outhit (`KismetSystemLibrary.LineTraceSingle` (`SceneComponent.K2_GetComponentLocation` (`self.BulletDirectionArrow`)) (`self.K2_GetActorLocation` (`local.Local_TargetActor`)) "TraceTypeQuery1"))
  (return (== (`local.Local_TargetActor`) (`.HitActor` (`GameplayStatics.BreakHitResult` _outhit)))))

(fn `FocusTowerGunOnActiveTarget`
  ;[0 1 1 0.5] If the tower has an active target, turn the turret to face it
  (`/Engine/EditorBlueprintResources/StandardMacros.IsValid` (`/Game/TowerDefenseStarterKit/Blueprints/Towers/SupportSystems/BPC_TurretLockOnSystem.RetrieveActiveTarget` (`self.TurretLockOnSystem`))
    (:`Is Valid`
      (`SceneComponent.K2_SetWorldRotation` (`self.TowerGun`) (`KismetMathLibrary.MakeRotator` (.roll (`SceneComponent.K2_GetComponentRotation` (`self.TowerGun`))) (.pitch (`SceneComponent.K2_GetComponentRotation` (`self.TowerGun`))) (.yaw (`KismetMathLibrary.FindLookAtRotation` (`SceneComponent.K2_GetComponentLocation` (`self.TowerGun`)) (`self.K2_GetActorLocation` (`/Game/TowerDefenseStarterKit/Blueprints/Towers/SupportSystems/BPC_TurretLockOnSystem.RetrieveActiveTarget` (`self.TurretLockOnSystem`)))))) false false))))

(fn `RetrieveTurretRechargeTime`
  (returns (RechargeTime :type "Float (double-precision)"))
  ;[0 1 0.4 0.5] BPI_TurretLockOnSystem interface function
  (return (`self.RechargeTime`)))

(fn `UserConstructionScript`
  (`parent.UserConstructionScript`))