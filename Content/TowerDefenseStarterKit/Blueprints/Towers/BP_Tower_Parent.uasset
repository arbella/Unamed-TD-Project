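; Base class for tower defense towers, handling armor, damage, timed deactivation, upgrading, selling and target info display.
; Child classes implement core system enable/disable, while the parent drives the 3D stats bar for armor, level and status effects.
; Interface events attach one Overdrive or Repair ability component at a time and apply level-up boosts through an additive output multiplier.
; Death and selling share a termination path that notifies the player controller and broadcasts pending deletion.
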(event `self.ReceiveBeginPlay`
  ;[0 1 0 0.5] Initialization Protocols
  (`self.InitializeTower`) ; Initialize default parameters
)

(event `self.ReceiveEndPlay`
  (params (EndPlayReason :type "EEndPlayReason Enum" :default "Destroyed"))
  ;[1 0 0 0.5] Spawn explosion particle when destroyed
  (`GameplayStatics.SpawnEmitterAtLocation` "/Game/TowerDefenseStarterKit/Effects/Explosion/P_Explosion_Small.P_Explosion_Small" (`self.K2_GetActorLocation`)))

(event `/Game/TowerDefenseStarterKit/Blueprints/GenericSystems/BPI_DamageApplicationSystem.ApplyDirectDamage`
  (params (BaseDamage :type "Float (single-precision)") (CritChance :type "Float (single-precision)") (CritDamageMultiplier :type "Float (single-precision)") (DamagedCauser :type "Actor Object Reference") (EventInstigator :type "Controller Object Reference"))
  ;[1 0 0 0.5] Receive Damage; Destroy self if health becomes less than or equal to zero
  (`self.ModifyArmor` (* (`/Game/TowerDefenseStarterKit/Blueprints/GenericSystems/BPC_DamageCalculator.CalculateFinalDamage` (`self.DamageCalculator`) BaseDamage CritChance CritDamageMultiplier) -1.0))
  (if (not (> (`self.CurrentArmor`) 0.0))
    (`self.InitiateTerminationProtocols`)))

(event `InitiateTerminationProtocols`
  ;[1 0 0 0.5] Termination Protocols
  (message `/Game/TowerDefenseStarterKit/Blueprints/Player/BPI_TowerConstructorInteraction.TowerInteractionDisabled` (`GameplayStatics.GetPlayerController` 0) self) ; Prevents the player from interacting with this tower
  (`self.TowerPendingDeletion` self) ; Event Dispatcher called to notify all listeners about the termination event
)

(event `DeactivateTower`
  (params (ReactivationDelay :type "Float (double-precision)"))
  ;[0 1 1 0.5] Tower activation/deactivation
  (if (`self.IsFunctional?`)
    (set `self.IsFunctional?` false)
    (`self.DisableCoreTowerSystems`)
    (`KismetSystemLibrary.Delay` ReactivationDelay)
    (`self.ActivateTower`) ; Auto-reactivates the tower after a delay
  ))

(event `ActivateTower`
  ;[0 1 1 0.5] Tower activation/deactivation
  (set `self.IsFunctional?` true)
  (`self.EnableCoreTowerSystems`))

(event `/Game/TowerDefenseStarterKit/Blueprints/Towers/TowerFunctions/BPI_TowerFunctions.AddOverdriveAbilityComponent`
  (params (OverDriveBoost :type "Float (single-precision)") (Duration :type "Float (single-precision)") (AbbreviatedName :type Text) (StatusBarFillColor :type "LinearColor Structure"))
  ;[0 1 0.4 0.5] BPI_TowerFunctions interface functions
  (`/Game/TowerDefenseStarterKit/Blueprints/Towers/TowerFunctions/BPI_TowerFunctions.DestroyActiveAbilityComponent`)
  (bind _returnvalue (`AddComponent|NODE_AddBPC_Overdrive-0` :`DamageBoost` OverDriveBoost :`AbilityDuration` Duration :`AbilityNameAbbreviation` AbbreviatedName :`AbilityStatusBarFillColor` StatusBarFillColor))
  (set `self.ActiveAbilityComponent` _returnvalue))

(event `/Game/TowerDefenseStarterKit/Blueprints/Towers/TowerFunctions/BPI_TowerFunctions.AddRepairAbilityComponent`
  (params (RepairValue :type "Float (single-precision)") (Duration :type "Float (single-precision)") (AbbreviatedName :type Text) (StatusBarFillColor :type "LinearColor Structure"))
  ;[0 1 0.4 0.5] BPI_TowerFunctions interface functions
  (`/Game/TowerDefenseStarterKit/Blueprints/Towers/TowerFunctions/BPI_TowerFunctions.DestroyActiveAbilityComponent`)
  (bind _returnvalue (`AddComponent|NODE_AddBPC_RepairAbility-0` :`RepairValue` RepairValue :`AbilityDuration` Duration :`AbilityNameAbbreviation` AbbreviatedName :`AbilityStatusBarFillColor` StatusBarFillColor))
  (set `self.ActiveAbilityComponent` _returnvalue))

(event `/Game/TowerDefenseStarterKit/Blueprints/Towers/TowerFunctions/BPI_TowerFunctions.DestroyActiveAbilityComponent`
  ;[0 1 0.4 0.5] BPI_TowerFunctions interface functions
  (`/Engine/EditorBlueprintResources/StandardMacros.IsValid` (`self.ActiveAbilityComponent`)
    (:`Is Valid`
      (`ActorComponent.K2_DestroyComponent` (`self.ActiveAbilityComponent`))
      (`/Game/TowerDefenseStarterKit/UI/Generic/Widget_3DStatsBar.HideStatusEffectIcon` (`self.StatsBarWidgetRef`))
      (set `self.ActiveAbilityComponent` null))))

(event `/Game/TowerDefenseStarterKit/Blueprints/Towers/TowerFunctions/BPI_TowerFunctions.ActivateOverdriveAbility`
  (params (BoostIncrement :type "Float (single-precision)") (StatusNameAbbreviation :type Text) (StatusEffectBarFillColor :type "LinearColor Structure"))
  ;[0 1 0.4 0.5] BPI_TowerFunctions interface functions
  (`self.ModifyOutputMultiplier` BoostIncrement)
  (`/Game/TowerDefenseStarterKit/UI/Generic/Widget_3DStatsBar.InitializeStatusEffectIcon` (`self.StatsBarWidgetRef`) StatusNameAbbreviation StatusEffectBarFillColor))

(event `/Game/TowerDefenseStarterKit/Blueprints/Towers/TowerFunctions/BPI_TowerFunctions.ActivateRepairAbility`
  (params (StatusNameAbbreviation :type Text) (StatusEffectBarFillColor :type "LinearColor Structure"))
  ;[0 1 0.4 0.5] BPI_TowerFunctions interface functions
  (`/Game/TowerDefenseStarterKit/UI/Generic/Widget_3DStatsBar.InitializeStatusEffectIcon` (`self.StatsBarWidgetRef`) StatusNameAbbreviation StatusEffectBarFillColor))

(event `/Game/TowerDefenseStarterKit/Blueprints/Towers/TowerFunctions/BPI_TowerFunctions.DeactivateOverdriveAbility`
  (params (BoostDecrement :type "Float (single-precision)"))
  ;[0 1 0.4 0.5] BPI_TowerFunctions interface functions
  (`self.ModifyOutputMultiplier` BoostDecrement))

(event `/Game/TowerDefenseStarterKit/Blueprints/Towers/TowerFunctions/BPI_TowerFunctions.DeactivateRepairAbility`
  ;[0 1 0.4 0.5] BPI_TowerFunctions interface functions
)

(event `/Game/TowerDefenseStarterKit/Blueprints/Towers/TowerFunctions/BPI_TowerFunctions.UpdateAbilityStatusDisplay`
  (params (StatusDurationBarPercent :type "Float (single-precision)"))
  ;[0 1 0.4 0.5] BPI_TowerFunctions interface functions
  (`/Game/TowerDefenseStarterKit/UI/Generic/Widget_3DStatsBar.UpdateStatusEffectIcon` (`self.StatsBarWidgetRef`) StatusDurationBarPercent))

(event `/Game/TowerDefenseStarterKit/Blueprints/Towers/TowerFunctions/BPI_TowerFunctions.RepairArmor`
  (params (ArmorIncrement :type "Float (single-precision)"))
  ;[0 1 0.4 0.5] BPI_TowerFunctions interface functions
  (if (< (`self.CurrentArmor`) (`self.MaxArmor`))
    (`self.ModifyArmor` ArmorIncrement)))

(event `/Game/TowerDefenseStarterKit/Blueprints/Towers/SupportSystems/BPI_TowerLevelUpSystem.TowerSkillLevelUpgraded`
  (params (NewLevel :type Integer) (LevelUpStatModifiers :type "/Game/TowerDefenseStarterKit/Blueprints/Towers/SupportSystems/Struct_TowerLevelUpStatModifiers Structure"))
  ;[0 1 0.4 0.5] BPI_TowerLevelUpSystem interface functions
  (`/Game/TowerDefenseStarterKit/UI/Generic/Widget_3DStatsBar.UpdateLevelDisplayText` (`self.StatsBarWidgetRef`) (`KismetTextLibrary.Conv_IntToText` NewLevel)) ; Displays the new tower level through the dedicated UI element
  (`self.ModifyOutputMultiplier` (`.LevelUpModifier_OutputPerCycle_6_2183FCEA4F8EDFD68E23838798A7DAF5` (break `/Game/TowerDefenseStarterKit/Blueprints/Towers/SupportSystems/Struct_TowerLevelUpStatModifiers` LevelUpStatModifiers))) ; Enhances the Output Per Cycle when Tower Level increases
)

(event `/Game/TowerDefenseStarterKit/Blueprints/Towers/SupportSystems/BPI_TowerLevelUpSystem.TowerLevelUpSystemInitialized`
  ;[0 1 0.4 0.5] BPI_TowerLevelUpSystem interface functions
  (bind _aswidget_3dstats_bar (cast `/Game/TowerDefenseStarterKit/UI/Generic/Widget_3DStatsBar` (`WidgetComponent.GetUserWidgetObject` (`self.3DStatsBar`))))
  (`/Game/TowerDefenseStarterKit/UI/Generic/Widget_3DStatsBar.InitializeLevelDisplayUIElements` _aswidget_3dstats_bar) ; Initializes the UI icon for displaying tower level
)

(fn `CalculateTrueOutputPerCycle`
  (returns (Value :type "Float (double-precision)"))
  ;[0 1 1 0.5] Calculates the output multiplier adjusted value of tower output per cycle
  (return (* (`self.OutputPerCycle`) (`self.OutputMultiplier`))))

(fn `DisableCoreTowerSystems`
  ;[0 1 1 0.5] Implemented through child classes
  (return))

(fn `EnableCoreTowerSystems`
  ;[0 1 1 0.5] Implemented through child classes
  (return))

(fn `GetGridData`
  (returns (GridCellIndex :type Integer) (GridGeneratorIndex :type Integer))
  ;[0 1 1 0.5] Retrieves Grid Cell & Generator index for the tower
  (return (`self.GridCellIndex`) (`self.GridGeneratorIndex`)))

(fn `InitializeTower`
  ;[0 1 1 0.5] Initialize default Tower parameters
  (bind _aswidget_3dstats_bar (cast `/Game/TowerDefenseStarterKit/UI/Generic/Widget_3DStatsBar` (`WidgetComponent.GetUserWidgetObject` (`self.3DStatsBar`))))
  (bind _output_get (set `self.StatsBarWidgetRef` _aswidget_3dstats_bar))
  (`/Game/TowerDefenseStarterKit/UI/Generic/Widget_3DStatsBar.InitializeHealthBar` _output_get (struct :`G` 1.0 :`A` 1.0) 1.0)
  (set `self.CurrentArmor` (`self.MaxArmor`))
  (`SphereComponent.SetSphereRadius` (`self.RangeSphere`) (`self.Range`) true))

(fn `ModifyArmor`
  (params (By :type "Float (double-precision)"))
  (bind _statsbarwidgetref (`self.StatsBarWidgetRef`))
  ;[0 1 1 0.5] Updates Armor & relays the information to Game HUD
  (set `self.CurrentArmor` (`KismetMathLibrary.FClamp` (+ (`self.CurrentArmor`) By) 0.0 (`self.MaxArmor`)))
  (`/Engine/EditorBlueprintResources/StandardMacros.IsValid` _statsbarwidgetref
    (:`Is Valid`
      (`/Game/TowerDefenseStarterKit/UI/Generic/Widget_3DStatsBar.UpdateHealthBar` _statsbarwidgetref (/ (`self.CurrentArmor`) (`self.MaxArmor`))))
    (:`Is Not Valid`
      _))
  (return))

(fn `ModifyOutputMultiplier`
  (params (By :type "Float (double-precision)"))
  (locals (Local_OutputPerCycle :type "Float (double-precision)"))
  ;[0 1 1 0.5] Modifies the Output Multiplier by the specified amount; Output Multipliers are then applied on a per instance basis to the base Output Per Cycle whenever the tower generates output
  (set `self.OutputMultiplier` (+ (`self.OutputMultiplier`) By)) ; Update Boost value
  (return))

(fn `RetrieveTargetInfo`
  (returns (Name :type Text) (Description :type Text) (Stats :type "Array of /Game/TowerDefenseStarterKit/Blueprints/HUDControl/Struct_HUDStats Structure"))
  ;[0 1 0.4 0.5] BPI_TargetInfoDisplay interface function
  (return (`self.TowerName`) (`self.ShortDescription`) (`|MakeArray` (make `/Game/TowerDefenseStarterKit/Blueprints/HUDControl/Struct_HUDStats` (`self.UIStatName_CoreFunction`) (`KismetTextLibrary.Conv_DoubleToText` (/ (`self.OutputPerCycle`) (`self.RechargeTime`)) "HalfToEven")) (make `/Game/TowerDefenseStarterKit/Blueprints/HUDControl/Struct_HUDStats` (`self.UIStatName_Defense`) (`KismetTextLibrary.Conv_IntToText` (`KismetMathLibrary.Round` (`self.MaxArmor`)))) (make `/Game/TowerDefenseStarterKit/Blueprints/HUDControl/Struct_HUDStats` (`self.UIStatName_LimitingFactor`) (`KismetTextLibrary.Conv_IntToText` (`KismetMathLibrary.Round` (`self.Range`)))))))

(fn `RetrieveTraceHitGridData`
  (params (TraceHitLocation :type "Vector Structure"))
  (returns (GridCellIndex :type Integer) (GridGeneratorIndex :type Integer))
  (bind (_gridcellindex _gridgeneratorindex) (`self.GetGridData`))
  ;[0 1 0.4 0.5] 'BPI_GridLink' interface function used to retrieve grid data of the implementing actor
  (return _gridcellindex _gridgeneratorindex))

(fn `SellTower`
  (`self.InitiateTerminationProtocols`))

(fn `UpgradeTower`
  (params (TowerModel :type "/Game/TowerDefenseStarterKit/Blueprints/Towers/ETowerModels Enum" :default "NewEnumerator2") (OutputPerCycle :type "Float (double-precision)") (RechargeTime :type "Float (double-precision)") (MaxArmor :type "Float (double-precision)") (Range :type "Float (double-precision)") (ResourceCap :type "Float (double-precision)") (TowerMesh :type "StaticMesh Object Reference") (TowerName :type Text) (ShortDescription :type Text))
  ;[0 1 1 0.5] Upgrades the Tower
  (set `self.TowerModel` TowerModel)
  (set `self.OutputPerCycle` OutputPerCycle) ; Set Upgraded  Output per cycle
  (set `self.RechargeTime` RechargeTime)
  (bind _output_get (set `self.MaxArmor` MaxArmor)) ; Set Upgraded Max Armor
  (set `self.CurrentArmor` _output_get) ; Set Upgraded Armor
  (set `self.Range` Range) ; Set upgraded range
  (set `self.ResourcesLeft` ResourceCap) ; Set Upgraded Resource Cap
  (`StaticMeshComponent.SetStaticMesh` (`self.Tower`) TowerMesh)
  (set `self.TowerName` TowerName)
  (set `self.ShortDescription` ShortDescription)
  (`SphereComponent.SetSphereRadius` (`self.RangeSphere`) (`self.Range`) true)
  (return))

(fn `UserConstructionScript`)