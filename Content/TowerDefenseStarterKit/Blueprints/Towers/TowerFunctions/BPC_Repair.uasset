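; Actor component that applies a timed Repair ability to its owning tower, gradually restoring Armor.
; After a zero-delay workaround for expose-on-spawn variables, BeginPlay verifies BPI_TowerFunctions, derives armor per tick and starts a looping timer.
; Each tick sends armor and status-bar updates to the owner through messages, then requests the component's destruction once time expires.
; EndPlay clears the timer and tells the owner to deactivate the ability.
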(event `self.ReceiveBeginPlay`
  ;[0 1 1 0.5] Activates Repair ability for the owning actor & starts timer to update the ability status icon
  (`KismetSystemLibrary.Delay` 0.0) ; Fix for components in UE4 failing to set variables exposed on spawn at Event Begin Play
  (if (`KismetSystemLibrary.DoesImplementInterface` (`self.GetOwner`) "/Game/TowerDefenseStarterKit/Blueprints/Towers/TowerFunctions/BPI_TowerFunctions.BPI_TowerFunctions_C")
    (set `self.ArmorIncrementPerCycle` (* (/ (`self.RepairValue`) (`self.AbilityDuration`)) (`self.RepairTowerArmorTimerInterval`)))
    (message `/Game/TowerDefenseStarterKit/Blueprints/Towers/TowerFunctions/BPI_TowerFunctions.ActivateRepairAbility` (`self.GetOwner`) (`self.AbilityNameAbbreviation`) (`self.AbilityStatusBarFillColor`))
    (set `self.RemainingTime` (`self.AbilityDuration`))
    (bind _returnvalue (`KismetSystemLibrary.K2_SetTimer` self "RepairTowerArmor" (`self.RepairTowerArmorTimerInterval`) true))
    (set `self.RepairTowerArmorTimer` _returnvalue)))

(event `self.ReceiveEndPlay`
  (params (EndPlayReason :type "EEndPlayReason Enum" :default "Destroyed"))
  (bind _repairtowerarmortimer (`self.RepairTowerArmorTimer`))
  ;[0 1 1 0.5] Handles pre termination protocols before the component gets destroyed
  (if (`KismetSystemLibrary.K2_TimerExistsHandle` _repairtowerarmortimer)
    (`KismetSystemLibrary.K2_ClearAndInvalidateTimerHandle` _repairtowerarmortimer))
  (message `/Game/TowerDefenseStarterKit/Blueprints/Towers/TowerFunctions/BPI_TowerFunctions.DeactivateRepairAbility` (`self.GetOwner`)) ; Request the owning actor to handle ability pre termination protocols before destroying the component
)

(fn `RepairTowerArmor`
  (bind _returnvalue (`self.GetOwner`))
  ;[0 1 1 0.5] Increased the Armor & updates the Repair Ability status icon on the parent actor, or destroy self based on ability duration checks
  (bind _output_get (set `self.RemainingTime` (- (`self.RemainingTime`) (`self.RepairTowerArmorTimerInterval`)))) ; Update the remaining time during every timer loop based on the timer interval
  (if (> _output_get 0.0)
    (message `/Game/TowerDefenseStarterKit/Blueprints/Towers/TowerFunctions/BPI_TowerFunctions.RepairArmor` _returnvalue (`self.ArmorIncrementPerCycle`)) ; Increase the Armor attribute of the owning actor
    (message `/Game/TowerDefenseStarterKit/Blueprints/Towers/TowerFunctions/BPI_TowerFunctions.UpdateAbilityStatusDisplay` _returnvalue (/ (`self.RemainingTime`) (`self.AbilityDuration`))) ; Updates the Repair Ability status icon on the owning actor
    (else
      (message `/Game/TowerDefenseStarterKit/Blueprints/Towers/TowerFunctions/BPI_TowerFunctions.DestroyActiveAbilityComponent` _returnvalue))))