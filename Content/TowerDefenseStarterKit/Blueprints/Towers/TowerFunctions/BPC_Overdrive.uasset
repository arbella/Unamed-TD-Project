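; Actor component that applies a timed Overdrive damage boost to its owning tower through the BPI_TowerFunctions interface.
; After a zero-delay fix for expose-on-spawn variables, it sends the boost, status name and bar color to the owner and starts a looping timer.
; The timer updates the owner's status display with remaining time, then asks it to destroy the component on expiry.
; EndPlay clears the timer and reverses the boost.
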(event `self.ReceiveBeginPlay`
  ;[0 1 1 0.5] Activates Overdrive ability for the owning actor & starts timer to update the ability status icon
  (`KismetSystemLibrary.Delay` 0.0) ; Fix for components in UE4 failing to set variables exposed on spawn at Event Begin Play
  (if (`KismetSystemLibrary.DoesImplementInterface` (`self.GetOwner`) "/Game/TowerDefenseStarterKit/Blueprints/Towers/TowerFunctions/BPI_TowerFunctions.BPI_TowerFunctions_C")
    (message `/Game/TowerDefenseStarterKit/Blueprints/Towers/TowerFunctions/BPI_TowerFunctions.ActivateOverdriveAbility` (`self.GetOwner`) (`self.DamageBoost`) (`self.AbilityNameAbbreviation`) (`self.AbilityStatusBarFillColor`))
    (set `self.RemainingTime` (`self.AbilityDuration`))
    (bind _returnvalue (`KismetSystemLibrary.K2_SetTimer` null "UpdateAbilityDurationDisplay" (`self.AbilityDurationDisplayUpdateTimerInterval`) true))
    (set `self.AbilityDurationDisplayUpdateTimer` _returnvalue)
    (else
      (`KismetSystemLibrary.PrintString` "WARNING: Owner does not meet interface requirements; Class: BPC_OverdriveAbility"))))

(event `self.ReceiveEndPlay`
  (params (EndPlayReason :type "EEndPlayReason Enum" :default "Destroyed"))
  (bind _abilitydurationdisplayupdatetimer (`self.AbilityDurationDisplayUpdateTimer`))
  ;[0 1 1 0.5] Handles pre termination protocols before the component gets destroyed
  (if (`KismetSystemLibrary.K2_TimerExistsHandle` _abilitydurationdisplayupdatetimer)
    (`KismetSystemLibrary.K2_ClearAndInvalidateTimerHandle` _abilitydurationdisplayupdatetimer))
  (message `/Game/TowerDefenseStarterKit/Blueprints/Towers/TowerFunctions/BPI_TowerFunctions.DeactivateOverdriveAbility` (`self.GetOwner`) (* (`self.DamageBoost`) -1.0)) ; Request the owning actor to handle ability pre termination protocols before destroying the component
)

(fn `UpdateAbilityDurationDisplay`
  (bind _returnvalue (`self.GetOwner`))
  ;[0 1 1 0.5] Updates the Overdrive Ability status icon on the parent actor or destroy self based on ability duration checks
  (bind _output_get (set `self.RemainingTime` (- (`self.RemainingTime`) (`self.AbilityDurationDisplayUpdateTimerInterval`)))) ; Update the remaining time during every timer loop based on the timer interval
  (if (> _output_get 0.0)
    (message `/Game/TowerDefenseStarterKit/Blueprints/Towers/TowerFunctions/BPI_TowerFunctions.UpdateAbilityStatusDisplay` _returnvalue (/ (`self.RemainingTime`) (`self.AbilityDuration`))) ; Updates the Overdrive Ability status icon on the owning actor
    (else
      (message `/Game/TowerDefenseStarterKit/Blueprints/Towers/TowerFunctions/BPI_TowerFunctions.DestroyActiveAbilityComponent` _returnvalue))))