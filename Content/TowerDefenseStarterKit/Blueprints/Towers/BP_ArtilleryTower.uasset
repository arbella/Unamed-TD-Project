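; Artillery tower that lobs arcing projectiles at enemies and earns XP per shot.
; Range sphere overlaps feed TurretLockOnSystem, which calls back through interface functions to validate targets and fire.
; The line-of-sight check solves a ballistic velocity by fixed launch angle (height-limited) or fixed impact time, then traces launcher-to-apex and apex-to-target.
; Firing spawns shells through the projectile spawn controller using that stored velocity with a random offset.
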(event `self.ReceiveBeginPlay`
  ;[0 1 1 0.5] Execute Parent Begin Play Logic
  (`parent.ReceiveBeginPlay`)
  (set `self.GravitationalAccelerationMagnitude` (`KismetMathLibrary.VSize` (`self.GravitationalAccelerationVector`))))

(event `self.RangeSphere.OnComponentBeginOverlap`
  (params (OverlappedComponent :type "PrimitiveComponent Object Reference") (OtherActor :type "Actor Object Reference") (OtherComp :type "PrimitiveComponent Object Reference") (OtherBodyIndex :type Integer) (bFromSweep :type Boolean) (SweepResult :type "HitResult Structure (by ref)"))
  ;[0 1 1 0.5] Store reference to overlapping targets; Initialize target acquisition
  (`/Game/TowerDefenseStarterKit/Blueprints/Towers/SupportSystems/BPC_TurretLockOnSystem.NewPotentialTargetDetected` (`self.TurretLockOnSystem`) OtherActor))

(event `self.RangeSphere.OnComponentEndOverlap`
  (params (OverlappedComponent :type "PrimitiveComponent Object Reference") (OtherActor :type "Actor Object Reference") (OtherComp :type "PrimitiveComponent Object Reference") (OtherBodyIndex :type Integer))
  ;[0 1 1 0.5] Remove stored enemy unit references based on end overlap events
  (`/Game/TowerDefenseStarterKit/Blueprints/Towers/SupportSystems/BPC_TurretLockOnSystem.PotentialTargetLost` (`self.TurretLockOnSystem`) OtherActor))

(event `self.DisableCoreTowerSystems`
  ;[0 1 1 0.5] Turns on/off core tower functionality
  (`/Game/TowerDefenseStarterKit/Blueprints/Towers/SupportSystems/BPC_TurretLockOnSystem.DisableLockOnSystem` (`self.TurretLockOnSystem`)))

(event `self.EnableCoreTowerSystems`
  ;[0 1 1 0.5] Turns on/off core tower functionality
  (`/Game/TowerDefenseStarterKit/Blueprints/Towers/SupportSystems/BPC_TurretLockOnSystem.EnableLockOnSystem` (`self.TurretLockOnSystem`)))

(event `/Game/TowerDefenseStarterKit/Blueprints/Towers/SupportSystems/BPI_TurretLockOnSystem.AttackActiveTarget`
  ;[0 1 0.4 0.5] BPI_LockOnSystem interface functions
  (`self.FireArtilleryShellsAtTargetLocation`)
  (`/Game/TowerDefenseStarterKit/Blueprints/Towers/SupportSystems/BPC_TowerXPManager.IncrementTowerXP` (`self.TowerXPManager`)) ; XP incremented for every output cycle
)

(event `/Game/TowerDefenseStarterKit/Blueprints/Towers/SupportSystems/BPI_TurretLockOnSystem.EnableTurretTracking`
  ;[0 1 0.4 0.5] BPI_LockOnSystem interface functions
)

(event `/Game/TowerDefenseStarterKit/Blueprints/Towers/SupportSystems/BPI_TurretLockOnSystem.DisableTurretTracking`
  ;[0 1 0.4 0.5] BPI_LockOnSystem interface functions
)

(fn `EvaluateLoSToTarget`
  (params (Target :type "/Game/TowerDefenseStarterKit/Blueprints/AI/Enemy/BP_EnemyAI_Parent Object Reference"))
  (returns (`Success?` :type Boolean))
  (locals (Local_TargetActor :type "/Game/TowerDefenseStarterKit/Blueprints/AI/Enemy/BP_EnemyAI_Parent Object Reference"))
  ;[0 1 0.4 0.5] BPI_TurretLockOnSystem interface function - Calculates a artillery projectile path toward the target & does a basic double line trace check if the path is free of obstacles
  (bind _output_get (set `local.Local_TargetActor` Target))
  (bind (_initialprojectilevelocity _maxheightlocation _success_) (`self.GetProjectilePathParametersForTarget` _output_get)) ; Calculate projectile path towards the target
  (if _success_
    (set `self.InitialProjectileVelocity` _initialprojectilevelocity)
    (bind (_outhit _returnvalue) (`KismetSystemLibrary.LineTraceSingle` (`SceneComponent.K2_GetComponentLocation` (`self.LaunchPlatform`)) _maxheightlocation "TraceTypeQuery1")) ; Line trace from launch platform to the highest position along the path
    (if _returnvalue
      (return false) ; Obstacle detected; No direct paths
      (else
        (bind _outhit_2 (`KismetSystemLibrary.LineTraceSingle` _maxheightlocation (`self.K2_GetActorLocation` (`local.Local_TargetActor`)) "TraceTypeQuery1")) ; Line trace from the highest position along the path to the target
        (return (`.bSuccess` (cast `/Game/TowerDefenseStarterKit/Blueprints/AI/Enemy/BP_EnemyAI_Parent` (`.HitActor` (`GameplayStatics.BreakHitResult` _outhit_2)) :!pure true)))))
    (else
      (return false))))

(fn `FireArtilleryShellsAtTargetLocation`
  (bind _velocityoffsetrange (`self.VelocityOffsetRange`))
  (bind _x (.x (`self.InitialProjectileVelocity`)))
  (bind _y (.y (`self.InitialProjectileVelocity`)))
  ;[0 1 1 0.5] Fire projectiles & set the initial velocities based on the results from earlier calculations
  (`/Game/TowerDefenseStarterKit/Blueprints/Projectiles/BP_ProjectileSpawnController.CreateArtilleryProjectile` (`/Game/TowerDefenseStarterKit/Blueprints/FunctionLibraries/BPFL_GetterFunctions.GetProjectileSpawnController` self) (`KismetMathLibrary.MakeTransform` (.location (`SceneComponent.K2_GetComponentToWorld` (`self.LaunchPlatform`))) (.rotation (`SceneComponent.K2_GetComponentToWorld` (`self.LaunchPlatform`)))) (`self.CalculateTrueOutputPerCycle`) (`self.CritHitChance`) (`self.CritHitDamageMultiplier`) self (`KismetMathLibrary.MakeVector` (`KismetMathLibrary.RandomFloatInRange` (- _x _velocityoffsetrange) (+ _x _velocityoffsetrange)) (`KismetMathLibrary.RandomFloatInRange` (- _y _velocityoffsetrange) (+ _y _velocityoffsetrange)) (.z (`self.InitialProjectileVelocity`))))
  (`GameplayStatics.PlaySoundAtLocation` "/Game/TowerDefenseStarterKit/Audio/SW_BulletFire.SW_BulletFire" (`SceneComponent.K2_GetComponentLocation` (`self.LaunchPlatform`)) (struct) 1.0 1.0 0.0 null null null) ; Play firing sound
)

(fn `GetProjectilePathParametersForTarget`
  (params (Target :type "/Game/TowerDefenseStarterKit/Blueprints/AI/Enemy/BP_EnemyAI_Parent Object Reference"))
  (returns (InitialProjectileVelocity :type "Vector Structure") (MaxHeightLocation :type "Vector Structure") (`Success?` :type Boolean))
  (locals (Local_Target :type "/Game/TowerDefenseStarterKit/Blueprints/AI/Enemy/BP_EnemyAI_Parent Object Reference") (Local_InitialForwardVelocity :type "Vector Structure") (Local_InitialUpwardVelocity :type "Vector Structure") (Local_TimeAtHighestPosition :type "Float (double-precision)") (Local_InitialProjectileVelocity :type "Vector Structure") (Local_MaxHeightLocation :type "Vector Structure") (Local_InitialVelocityMagnitude :type "Float (double-precision)" :default 0.0) (Local_MaxHeight :type "Float (double-precision)" :default 0.0) (Local_TotalHorizontalDisplacement :type "Vector Structure") (Local_TotalVerticalDisplacement :type "Vector Structure"))
  (bind _local_timeathighestposition (`local.Local_TimeAtHighestPosition`))
  (bind _returnvalue (`KismetMathLibrary.VSize` (`local.Local_TotalHorizontalDisplacement`)))
  (bind _returnvalue_2 (`KismetMathLibrary.Normal` (`local.Local_TotalHorizontalDisplacement`)))
  ;[0 1 1 0.5] Calculate projectile path parameters based on the given constraints
  (set `local.Local_Target` Target)
  (if (>= (`self.GetDistanceTo` (`local.Local_Target`)) (`self.MinimumTargetDistance`))
    (switch `/Game/TowerDefenseStarterKit/Blueprints/Towers/EProjectilePathConstraints` (`self.ProjectilePathConstraints`)
      (:`NewEnumerator1`
        (set `local.Local_TotalHorizontalDisplacement` (`KismetMathLibrary.MakeVector` (- (.x (`SceneComponent.K2_GetComponentLocation` (`Character.Mesh` (`local.Local_Target`)))) (.x (`SceneComponent.K2_GetComponentLocation` (`self.LaunchPlatform`)))) (- (.y (`SceneComponent.K2_GetComponentLocation` (`Character.Mesh` (`local.Local_Target`)))) (.y (`SceneComponent.K2_GetComponentLocation` (`self.LaunchPlatform`))))))
        (set `local.Local_TotalVerticalDisplacement` (`KismetMathLibrary.MakeVector` 0.0 0.0 (- (.z (`SceneComponent.K2_GetComponentLocation` (`Character.Mesh` (`local.Local_Target`)))) (.z (`SceneComponent.K2_GetComponentLocation` (`self.LaunchPlatform`))))))
        (set `local.Local_InitialVelocityMagnitude` (/ (* _returnvalue (`KismetMathLibrary.MultiplyMultiply_FloatFloat` (`KismetMathLibrary.Abs` (/ (`self.GravitationalAccelerationMagnitude`) (* (- (.z (`local.Local_TotalVerticalDisplacement`)) (* _returnvalue (`KismetMathLibrary.DegTan` (`self.LaunchAngle`)))) 2.0))) 0.5)) (`KismetMathLibrary.DegCos` (`self.LaunchAngle`))))
        (set `local.Local_MaxHeight` (/ (`KismetMathLibrary.MultiplyMultiply_FloatFloat` (* (`local.Local_InitialVelocityMagnitude`) (`KismetMathLibrary.DegSin` (`self.LaunchAngle`))) 2.0) (* (`self.GravitationalAccelerationMagnitude`) 2.0)))
        (if (`KismetMathLibrary.InRange_FloatFloat` (`local.Local_MaxHeight`) (`self.MinProjectileHeight`) (`self.MaxProjectileHeight`))
          (bind _output_get (set `local.Local_InitialProjectileVelocity` (* (`KismetMathLibrary.Normal` (`KismetMathLibrary.RotateAngleAxis` _returnvalue_2 (`self.LaunchAngle`) (* (`KismetMathLibrary.GetRightVector` (`KismetMathLibrary.Conv_VectorToRotator` _returnvalue_2)) -1.0))) (`local.Local_InitialVelocityMagnitude`))))
          (set `local.Local_InitialForwardVelocity` (`KismetMathLibrary.MakeVector` (.x _output_get) (.y _output_get)))
          (set `local.Local_InitialUpwardVelocity` (`KismetMathLibrary.MakeVector` 0.0 0.0 (.z _output_get)))
          (else
            (return (`local.Local_InitialProjectileVelocity`) (`local.Local_MaxHeightLocation`) false) ; Path doesn't meet height requirements; Cancel current iteration
          )))
      (:`NewEnumerator0`
        (bind _output_get_2 (set `local.Local_InitialProjectileVelocity` (- (/ (- (`SceneComponent.K2_GetComponentLocation` (`Character.Mesh` (`local.Local_Target`))) (`SceneComponent.K2_GetComponentLocation` (`self.LaunchPlatform`))) (`self.TimeToImpact`)) (* (`self.GravitationalAccelerationVector`) (* (`self.TimeToImpact`) 0.5))))) ; v = s/t - 0.5at
        (set `local.Local_InitialForwardVelocity` (`KismetMathLibrary.MakeVector` (.x _output_get_2) (.y _output_get_2)))
        (set `local.Local_InitialUpwardVelocity` (`KismetMathLibrary.MakeVector` 0.0 0.0 (.z _output_get_2)))
        (set `local.Local_TimeAtHighestPosition` (/ (`KismetMathLibrary.VSize` (`local.Local_InitialUpwardVelocity`)) (`self.GravitationalAccelerationMagnitude`))) ; t at H
      ))
    (set `local.Local_MaxHeightLocation` (`KismetMathLibrary.MakeVector` (+ (.x (`SceneComponent.K2_GetComponentLocation` (`self.LaunchPlatform`))) (.x (* (`local.Local_InitialForwardVelocity`) _local_timeathighestposition))) (+ (.y (`SceneComponent.K2_GetComponentLocation` (`self.LaunchPlatform`))) (.y (* (`local.Local_InitialForwardVelocity`) _local_timeathighestposition))) (+ (.z (`SceneComponent.K2_GetComponentLocation` (`self.LaunchPlatform`))) (- (* (`KismetMathLibrary.VSize` (`local.Local_InitialUpwardVelocity`)) _local_timeathighestposition) (* 0.5 (`self.GravitationalAccelerationMagnitude`) (`KismetMathLibrary.MultiplyMultiply_FloatFloat` (`local.Local_TimeAtHighestPosition`) 2.0))))))
    (return (`local.Local_InitialProjectileVelocity`) (`local.Local_MaxHeightLocation`) true)
    (else
      (return (0.0 0.0 0.0) (0.0 0.0 0.0) false))))

(fn `RetrieveTurretRechargeTime`
  (returns (RechargeTime :type "Float (double-precision)"))
  ;[0 1 0.4 0.5] BPI_TurretLockOnSystem interface function
  (return (`self.RechargeTime`)))

(fn `UserConstructionScript`
  (`parent.UserConstructionScript`))