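; BP_TowerConstructor is the tower defense helper actor that shows the tower interaction UI and range display at a grid cell.
; It initializes a Widget_TowerInteraction component widget, then switches it between creation and control modes, moving itself via UpdateTransform.
; The range display scales by requested range over a default radius measured from its local bounds at initialization.
; Separate events refresh the UI or hide both modules.
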(event `Initialize`
  (params (NumberOfTowerModels :type Integer) (NumberOfTowerFunctions :type Integer))
  (bind (_min _max) (`StaticMeshComponent.GetLocalBounds` (`self.TowerRangeDisplay`)))
  ;[0 1 0 0.5] Initialization Protocols
  (set `self.DefaultRange` (.x (/ (- _max _min) 2.0)))
  (bind _aswidget_tower_interaction (cast `/Game/TowerDefenseStarterKit/UI/TowerConstructor/Widget_TowerInteraction` (`WidgetComponent.GetUserWidgetObject` (`self.TowerInteractionUI`))))
  (`/Game/TowerDefenseStarterKit/UI/TowerConstructor/Widget_TowerInteraction.Initialize` _aswidget_tower_interaction NumberOfTowerModels NumberOfTowerFunctions))

(event `ActivateTowerRangeDisplay`
  (params (Range :type "Float (double-precision)"))
  ;[0 1 1 0.5] Tower Range Display Control
  (`self.UpdateRangeDisplayScale` Range)
  (`SceneComponent.SetHiddenInGame` (`self.TowerRangeDisplay`) false false))

(event `UpdateRangeDisplayScale`
  (params (NewRange :type "Float (double-precision)"))
  ;[0 1 1 0.5] Tower Range Display Control
  (`SceneComponent.SetWorldScale3D` (`self.TowerRangeDisplay`) (`KismetMathLibrary.Conv_DoubleToVector` (/ NewRange (`self.DefaultRange`)))))

(event `DeactivateTowerRangeDisplay`
  ;[0 1 1 0.5] Tower Range Display Control
  (`SceneComponent.SetHiddenInGame` (`self.TowerRangeDisplay`) true false)
  (`self.UpdateRangeDisplayScale` 0.0))

(event `ActivateTowerCreationUI`
  (params (TowerMapData :type "Map of /Game/TowerDefenseStarterKit/Blueprints/Towers/ETowerModels Enum to DataTableRowHandle Structure" :default _) (SelectedTowerModels :type "Array of /Game/TowerDefenseStarterKit/Blueprints/Towers/ETowerModels Enum (by ref)" :default _) (GridCellIndex :type Integer) (GridGeneratorIndex :type Integer))
  ;[0 1 1 0.5] Tower Interaction UI Control
  (bind _aswidget_tower_interaction (cast `/Game/TowerDefenseStarterKit/UI/TowerConstructor/Widget_TowerInteraction` (`WidgetComponent.GetUserWidgetObject` (`self.TowerInteractionUI`))))
  (`/Game/TowerDefenseStarterKit/UI/TowerConstructor/Widget_TowerInteraction.DisplayTowerCreationUI` _aswidget_tower_interaction TowerMapData SelectedTowerModels)
  (`self.UpdateTransform` GridCellIndex GridGeneratorIndex)
  (`SceneComponent.SetHiddenInGame` (`self.TowerInteractionUI`) false false :!label _label))

(event `DeactivateTowerInteractionUI`
  ;[0 1 1 0.5] Tower Interaction UI Control
  (`SceneComponent.SetHiddenInGame` (`self.TowerInteractionUI`) true false))

(event `ActivateTowerControlUI`
  (params (TowerMapData :type "Map of /Game/TowerDefenseStarterKit/Blueprints/Towers/ETowerModels Enum to DataTableRowHandle Structure" :default _) (TowerModel :type "/Game/TowerDefenseStarterKit/Blueprints/Towers/ETowerModels Enum" :default "NewEnumerator2") (AvailableTowerFunctions :type "Array of /Game/TowerDefenseStarterKit/Blueprints/Towers/TowerFunctions/ETowerFunctions Enum (by ref)" :default _) (TowerFunctionsMapData :type "Map of /Game/TowerDefenseStarterKit/Blueprints/Towers/TowerFunctions/ETowerFunctions Enum to DataTableRowHandle Structure" :default _) (GridCellIndex :type Integer) (GridGeneratorindex :type Integer))
  ;[0 1 1 0.5] Tower Interaction UI Control
  (bind _aswidget_tower_interaction (cast `/Game/TowerDefenseStarterKit/UI/TowerConstructor/Widget_TowerInteraction` (`WidgetComponent.GetUserWidgetObject` (`self.TowerInteractionUI`))))
  (`/Game/TowerDefenseStarterKit/UI/TowerConstructor/Widget_TowerInteraction.DisplayTowerControlUI` _aswidget_tower_interaction TowerMapData TowerModel AvailableTowerFunctions TowerFunctionsMapData)
  (`self.UpdateTransform` GridCellIndex GridGeneratorindex)
  (goto _label))

(event `RefreshTowerInteractionUI`
  ;[0 1 1 0.5] Tower Interaction UI Control
  (bind _aswidget_tower_interaction (cast `/Game/TowerDefenseStarterKit/UI/TowerConstructor/Widget_TowerInteraction` (`WidgetComponent.GetUserWidgetObject` (`self.TowerInteractionUI`))))
  (`/Game/TowerDefenseStarterKit/UI/TowerConstructor/Widget_TowerInteraction.RefreshWidgetState` _aswidget_tower_interaction))

(event `DeactivateAllModules`
  ;[1 0 0 0.5] Deactivation Logic
  (`self.DeactivateTowerInteractionUI`)
  (`self.DeactivateTowerRangeDisplay`))

(fn `UpdateTransform`
  (params (GridCellIndex :type Integer) (GridGeneratorindex :type Integer))
  (bind ((`GridGeneratorData_11_13E757544C1E18F1261E9C9C7CA2FC04` _gridgeneratordata) (`GridGenerator_13_116FE1614615A5B5C63B70B45CFF220B` _gridgenerator)) (break `/Game/TowerDefenseStarterKit/Blueprints/GridSystems/Struct_GridData` (`|GetArrayItem` (`/Game/TowerDefenseStarterKit/Blueprints/FunctionLibraries/BPFL_GetterFunctions.GetGridDataArray` self) GridGeneratorindex)))
  ;[0 1 1 0.5] Version 2.5: Updates actor transform based on the specified grid cell
  (`self.K2_SetActorTransform` (`KismetMathLibrary.MakeTransform` (`.GridVector_10_7F7B6B8542ECC301E9FFB082D723054A` (break `/Game/TowerDefenseStarterKit/Blueprints/GridSystems/Struct_GridCellData` (`|GetArrayItem` _gridgeneratordata GridCellIndex))) (`self.K2_GetActorRotation` _gridgenerator)))
  (return))

(fn `UserConstructionScript`)