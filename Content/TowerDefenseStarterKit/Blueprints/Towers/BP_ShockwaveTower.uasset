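; Area-of-effect shockwave tower for tower defense that periodically damages every enemy inside its range sphere.
; Range overlaps maintain a target list, starting a looping recharge timer on acquisition and clearing it when the list empties.
; Each pulse sends direct damage with critical-hit parameters to all valid targets and increments tower XP once per target.
; Enable and disable events resume the timer if targets remain or stop it.
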(event `self.RangeSphere.OnComponentBeginOverlap`
  (params (OverlappedComponent :type "PrimitiveComponent Object Reference") (OtherActor :type "Actor Object Reference") (OtherComp :type "PrimitiveComponent Object Reference") (OtherBodyIndex :type Integer) (bFromSweep :type Boolean) (SweepResult :type "HitResult Structure (by ref)"))
  ;[0 1 1 0.5] Detect targets in range & activates timed shockwave damage
  (bind _asbp_enemy_ai_parent (cast `/Game/TowerDefenseStarterKit/Blueprints/AI/Enemy/BP_EnemyAI_Parent` OtherActor))
  (`KismetArrayLibrary.Array_Add` (`self.TargetsInRange`) _asbp_enemy_ai_parent)
  (if (`self.IsFunctional?`)
    (if (not (`self.TargetsAcquired?`))
      (set `self.TargetsAcquired?` true)
      (`self.InitiateAttackTimer`))))

(event `self.RangeSphere.OnComponentEndOverlap`
  (params (OverlappedComponent :type "PrimitiveComponent Object Reference") (OtherActor :type "Actor Object Reference") (OtherComp :type "PrimitiveComponent Object Reference") (OtherBodyIndex :type Integer))
  ;[0 1 1 0.5] Remove units that are outside range, update units in range array; If no enemy units in range, clear shockwave timer
  (bind _asbp_enemy_ai_parent (cast `/Game/TowerDefenseStarterKit/Blueprints/AI/Enemy/BP_EnemyAI_Parent` OtherActor))
  (if (`KismetArrayLibrary.Array_Contains` (`self.TargetsInRange`) _asbp_enemy_ai_parent)
    (`KismetArrayLibrary.Array_RemoveItem` (`self.TargetsInRange`) _asbp_enemy_ai_parent)
    (if (not (> (`KismetArrayLibrary.Array_Length` (`self.TargetsInRange`)) 0))
      (`KismetSystemLibrary.K2_ClearAndInvalidateTimerHandle` (`self.AttackTimerHandle`))
      (set `self.TargetsAcquired?` false))))

(event `self.DisableCoreTowerSystems`
  ;[0 1 1 0.5] Turns on/off core tower functionality
  (`KismetSystemLibrary.K2_ClearAndInvalidateTimerHandle` (`self.AttackTimerHandle`)))

(event `self.EnableCoreTowerSystems`
  ;[0 1 1 0.5] Turns on/off core tower functionality
  (if (> (`KismetArrayLibrary.Array_Length` (`self.TargetsInRange`)) 0)
    (set `self.TargetsAcquired?` true)
    (`self.InitiateAttackTimer`) ; Initiates the attack timer if targets are in range
  ))

(fn `AttackEnemyUnits`
  ;[1 0 0 0.5] Attack all units in range
  (for _array_element (`self.TargetsInRange`)
    (`/Engine/EditorBlueprintResources/StandardMacros.IsValid` _array_element
      (:`Is Valid`
        (message `/Game/TowerDefenseStarterKit/Blueprints/GenericSystems/BPI_DamageApplicationSystem.ApplyDirectDamage` _array_element (`self.CalculateTrueOutputPerCycle`) (`self.CritHitChance`) (`self.CritHitDamageMultiplier`) self null)
        (`/Game/TowerDefenseStarterKit/Blueprints/Towers/SupportSystems/BPC_TowerXPManager.IncrementTowerXP` (`self.TowerXPManager`)) ; XP incremented for every output cycle
      )))
  (return))

(fn `InitiateAttackTimer`
  ;[0 1 1 0.5] Starts the attack timer
  (bind _returnvalue (`KismetSystemLibrary.K2_SetTimer` self "AttackEnemyUnits" (`self.RechargeTime`) true))
  (set `self.AttackTimerHandle` _returnvalue)
  (return))

(fn `UserConstructionScript`
  (`parent.UserConstructionScript`))