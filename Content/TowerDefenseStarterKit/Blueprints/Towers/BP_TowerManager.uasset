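; BP_TowerManager is the tower defense manager actor that spawns, destroys and upgrades towers, tracks them, and activates their Overdrive or Repair functions.
; It maps tower models and functions to data table row handles, using those rows for tower attributes and UI stats.
; It spawns a TowerConstructor actor to handle creation, control and range-display UI.
; Spawning and destruction update the GridManager obtained from BP_GameMode.
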(event `InitiateTowerCreationSystem`
  (params (GridCellIndex :type Integer) (GridGeneratorIndex :type Integer))
  ;[0 1 1 0.5] Tower Constructor Logic
  (`/Game/TowerDefenseStarterKit/Blueprints/Towers/BP_TowerConstructor.ActivateTowerCreationUI` (`self.TowerConstructor`) (`self.TowerDTMap`) (`self.SelectedBaseTowerModels`) GridCellIndex GridGeneratorIndex))

(event `InitiateTowerControlSystem`
  (params (TowerModel :type "/Game/TowerDefenseStarterKit/Blueprints/Towers/ETowerModels Enum" :default "NewEnumerator2") (GridCellIndex :type Integer) (GridGeneratorindex :type Integer))
  ;[0 1 1 0.5] Tower Constructor Logic
  (`/Game/TowerDefenseStarterKit/Blueprints/Towers/BP_TowerConstructor.ActivateTowerControlUI` (`self.TowerConstructor`) (`self.TowerDTMap`) TowerModel (`self.AvailableTowerFunctions`) (`self.TowerFunctionsDTMap`) GridCellIndex GridGeneratorindex))

(event `StopTowerConstructionSystems`
  ;[0 1 1 0.5] Tower Constructor Logic
  (`/Game/TowerDefenseStarterKit/Blueprints/Towers/BP_TowerConstructor.DeactivateAllModules` (`self.TowerConstructor`)))

(event `RefreshTowerConstructor`
  (bind _towerconstructor (`self.TowerConstructor`))
  ;[0 1 1 0.5] Tower Constructor Logic
  (`/Engine/EditorBlueprintResources/StandardMacros.IsValid` _towerconstructor
    (:`Is Valid`
      (`/Game/TowerDefenseStarterKit/Blueprints/Towers/BP_TowerConstructor.RefreshTowerInteractionUI` _towerconstructor))))

(event `DisplayRangeForTowerModel`
  (params (TowerModel :type "/Game/TowerDefenseStarterKit/Blueprints/Towers/ETowerModels Enum" :default "NewEnumerator2"))
  ;[0 1 1 0.5] Tower Constructor Logic
  (bind _towerdata (`self.GetRowDataForTowerModel` TowerModel)
    (:`Success`
      (`/Game/TowerDefenseStarterKit/Blueprints/Towers/BP_TowerConstructor.ActivateTowerRangeDisplay` (`self.TowerConstructor`) (`.Range_112_4C32B27E4B658C6B36A5BC96FC49E7DB` (break `/Game/TowerDefenseStarterKit/Blueprints/Towers/Struct_TowerData` _towerdata))))))

(event `HideTowerRange`
  ;[0 1 1 0.5] Tower Constructor Logic
  (`/Game/TowerDefenseStarterKit/Blueprints/Towers/BP_TowerConstructor.DeactivateTowerRangeDisplay` (`self.TowerConstructor`)))

(fn `ActivateTowerFunctionForTower`
  (params (Tower :type "Actor Object Reference") (TowerFunction :type "/Game/TowerDefenseStarterKit/Blueprints/Towers/TowerFunctions/ETowerFunctions Enum (by ref)" :default "NewEnumerator0"))
  ;[0 1 1 0.5] Initiates Tower Function activation
  (bind _towerfunctiondata (`self.GetRowDataForTowerFunction` TowerFunction)
    (:`Success`
      (bind ((`FunctionType_65_96563D8D45806ACC38ADDB98BAA247E9` _functiontype) (`Output_66_30759DDF438AF318B3B3EB93E872D3BE` _output) (`Duration_64_E797674D4F9E58E1A1EA4E8607CF011E` _duration) (`AbbreviatedName_56_7B8EDB924FE8DBA0D11B49B24483B64B` _abbreviatedname) (`StatusBarFillColor_69_E748892F477395F3BB2C78A4B8B5D91E` _statusbarfillcolor)) (break `/Game/TowerDefenseStarterKit/Blueprints/Towers/TowerFunctions/Struct_TowerFunctions` _towerfunctiondata))
      (switch `/Game/TowerDefenseStarterKit/Blueprints/Towers/TowerFunctions/ETowerFunctions` _functiontype
        (:`NewEnumerator0`
          (message `/Game/TowerDefenseStarterKit/Blueprints/Towers/TowerFunctions/BPI_TowerFunctions.AddOverdriveAbilityComponent` Tower _output _duration _abbreviatedname _statusbarfillcolor))
        (:`NewEnumerator1`
          (message `/Game/TowerDefenseStarterKit/Blueprints/Towers/TowerFunctions/BPI_TowerFunctions.AddRepairAbilityComponent` Tower _output _duration _abbreviatedname _statusbarfillcolor)))
      (return))
    (:`Failed`
      (return))))

(fn `DestroyTower`
  (params (TowerActor :type "/Game/TowerDefenseStarterKit/Blueprints/Towers/BP_Tower_Parent Object Reference"))
  (locals (Local_TowerActor :type "/Game/TowerDefenseStarterKit/Blueprints/Towers/BP_Tower_Parent Object Reference") (Local_GridGeneratorIndex :type Integer) (Local_GridCellIndex :type Integer :default 0))
  (bind (_gridcellindex _gridgeneratorindex) (`/Game/TowerDefenseStarterKit/Blueprints/Towers/BP_Tower_Parent.GetGridData` (`local.Local_TowerActor`)))
  ;[1 0 0 0.5] Destroys Tower; Updates the grid data arrays; Removed tower reference from the Tower Array
  (`/Engine/EditorBlueprintResources/StandardMacros.IsValid` TowerActor
    (:`Is Valid`
      (set `local.Local_TowerActor` TowerActor)
      (bind _asbp_game_mode (cast `/Game/TowerDefenseStarterKit/Blueprints/BP_GameMode` (`GameplayStatics.GetGameMode`)))
      (`/Game/TowerDefenseStarterKit/Blueprints/GridSystems/BP_GridManager.UpdateGridData` (`/Game/TowerDefenseStarterKit/Blueprints/BP_GameMode.RetrieveGridManager` _asbp_game_mode) _gridcellindex _gridgeneratorindex null "NewEnumerator0")
      (`KismetArrayLibrary.Array_RemoveItem` (`self.Towers`) (`local.Local_TowerActor`))
      (`self.K2_DestroyActor` (`local.Local_TowerActor`))
      (return))
    (:`Is Not Valid`
      (return))))

(fn `GetInfoAboutTowerFunction`
  (params (TowerFunction :type "/Game/TowerDefenseStarterKit/Blueprints/Towers/TowerFunctions/ETowerFunctions Enum" :default "NewEnumerator0"))
  (returns (FunctionName :type Text) (FunctionDescription :type Text) (Stats :type "Array of /Game/TowerDefenseStarterKit/Blueprints/HUDControl/Struct_HUDStats Structure"))
  ;[0 1 1 0.5] Returns information about the specified Tower Function
  (bind _towerfunctiondata (`self.GetRowDataForTowerFunction` TowerFunction)
    (:`Success`
      (bind ((`Output_66_30759DDF438AF318B3B3EB93E872D3BE` _output) (`Duration_64_E797674D4F9E58E1A1EA4E8607CF011E` _duration) (`FunctionName_54_3C56AE4A41587B969DAF63B6C1A6697E` _functionname) (`Description_50_BE7CCFD342D00631E73B398B4D907EBD` _description) (`UIStatName_CoreFunction_58_45FE1D2B46DE6A2EA93C0F8631A8F620` _uistatname_corefunction) (`UIStatName_LimitingFactor_59_0CEB480644CB2EB931B1FBA23EECD88B` _uistatname_limitingfactor)) (break `/Game/TowerDefenseStarterKit/Blueprints/Towers/TowerFunctions/Struct_TowerFunctions` _towerfunctiondata))
      (return _functionname _description (`|MakeArray` (make `/Game/TowerDefenseStarterKit/Blueprints/HUDControl/Struct_HUDStats` _uistatname_corefunction (`KismetTextLibrary.Conv_DoubleToText` _output "HalfToEven" false true 1 324 1)) (make `/Game/TowerDefenseStarterKit/Blueprints/HUDControl/Struct_HUDStats` _uistatname_limitingfactor (`KismetTextLibrary.Conv_DoubleToText` _duration "HalfToEven")))))
    (:`Failed`
      (return "" ""))))

(fn `GetInfoAboutTowerModel`
  (params (TowerModel :type "/Game/TowerDefenseStarterKit/Blueprints/Towers/ETowerModels Enum" :default "NewEnumerator2"))
  (returns (TowerName :type Text) (Description :type Text) (Stats :type "Array of /Game/TowerDefenseStarterKit/Blueprints/HUDControl/Struct_HUDStats Structure"))
  (locals (Local_LimitingFactorValue :type Text))
  ;[0 1 1 0.5] Returns information about the specified Tower Model
  (bind _towerdata (`self.GetRowDataForTowerModel` TowerModel)
    (:`Success`
      (bind ((`TowerModel_162_92ABD63D4C95B211A4F92C9576119898` _towermodel) (`OutputPerCycle_106_B6FA705847A52849B1B860A8DFC9E2EE` _outputpercycle) (`RateOfFire_110_3124D71F42CA24D37A1CD48108BCF959` _rateoffire) (`Armor_111_4EEDF32F48C02E074AB58EAF75B8F1EF` _armor) (`Range_112_4C32B27E4B658C6B36A5BC96FC49E7DB` _range) (`ResourceCap_115_2231880F440FBAEF3A1D9B9796DD1DAE` _resourcecap) (`TowerName_144_3B0A095B422712C96BC64A979E52F0D7` _towername) (`ShortDescription_43_4ACF3CC94015F3233C086B9B3CED3B1A` _shortdescription) (`UIStatName_CoreFunction_154_BB67803E4F3D9BCACDAC22A87B5E708E` _uistatname_corefunction) (`UIStatName_Defense_155_32B799A3451D85B1356719A97218F38A` _uistatname_defense) (`UIStatName_LimitingFactor_156_8B282A154AB760FB33184CBE31E4E6E5` _uistatname_limitingfactor)) (break `/Game/TowerDefenseStarterKit/Blueprints/Towers/Struct_TowerData` _towerdata))
      (switch `/Game/TowerDefenseStarterKit/Blueprints/Towers/ETowerModels` _towermodel
        (:`NewEnumerator2`
          (set `local.Local_LimitingFactorValue` (`KismetTextLibrary.Conv_IntToText` (`KismetMathLibrary.Round` _range)) :!label _label) ; Limiting Factor = Range
        )
        (:`NewEnumerator10`
          (goto _label))
        (:`NewEnumerator13`
          (goto _label))
        (:`NewEnumerator1`
          (goto _label))
        (:`NewEnumerator11`
          (goto _label))
        (:`NewEnumerator14`
          (goto _label))
        (:`NewEnumerator3`
          (goto _label))
        (:`NewEnumerator12`
          (goto _label))
        (:`NewEnumerator15`
          (goto _label))
        (:`NewEnumerator6`
          (goto _label))
        (:`NewEnumerator16`
          (goto _label))
        (:`NewEnumerator17`
          (goto _label))
        (:`NewEnumerator4`
          (goto _label))
        (:`NewEnumerator18`
          (goto _label))
        (:`NewEnumerator19`
          (goto _label))
        (:`NewEnumerator9`
          (goto _label))
        (:`NewEnumerator20`
          (goto _label))
        (:`NewEnumerator21`
          (goto _label))
        (:`NewEnumerator8`
          (set `local.Local_LimitingFactorValue` (`KismetTextLibrary.Conv_IntToText` (`KismetMathLibrary.Round` _resourcecap))) ; Limiting Factor = Resource Cap
        ))
      (return _towername _shortdescription (`|MakeArray` (make `/Game/TowerDefenseStarterKit/Blueprints/HUDControl/Struct_HUDStats` _uistatname_corefunction (`KismetTextLibrary.Conv_DoubleToText` (* _outputpercycle _rateoffire) "HalfToEven")) (make `/Game/TowerDefenseStarterKit/Blueprints/HUDControl/Struct_HUDStats` _uistatname_defense (`KismetTextLibrary.Conv_IntToText` (`KismetMathLibrary.Round` _armor))) (make `/Game/TowerDefenseStarterKit/Blueprints/HUDControl/Struct_HUDStats` _uistatname_limitingfactor (`local.Local_LimitingFactorValue`)))))
    (:`Failed`
      (return "" ""))))

(fn `GetTowers`
  (returns (TowerActorsArray :type "Array of /Game/TowerDefenseStarterKit/Blueprints/Towers/BP_Tower_Parent Object Reference"))
  (return (`self.Towers`)))

(fn `InitializeTowerManager`
  (params (`UseSelectedTowers?` :type Boolean) (SelectedBaseTowerModels :type "Array of /Game/TowerDefenseStarterKit/Blueprints/Towers/ETowerModels Enum" :default _))
  ;[0 1 0 0.5] Initialize the Tower Manager actor at level start
  (if `UseSelectedTowers?`
    (`self.SetSelectedBaseTowerModels` SelectedBaseTowerModels)
    (`self.MapTowerFunctionsToRowHandles`)
    (else
      (`self.SetSelectedBaseTowerModels` (`self.BaseTowerModels`))))
  (bind _returnvalue (`|SpawnActorFromClass` (`self.TowerConstructorClass`) (`self.GetTransform`) "AlwaysSpawn" "OverrideRootScale" null null))
  (bind _output_get (set `self.TowerConstructor` _returnvalue))
  (`/Game/TowerDefenseStarterKit/Blueprints/Towers/BP_TowerConstructor.Initialize` _output_get (`KismetArrayLibrary.Array_Length` (`self.SelectedBaseTowerModels`)) (`BlueprintMapLibrary.Map_Length` (`self.TowerFunctionsDTMap`)))
  (return))

(fn `MapTowerFunctionsToRowHandles`
  ;[0 1 1 0.5] Creates a mapping between tower functions & their associated rows in the Tower Functions data table
  (bind _outrownames (`DataTableFunctionLibrary.GetDataTableRowNames` "/Game/TowerDefenseStarterKit/Blueprints/Towers/TowerFunctions/DT_TowerFunctions.DT_TowerFunctions"))
  (for _array_element _outrownames
    (bind _returnvalue (`|GetDataTableRow` "/Game/TowerDefenseStarterKit/Blueprints/Towers/TowerFunctions/DT_TowerFunctions.DT_TowerFunctions" _array_element)
      (:`then`
        (`BlueprintMapLibrary.Map_Add` (`self.TowerFunctionsDTMap`) (`.FunctionType_65_96563D8D45806ACC38ADDB98BAA247E9` (break `/Game/TowerDefenseStarterKit/Blueprints/Towers/TowerFunctions/Struct_TowerFunctions` _returnvalue)) (make `DataTableRowHandle` "/Game/TowerDefenseStarterKit/Blueprints/Towers/TowerFunctions/DT_TowerFunctions.DT_TowerFunctions" _array_element)))))
  (return))

(fn `MapTowerModelToRowHandles`
  ;[0 1 1 0.5] Creates a mapping between tower models & their associated rows in the Tower Data data table
  (bind _outrownames (`DataTableFunctionLibrary.GetDataTableRowNames` "/Game/TowerDefenseStarterKit/Blueprints/Towers/DT_TowerData.DT_TowerData"))
  (for _array_element _outrownames
    (bind _returnvalue (`|GetDataTableRow` "/Game/TowerDefenseStarterKit/Blueprints/Towers/DT_TowerData.DT_TowerData" _array_element)
      (:`then`
        (`BlueprintMapLibrary.Map_Add` (`self.TowerDTMap`) (`.TowerModel_162_92ABD63D4C95B211A4F92C9576119898` (break `/Game/TowerDefenseStarterKit/Blueprints/Towers/Struct_TowerData` _returnvalue)) (make `DataTableRowHandle` "/Game/TowerDefenseStarterKit/Blueprints/Towers/DT_TowerData.DT_TowerData" _array_element)))))
  (return))

(fn `SetSelectedBaseTowerModels`
  (params (SelectedBaseTowerModels :type "Array of /Game/TowerDefenseStarterKit/Blueprints/Towers/ETowerModels Enum" :default _))
  (set `self.SelectedBaseTowerModels` SelectedBaseTowerModels)
  (return))

(fn `SpawnTower`
  (params (GridCellIndex :type Integer) (GridGeneratorIndex :type Integer) (TowerModel :type "/Game/TowerDefenseStarterKit/Blueprints/Towers/ETowerModels Enum" :default "NewEnumerator2"))
  (locals (Local_SpawnedTower :type "/Game/TowerDefenseStarterKit/Blueprints/Towers/BP_Tower_Parent Object Reference") (Local_SelectedGridCellIndex :type Integer :default 0) (Local_SelectedGridGeneratorIndex :type Integer :default 0))
  (bind ((`GridGeneratorData_11_13E757544C1E18F1261E9C9C7CA2FC04` _gridgeneratordata) (`GridGenerator_13_116FE1614615A5B5C63B70B45CFF220B` _gridgenerator)) (break `/Game/TowerDefenseStarterKit/Blueprints/GridSystems/Struct_GridData` (`|GetArrayItem` (`/Game/TowerDefenseStarterKit/Blueprints/FunctionLibraries/BPFL_GetterFunctions.GetGridDataArray` self) (`local.Local_SelectedGridGeneratorIndex`))))
  ;[0 1 1 0.5] Spawns Tower & updates Grid Gata; ; Adds tower to the Tower Array
  (set `local.Local_SelectedGridCellIndex` GridCellIndex)
  (set `local.Local_SelectedGridGeneratorIndex` GridGeneratorIndex)
  (bind _towerdata (`self.GetRowDataForTowerModel` TowerModel)
    (:`Success`
      (bind ((`SpawnClass_170_98F16BAF45FDB1271B0F7AAFED119690` _spawnclass) (`TowerModel_162_92ABD63D4C95B211A4F92C9576119898` _towermodel) (`SellingPrice_141_CDD596F947137FBEE513B99E18DE37FB` _sellingprice) (`OutputPerCycle_106_B6FA705847A52849B1B860A8DFC9E2EE` _outputpercycle) (`RateOfFire_110_3124D71F42CA24D37A1CD48108BCF959` _rateoffire) (`CritHitChance_133_ECE51C2C40E39F6DD290078D922021FD` _crithitchance) (`CritHitDamageMultiplier_136_5F0A559F480C42EE70DEE2B40584ABAD` _crithitdamagemultiplier) (`Armor_111_4EEDF32F48C02E074AB58EAF75B8F1EF` _armor) (`Range_112_4C32B27E4B658C6B36A5BC96FC49E7DB` _range) (`ResourceCap_115_2231880F440FBAEF3A1D9B9796DD1DAE` _resourcecap) (`TowerName_144_3B0A095B422712C96BC64A979E52F0D7` _towername) (`ShortDescription_43_4ACF3CC94015F3233C086B9B3CED3B1A` _shortdescription) (`UIStatName_CoreFunction_154_BB67803E4F3D9BCACDAC22A87B5E708E` _uistatname_corefunction) (`UIStatName_Defense_155_32B799A3451D85B1356719A97218F38A` _uistatname_defense) (`UIStatName_LimitingFactor_156_8B282A154AB760FB33184CBE31E4E6E5` _uistatname_limitingfactor)) (break `/Game/TowerDefenseStarterKit/Blueprints/Towers/Struct_TowerData` _towerdata))
      (bind _returnvalue (`|SpawnActorFromClass` _spawnclass (`KismetMathLibrary.MakeTransform` (`KismetMathLibrary.MakeVector` (.x (`.GridVector_10_7F7B6B8542ECC301E9FFB082D723054A` (break `/Game/TowerDefenseStarterKit/Blueprints/GridSystems/Struct_GridCellData` (`|GetArrayItem` _gridgeneratordata (`local.Local_SelectedGridCellIndex`))))) (.y (`.GridVector_10_7F7B6B8542ECC301E9FFB082D723054A` (break `/Game/TowerDefenseStarterKit/Blueprints/GridSystems/Struct_GridCellData` (`|GetArrayItem` _gridgeneratordata (`local.Local_SelectedGridCellIndex`))))) (+ (`self.TowerHeight`) (.z (`.GridVector_10_7F7B6B8542ECC301E9FFB082D723054A` (break `/Game/TowerDefenseStarterKit/Blueprints/GridSystems/Struct_GridCellData` (`|GetArrayItem` _gridgeneratordata (`local.Local_SelectedGridCellIndex`))))))) (`KismetMathLibrary.MakeRotator` 0.0 0.0 (.yaw (`self.K2_GetActorRotation` _gridgenerator)))) "AlwaysSpawn" "OverrideRootScale" null _towermodel _sellingprice _outputpercycle _crithitchance _crithitdamagemultiplier _armor _range _resourcecap (/ 1.0 _rateoffire) _towername _shortdescription _uistatname_corefunction _uistatname_defense _uistatname_limitingfactor (`local.Local_SelectedGridCellIndex`) (`local.Local_SelectedGridGeneratorIndex`) null)) ; Set Default Attributes at Spawn based on information stored in Tower Data Array
      (set `local.Local_SpawnedTower` _returnvalue)
      (bind _asbp_game_mode (cast `/Game/TowerDefenseStarterKit/Blueprints/BP_GameMode` (`GameplayStatics.GetGameMode`)))
      (`/Game/TowerDefenseStarterKit/Blueprints/GridSystems/BP_GridManager.UpdateGridData` (`/Game/TowerDefenseStarterKit/Blueprints/BP_GameMode.RetrieveGridManager` _asbp_game_mode) (`local.Local_SelectedGridCellIndex`) (`local.Local_SelectedGridGeneratorIndex`) (`local.Local_SpawnedTower`) "NewEnumerator1")
      (`KismetArrayLibrary.Array_Add` (`self.Towers`) (`local.Local_SpawnedTower`))
      (add `/Game/TowerDefenseStarterKit/Blueprints/Towers/BP_Tower_Parent.TowerPendingDeletion` (`local.Local_SpawnedTower`) (`|CreateDelegate` :!event `DestroyTower`)) ; Starts listening to Tower Deletion Events
      (return))))

(fn `UpgradeTower`
  (params (Tower :type "Actor Object Reference") (UpgradedTowerModel :type "/Game/TowerDefenseStarterKit/Blueprints/Towers/ETowerModels Enum" :default "NewEnumerator2"))
  ;[0 1 1 0.5] Initiates the Tower Upgrade process
  (bind _asbp_tower_parent (cast `/Game/TowerDefenseStarterKit/Blueprints/Towers/BP_Tower_Parent` Tower))
  (bind _towerdata (`self.GetRowDataForTowerModel` UpgradedTowerModel)
    (:`Success`
      (bind ((`TowerModel_162_92ABD63D4C95B211A4F92C9576119898` _towermodel) (`OutputPerCycle_106_B6FA705847A52849B1B860A8DFC9E2EE` _outputpercycle) (`RateOfFire_110_3124D71F42CA24D37A1CD48108BCF959` _rateoffire) (`Armor_111_4EEDF32F48C02E074AB58EAF75B8F1EF` _armor) (`Range_112_4C32B27E4B658C6B36A5BC96FC49E7DB` _range) (`ResourceCap_115_2231880F440FBAEF3A1D9B9796DD1DAE` _resourcecap) (`TowerMesh_148_494C675447F9E89B21E0DE82E2577791` _towermesh) (`TowerName_144_3B0A095B422712C96BC64A979E52F0D7` _towername) (`ShortDescription_43_4ACF3CC94015F3233C086B9B3CED3B1A` _shortdescription)) (break `/Game/TowerDefenseStarterKit/Blueprints/Towers/Struct_TowerData` _towerdata))
      (`/Game/TowerDefenseStarterKit/Blueprints/Towers/BP_Tower_Parent.UpgradeTower` _asbp_tower_parent _towermodel _outputpercycle (/ 1.0 _rateoffire) _armor _range _resourcecap _towermesh _towername _shortdescription)
      (return))))

(fn `UserConstructionScript`
  ;[0 1 0 0.5] Initialization Protocols
  (`self.MapTowerModelToRowHandles`))