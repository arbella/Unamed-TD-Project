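; Placeable bounds actor that defines the space in which the player's camera can move.
; The construction script sizes a TraceBlocker box from the TraceBlockerExtent variable.
; RetrieveCameraBoundsCoordinates returns min and max corners centered on the actor's location, derived by dividing that extent by BlockerBoundsToMovementBoundsRatio, so movement limits scale with the blocker box.
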(fn `RetrieveCameraBoundsCoordinates`
  (returns (MinCoordinates :type "Vector Structure") (MaxCoordinates :type "Vector Structure"))
  (bind _returnvalue (`self.K2_GetActorLocation`))
  (bind _returnvalue_2 (/ (`self.TraceBlockerExtent`) (`self.BlockerBoundsToMovementBoundsRatio`)))
  ;[0 1 1 0.5] Returns the lowest & highest possible vector coordinates which define the player movement space
  (return (- _returnvalue _returnvalue_2) (+ _returnvalue _returnvalue_2)))

(fn `UserConstructionScript`
  ;[0 1 1 0.5] Set default Box Extent for the Kill Z Volume
  (`BoxComponent.SetBoxExtent` (`self.TraceBlocker`) (`self.TraceBlockerExtent`) true))