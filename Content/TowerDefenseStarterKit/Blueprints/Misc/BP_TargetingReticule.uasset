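; Targeting reticule actor that marks a target location and shows whether it meets deployment requirements, apparently for Global Abilities.
; The construction script puts a dynamic material instance on the reticule mesh so its color can change at runtime.
; Display teleports the actor to the target and tints it red when valid or white when not, while Hide conceals it.
; A getter exposes the interface used to deploy Global Abilities.
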(fn `DisplayTargetingReticule`
  (params (TargetLocation :type "Vector Structure") (`ValidTarget?` :type Boolean))
  (bind _dmi_targetingreticule (`self.DMI_TargetingReticule`))
  ;[0 1 1 0.5] Updates the targeting reticule transform & color; Sets it to not hidden
  (`self.K2_SetActorTransform` (`KismetMathLibrary.Conv_VectorToTransform` TargetLocation) false true)
  (if `ValidTarget?`
    (`MaterialInstanceDynamic.SetVectorParameterValue` _dmi_targetingreticule "Color" (struct :`R` 4.0 :`A` 1.0)) ; Target actor meets deployment requirement
    (else
      (`MaterialInstanceDynamic.SetVectorParameterValue` _dmi_targetingreticule "Color" (struct :`R` 2.0 :`G` 2.0 :`B` 2.0 :`A` 1.0)) ; Target actor does not meet deployment requirements
    ))
  (`self.SetActorHiddenInGame` false))

(fn `GetGlobalAbilityTargetInterface`
  (returns (GlobalAbilityTargetInterface :type "Interface Class Reference"))
  ;[0 1 1 0.5] Returns the interface that enables deployment of Global Abilities
  (return (`self.GlobalAbilityTargetInterface`)))

(fn `HideTargetingReticule`
  ;[0 1 1 0.5] Hides the targeting reticule
  (`self.SetActorHiddenInGame` true)
  (return))

(fn `UserConstructionScript`
  ;[0 1 1 0.5] Create a Dynamic Material Instance to change the color of the Targeting Reticule Mesh at runtime
  (bind _returnvalue (`KismetMaterialLibrary.CreateDynamicMaterialInstance` "/Game/TowerDefenseStarterKit/Materials/M_TargetingReticule.M_TargetingReticule"))
  (set `self.DMI_TargetingReticule` _returnvalue)
  (`PrimitiveComponent.SetMaterial` (`self.TargetingReticuleMesh`) 0 (`self.DMI_TargetingReticule`)))