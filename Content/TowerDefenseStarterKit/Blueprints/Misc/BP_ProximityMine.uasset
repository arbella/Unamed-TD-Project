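; BP_ProximityMine is a tower defense mine that explodes when an enemy enters its trigger radius or an auto-detonation delay expires.
; Both paths share a DoOnce that plays effects, damages enemies found by a blast-radius sphere overlap, then destroys the mine.
; The construction script sizes the collision sphere and derives the range display's maximum scale from the trigger radius.
; A looping timer replays a timeline that pulses that holographic display.
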(event `OnActivateHolographicRangeDisplay`
  ;[0 1 1 0.5] Holographic Range Display
  (bind (_direction _lerpcontrol) (`Timeline|Timeline_TriggerRangeDisplay` :!via `PlayFromStart`)
    (:`Update`
      (`SceneComponent.SetRelativeScale3D` (`self.RangeDisplay`) (`KismetMathLibrary.Conv_DoubleToVector` (`KismetMathLibrary.Lerp` 0.0 (`self.MaxRangeDisplayScaleMultiplier`) _lerpcontrol))))))

(event `self.ReceiveBeginPlay`
  ;[0 1 0 0.5] Initialization Protocols
  (`self.OnActivateHolographicRangeDisplay`)
  (`KismetSystemLibrary.K2_SetTimerDelegate` (delegate `OnActivateHolographicRangeDisplay`) 1.2 true) ; Timer to repeat range display pulse
  (`KismetSystemLibrary.Delay` (`self.AutoDetonationTime`)) ; Auto Detonation Time Period
  ;[0 1 1 0.5] Explosion
  (`/Engine/EditorBlueprintResources/StandardMacros.DoOnce` false :!label _label ; Ensures that the explosion logic gets called only once
    (:`Completed`
      (`GameplayStatics.SpawnEmitterAtLocation` "/Game/TowerDefenseStarterKit/Effects/Explosion/P_Explosion_Standard.P_Explosion_Standard" (`self.K2_GetActorLocation`))
      (`GameplayStatics.PlaySound2D` "/Game/TowerDefenseStarterKit/Audio/Explosion/S_Explosion_Cue.S_Explosion_Cue" 1.0 1.0 0.0 null null)
      (bind _outactors (`KismetSystemLibrary.SphereOverlapActors` (`self.K2_GetActorLocation`) (`self.BlastRadius`) (`|MakeArray` "ObjectTypeQuery3" :!type "EObjectTypeQuery Enum") "/Game/TowerDefenseStarterKit/Blueprints/AI/Enemy/BP_EnemyAI_Parent.BP_EnemyAI_Parent_C"))
      (for _array_element _outactors
        (`/Engine/EditorBlueprintResources/StandardMacros.IsValid` _array_element
          (:`Is Valid`
            (message `/Game/TowerDefenseStarterKit/Blueprints/GenericSystems/BPI_DamageApplicationSystem.ApplyDirectDamage` _array_element (`self.Damage`) 0.0 0.0 self null))))
      (`self.K2_DestroyActor`))))

(event `self.SphereCollision.OnComponentBeginOverlap`
  (params (OverlappedComponent :type "PrimitiveComponent Object Reference") (OtherActor :type "Actor Object Reference") (OtherComp :type "PrimitiveComponent Object Reference") (OtherBodyIndex :type Integer) (bFromSweep :type Boolean) (SweepResult :type "HitResult Structure (by ref)"))
  ;[0 1 1 0.5] Proximity Trigger
  (cast `/Game/TowerDefenseStarterKit/Blueprints/AI/Enemy/BP_EnemyAI_Parent` OtherActor)
  (goto _label))

(fn `UserConstructionScript`
  (bind (_min _max) (`StaticMeshComponent.GetLocalBounds` (`self.RangeDisplay`)))
  ;[0 1 0 0.5] Initialization Protocols
  (set `self.MaxRangeDisplayScaleMultiplier` (/ (* (`self.TriggerRadius`) 2.0) (.x (- _max _min))))
  (`SphereComponent.SetSphereRadius` (`self.SphereCollision`) (`self.TriggerRadius`) true) ; Updates collision radius to match mine trigger radius
)