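; BP_GridCellHighlighter is an actor that marks a single grid cell in the tower defense kit by moving onto it and showing itself.
; HighlightGridCellAtIndex teleports it using CreateActorTransform and unhides it, while RemoveGridCellHighlights hides it.
; CreateActorTransform contains a transform node combining the indexed cell's position with its grid generator's rotation at unit scale, though that node appears unconnected.
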(event `HighlightGridCellAtIndex`
  (params (GridCellIndex :type Integer) (GridGeneratorindex :type Integer))
  (bind ((`GridGeneratorData_11_13E757544C1E18F1261E9C9C7CA2FC04` _gridgeneratordata) (`GridGenerator_13_116FE1614615A5B5C63B70B45CFF220B` _gridgenerator)) (break `/Game/TowerDefenseStarterKit/Blueprints/GridSystems/Struct_GridData` (`|GetArrayItem` (`/Game/TowerDefenseStarterKit/Blueprints/FunctionLibraries/BPFL_GetterFunctions.GetGridDataArray` self) GridGeneratorindex)))
  ;[0 1 1 0.5] Actor Transform + Visibility Control
  (`self.K2_SetActorTransform` (`KismetMathLibrary.MakeTransform` (`.GridVector_10_7F7B6B8542ECC301E9FFB082D723054A` (break `/Game/TowerDefenseStarterKit/Blueprints/GridSystems/Struct_GridCellData` (`|GetArrayItem` _gridgeneratordata GridCellIndex))) (`self.K2_GetActorRotation` _gridgenerator)) false true) ; Updates actor transform based on the specified grid cell
  (`self.SetActorHiddenInGame` false))

(event `RemoveGridCellHighlights`
  ;[0 1 1 0.5] Actor Transform + Visibility Control
  (`self.SetActorHiddenInGame` true))

(fn `UserConstructionScript`)