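; BP_ExitPoint is the tower defense exit that enemy units try to reach, costing the player score when they get there.
; On box overlap, it lowers the player state score by the enemy's score reduction value and tells the enemy to run its termination protocols.
; When the score hits zero, it has the HUD show a failure mission summary and destroys itself.
; The construction script tints its marker via a dynamic grid material.
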(event `self.Box.OnComponentBeginOverlap`
  (params (OverlappedComponent :type "PrimitiveComponent Object Reference") (OtherActor :type "Actor Object Reference") (OtherComp :type "PrimitiveComponent Object Reference") (OtherBodyIndex :type Integer) (bFromSweep :type Boolean) (SweepResult :type "HitResult Structure (by ref)"))
  ;[1 0 0 0.5] Reduces score based on the score modifier of the enemy unit; Calls HUD updates; & Handles End Game validations
  (bind _asbp_enemy_ai_parent (cast `/Game/TowerDefenseStarterKit/Blueprints/AI/Enemy/BP_EnemyAI_Parent` OtherActor))
  (bind _asbp_player_state (cast `/Game/TowerDefenseStarterKit/Blueprints/Player/BP_PlayerState` (`Controller.PlayerState` (`GameplayStatics.GetPlayerController` 0))))
  (bind _newscore (`/Game/TowerDefenseStarterKit/Blueprints/Player/BP_PlayerState.ModifyPlayerScore` _asbp_player_state (`/Game/TowerDefenseStarterKit/Blueprints/AI/Enemy/BP_EnemyAI_Parent.GetPlayerScoreReduction` _asbp_enemy_ai_parent)))
  (`/Game/TowerDefenseStarterKit/Blueprints/AI/Enemy/BP_EnemyAI_Parent.ActivateTerminationProtocols` _asbp_enemy_ai_parent true) ; Request the overlapping enemy unit to activate it's termination protocols before destroying itself
  (if (not (> _newscore 0))
    (bind _asbp_player_hud (cast `/Game/TowerDefenseStarterKit/Blueprints/Player/BP_PlayerHUD` (`PlayerController.GetHUD` (`GameplayStatics.GetPlayerController` 0))))
    (`/Game/TowerDefenseStarterKit/Blueprints/Player/BP_PlayerHUD.DisplayMissionSummary` _asbp_player_hud false) ; Mission Failure: Requests Player HUD to display Mission Summary screen
    (`self.K2_DestroyActor` self)))

(fn `UserConstructionScript`
  (bind _returnvalue (`PrimitiveComponent.CreateDynamicMaterialInstance` (`self.Marker`) 0 "/Game/TowerDefenseStarterKit/Materials/M_Grid.M_Grid" "None"))
  (`MaterialInstanceDynamic.SetVectorParameterValue` _returnvalue "Color" (struct :`G` 0.75 :`B` 1.0 :`A` 1.0)))